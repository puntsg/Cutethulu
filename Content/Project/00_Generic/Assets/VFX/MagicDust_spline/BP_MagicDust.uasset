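; BP_MagicDust is a spline-driven Niagara VFX actor for a magic dust effect.
; On construction and at BeginPlay, it passes its spline component to the Niagara system's "Spline" variable.
; A helper estimates padded bounds by sampling points along the spline, but it and the fixed-bounds call are unwired, so neither runs.
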(event EventBeginPlay
  (CallFunction|SetupNiagraSystem))

(fn ConstructionScript
  (CallFunction|SetupNiagraSystem))

(fn SetupNiagraSystem
  (Niagara|SetNiagaraVariable(Object) (Variables|Default|GetNiagara) "Spline" (Variables|Default|GetSpline)))

(fn EstimateSplineBounds
  (bind _boundsoffset (Variables|Default|GetBoundsOffset))
  ;[0.15 0.15 0.15 0.5] Calculate new Bounds
  (bind _output_get (Variables|Default|SetThis%20Min "100000000000000001463069523067487303097004298786465505927861078716979636425114821591040.000000,100000000000000001463069523067487303097004298786465505927861078716979636425114821591040.000000,100000000000000001463069523067487303097004298786465505927861078716979636425114821591040.000000"))
  (Variables|Default|SetThis%20Max (* _output_get -1.0))
  (for _index (range 0 99)
    (bind _output_get_2 (Variables|Default|SetThis%20Sample (- (Spline|GetLocationatTime (Variables|Default|GetSpline) (/ _index 1e+02) "Local" false) (Transformation|GetActorLocation))))
    (Variables|Default|SetThis%20Min (Math|Vector|MakeVector (Math|Float|Min(Float) (.X (Math|Vector|BreakVector _output_get_2)) (.X (Math|Vector|BreakVector (Variables|Default|GetThis%20Min)))) (Math|Float|Min(Float) (.Y (Math|Vector|BreakVector _output_get_2)) (.Y (Math|Vector|BreakVector (Variables|Default|GetThis%20Min)))) (Math|Float|Min(Float) (.Z (Math|Vector|BreakVector _output_get_2)) (.Z (Math|Vector|BreakVector (Variables|Default|GetThis%20Min))))))
    (Variables|Default|SetThis%20Max (Math|Vector|MakeVector (Math|Float|Max(Float) (.X (Math|Vector|BreakVector _output_get_2)) (.X (Math|Vector|BreakVector (Variables|Default|GetThis%20Max)))) (Math|Float|Max(Float) (.Y (Math|Vector|BreakVector _output_get_2)) (.Y (Math|Vector|BreakVector (Variables|Default|GetThis%20Max)))) (Math|Float|Max(Float) (.Z (Math|Vector|BreakVector _output_get_2)) (.Z (Math|Vector|BreakVector (Variables|Default|GetThis%20Max)))))))
  (return (- (Variables|Default|GetThis%20Min) _boundsoffset) (+ (Variables|Default|GetThis%20Max) _boundsoffset)))