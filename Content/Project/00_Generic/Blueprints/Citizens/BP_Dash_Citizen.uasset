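; BP_Dash_Citizen is a citizen NPC that talks when the player comes near and swaps its shell material between cute and horror worlds.
; Player detection toggles an exclamation mark until it has spoken, deferring display until OnHealedWorld if the world is healing.
; Near and flee events start and stop the text system, and leaving detection finishes the tutorial for tutorial NPCs.
; SetCitizenType picks the shell material pair based on whether the citizen is transformed.
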(event Custom|Begin%20To%20Detect
  (params (Character :type BP%20Playable%20Character%20Object%20Reference))
  (bind _returnvalue (Game|GetGameMode))
  (bind _asyako_taki_game_mode (Utilities|Casting|CastToYakoTakiGameMode _returnvalue))
  ;[0.15 0.15 0.15 0.5] Subscribe on begin to detect
  (if (not (Variables|Default|GetHasSpeak))
    (if (not (Variables|/Game/Project/00_Generic/Blueprints/GameModes/YakoTakiGameMode.YakoTakiGameMode_C|GethealingWorld _asyako_taki_game_mode))
      (Development|SetHiddeninGame (Variables|Default|GetWidgetExlamationMark) false false)
      (else
        ;[0.15 0.15 0.15 0.5] Hide while healing world
        (EventDispatchers|AssignOnHealedWorld _asyako_taki_game_mode (delegate Custom|OnHealedWorld_Event))))))

(event Custom|End%20To%20Detect
  (params (Character :type BP%20Playable%20Character%20Object%20Reference))
  ;[0.15 0.15 0.15 0.5] Subscribe on leave to detect
  (Development|SetHiddeninGame (Variables|Default|GetWidgetExlamationMark) true false)
  (if (Variables|Default|GetIsTutorialNPC)
    (Default|FinishTutorial (Variables|Default|GetAC_TutorialMessage))))

(event Custom|Begin%20To%20Interact
  (params (Character :type BP%20Playable%20Character%20Object%20Reference))
  ;[0.15 0.15 0.15 0.5] Subscribe on leave to interact
  (Default|StopSpeak (Variables|Default|GetSC_TextSystem)))

(event Custom|End%20To%20Interact
  (params (Character :type BP%20Playable%20Character%20Object%20Reference))
  ;[0.15 0.15 0.15 0.5] Subscribe on begin to interact
  (Variables|Default|SetHasSpeak true)
  (Default|Speak (Variables|Default|GetSC_TextSystem))
  (Development|SetHiddeninGame (Variables|Default|GetWidgetExlamationMark) true false))

(event Custom|OnHealedWorld_Event
  ;[0.15 0.15 0.15 0.5] Hide while healing world
  (Development|SetHiddeninGame (Variables|Default|GetWidgetExlamationMark) false false))

(event EventBeginPlay
  ;[0.15 0.15 0.15 0.5] Subscribe on begin to detect
  (|CallParentFunction)
  (EventDispatchers|BindEventtoOnPlayerEnterDetection (delegate Custom|Begin%20To%20Detect))
  ;[0.15 0.15 0.15 0.5] Subscribe on begin to interact
  (EventDispatchers|BindEventtoOnPlayerNear (delegate Custom|End%20To%20Interact))
  ;[0.15 0.15 0.15 0.5] Subscribe on leave to detect
  (EventDispatchers|BindEventtoOnPlayerExitsDetection (delegate Custom|End%20To%20Detect))
  ;[0.15 0.15 0.15 0.5] Subscribe on leave to interact
  (EventDispatchers|BindEventtoOnPlayerFlees (delegate Custom|Begin%20To%20Interact)))

(event EventOnHorrorLoaded
  ;[0.15 0.15 0.15 0.5] Replace material on cute/horror change
  (|CallParentFunction)
  (Rendering|Material|SetMaterial (Variables|Character|GetMesh) 1 (Variables|Default|GetShell%20Material%20Horror)))

(event EventOnCuteLoaded
  ;[0.15 0.15 0.15 0.5] Replace material on cute/horror change
  (|CallParentFunction)
  (Rendering|Material|SetMaterial (Variables|Character|GetMesh) 1 (Variables|Default|GetShell%20Material%20Cute)))

(fn ConstructionScript
  (|CallParentFunction))

(fn SetCitizenType
  (params (IsTransformCitizen :type Boolean))
  (|CallParentFunction IsTransformCitizen)
  (if IsTransformCitizen
    (Variables|Default|SetShell%20Material%20Horror (Variables|Default|GetShell%20Material%20Horror%20Has%20Transform))
    (Variables|Default|SetShell%20Material%20Cute (Variables|Default|GetShell%20Material%20Cute%20Has%20Transform))
    (else
      (Variables|Default|SetShell%20Material%20Horror (Variables|Default|GetShell%20Material%20Horror%20Without%20Transform))
      (Variables|Default|SetShell%20Material%20Cute (Variables|Default|GetShell%20Material%20Cute%20Without%20Transform)))))