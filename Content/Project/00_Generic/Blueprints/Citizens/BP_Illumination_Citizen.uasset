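; Citizen NPC Blueprint for the Illumination citizen, which talks to the player and swaps its look between Horror and Cute worlds.
; Parent detection and proximity events toggle an exclamation mark until it has spoken, start or stop speech, and finish tutorials for tutorial NPCs.
; World-load events swap body material, fire Niagara effect and bow material, with body variants chosen by citizen type.
; The Romeo flag reveals the bow mesh.
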(event Custom|Begin%20To%20Detect
  (params (Character :type BP%20Playable%20Character%20Object%20Reference))
  ;[0.15 0.15 0.15 0.5] Subscribe on begin to detect
  (if (not (Variables|Default|GetHasSpeak))
    (Development|SetHiddeninGame (Variables|Default|GetWidgetExlamationMark) false false)))

(event Custom|End%20To%20Detect
  (params (Character :type BP%20Playable%20Character%20Object%20Reference))
  ;[0.15 0.15 0.15 0.5] Subscribe on leave to detect
  (Development|SetHiddeninGame (Variables|Default|GetWidgetExlamationMark) true false)
  (if (Variables|Default|GetIsTutorialNPC)
    (Default|FinishTutorial (Variables|Default|GetAC_TutorialMessage))))

(event Custom|Begin%20To%20Interact
  (params (Character :type BP%20Playable%20Character%20Object%20Reference))
  ;[0.15 0.15 0.15 0.5] Subscribe on leave to interact
  (Default|StopSpeak (Variables|Default|GetSC_TextSystem)))

(event Custom|End%20To%20Interact
  (params (Character :type BP%20Playable%20Character%20Object%20Reference))
  ;[0.15 0.15 0.15 0.5] Subscribe on begin to interact
  (Variables|Default|SetHasSpeak true)
  (Default|Speak (Variables|Default|GetSC_TextSystem))
  (Development|SetHiddeninGame (Variables|Default|GetWidgetExlamationMark) true false))

(event EventBeginPlay
  (if (Variables|Default|GetIsRomeo?)
    (Rendering|SetVisibility (Variables|Default|GetSM_BowLight) true false))
  (|CallParentFunction)
  ;[0.15 0.15 0.15 0.5] Subscribe on begin to detect
  (EventDispatchers|BindEventtoOnPlayerEnterDetection (delegate Custom|Begin%20To%20Detect))
  ;[0.15 0.15 0.15 0.5] Subscribe on begin to interact
  (EventDispatchers|BindEventtoOnPlayerNear (delegate Custom|End%20To%20Interact))
  ;[0.15 0.15 0.15 0.5] Subscribe on leave to detect
  (EventDispatchers|BindEventtoOnPlayerExitsDetection (delegate Custom|End%20To%20Detect))
  ;[0.15 0.15 0.15 0.5] Subscribe on leave to interact
  (EventDispatchers|BindEventtoOnPlayerFlees (delegate Custom|Begin%20To%20Interact)))

(event EventOnHorrorLoaded
  (|CallParentFunction)
  (Rendering|Material|SetMaterial (Variables|Character|GetMesh) 1 (Variables|Materials|Horror|GetBody%20Material%20Horror))
  (Class|NiagaraComponent|SetAsset (Variables|Default|GetNiagara_0) "/Game/Project/00_Generic/Assets/VFX/FireHead/FXS_FireCitizen_h.FXS_FireCitizen_h" true)
  (Rendering|Material|SetMaterial (Variables|Default|GetSM_BowLight) 0 (Variables|Materials|Horror|GetBow%20Material%20Horror)))

(event EventOnCuteLoaded
  (|CallParentFunction)
  (Rendering|Material|SetMaterial (Variables|Character|GetMesh) 1 (Variables|Materials|Cute|GetBody%20Material%20Cute))
  (Class|NiagaraComponent|SetAsset (Variables|Default|GetNiagara_0) "/Game/Project/00_Generic/Assets/VFX/FireHead/FXS_FireCitizen_c.FXS_FireCitizen_c" true)
  (Rendering|Material|SetMaterial (Variables|Default|GetSM_BowLight) 0 (Variables|Materials|Cute|GetBow%20Material%20Cute)))

(fn ConstructionScript
  (|CallParentFunction))

(fn SetCitizenType
  (params (IsTransformCitizen :type Boolean))
  (|CallParentFunction IsTransformCitizen)
  (if IsTransformCitizen
    (Variables|Materials|Horror|SetBody%20Material%20Horror (Variables|Materials|Horror|GetBody%20Material%20Horror%20Has%20Transform))
    (Variables|Materials|Cute|SetBody%20Material%20Cute (Variables|Materials|Cute|GetBody%20Material%20Cute%20Has%20Transform))
    (else
      (Variables|Materials|Horror|SetBody%20Material%20Horror (Variables|Materials|Horror|GetBody%20Material%20Horror%20Withour%20Transform))
      (Variables|Materials|Cute|SetBody%20Material%20Cute (Variables|Materials|Cute|GetBody%20Material%20Cute%20Withour%20Transform)))))