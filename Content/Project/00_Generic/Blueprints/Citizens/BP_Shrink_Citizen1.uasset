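; BP_Shrink_Citizen1 is a citizen Blueprint that speaks through its text system when the player comes near and stops when the player flees.
; On BeginPlay it binds handlers to inherited player detection and proximity events.
; The detection enter and exit handlers are empty.
; Interaction handler names are inverted: EndToInteract starts speech and BeginToInteract stops it.
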(event Custom|Begin%20To%20Detect
  (params (Character :type BP%20Playable%20Character%20Object%20Reference))
  ;[0.15 0.15 0.15 0.5] Subscribe on begin to detect
)

(event Custom|End%20To%20Detect
  (params (Character :type BP%20Playable%20Character%20Object%20Reference))
  ;[0.15 0.15 0.15 0.5] Subscribe on leave to detect
)

(event Custom|Begin%20To%20Interact
  (params (Character :type BP%20Playable%20Character%20Object%20Reference))
  ;[0.15 0.15 0.15 0.5] Subscribe on leave to interact
  (Default|StopSpeak (Variables|Default|GetSC_TextSystem)))

(event Custom|End%20To%20Interact
  (params (Character :type BP%20Playable%20Character%20Object%20Reference))
  ;[0.15 0.15 0.15 0.5] Subscribe on begin to interact
  (Default|Speak (Variables|Default|GetSC_TextSystem)))

(event EventBeginPlay
  (|CallParentFunction)
  ;[0.15 0.15 0.15 0.5] Subscribe on begin to detect
  (EventDispatchers|BindEventtoOnPlayerEnterDetection (delegate Custom|Begin%20To%20Detect))
  ;[0.15 0.15 0.15 0.5] Subscribe on begin to interact
  (EventDispatchers|BindEventtoOnPlayerNear (delegate Custom|End%20To%20Interact))
  ;[0.15 0.15 0.15 0.5] Subscribe on leave to detect
  (EventDispatchers|BindEventtoOnPlayerExitsDetection (delegate Custom|End%20To%20Detect))
  ;[0.15 0.15 0.15 0.5] Subscribe on leave to interact
  (EventDispatchers|BindEventtoOnPlayerFlees (delegate Custom|Begin%20To%20Interact)))

(event Collision|EventActorBeginOverlap
  (params (OtherActor :type Actor%20Object%20Reference)))

(fn ConstructionScript
  (|CallParentFunction))