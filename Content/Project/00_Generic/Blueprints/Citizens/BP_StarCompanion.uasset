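; BP_StarCompanion is a star companion citizen that speaks while the player character is near it.
; On BeginPlay it hands its face mesh to the SCTextSystem component, has that component assign its primitive component, and plays its ActorSequence.
; Overlaps on TextCollider with BP_PlayableCharacter call Speak on enter and StopSpeak on exit, leaving the dialogue itself to the text system.
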(event OnComponentBeginOverlap(TextCollider)
  (params (OverlappedComponent :type Primitive%20Component%20Object%20Reference) (OtherActor :type Actor%20Object%20Reference) (OtherComp :type Primitive%20Component%20Object%20Reference) (OtherBodyIndex :type Integer) (bFromSweep :type Boolean) (SweepResult :type Hit%20Result%20Structure%20%28by%20ref%29))
  ;[0.15 0.15 0.15 0.5] Colliders to Start /End Dialogue
  (Utilities|Casting|CastToBP_PlayableCharacter OtherActor)
  (Default|Speak (Variables|Default|GetSC_TextSystem)))

(event OnComponentEndOverlap(TextCollider)
  (params (OverlappedComponent :type Primitive%20Component%20Object%20Reference) (OtherActor :type Actor%20Object%20Reference) (OtherComp :type Primitive%20Component%20Object%20Reference) (OtherBodyIndex :type Integer))
  ;[0.15 0.15 0.15 0.5] Colliders to Start /End Dialogue
  (Utilities|Casting|CastToBP_PlayableCharacter OtherActor)
  (Default|StopSpeak (Variables|Default|GetSC_TextSystem)))

(event EventBeginPlay
  (bind _sc_textsystem (Variables|Default|GetSC_TextSystem))
  ;[0.15 0.15 0.15 0.5] Setting text system
  (Variables|/Game/Project/00_Generic/Blueprints/Components/SC_TextSystem.SC_TextSystem_C|SetSM_Reference _sc_textsystem (Variables|Default|GetSM_StarCompanion_Face))
  (Default|AssignPrimitiveComponent _sc_textsystem)
  (Class|ActorSequenceComponent|PlaySequence (Variables|Default|GetActorSequence)))

(fn ConstructionScript)