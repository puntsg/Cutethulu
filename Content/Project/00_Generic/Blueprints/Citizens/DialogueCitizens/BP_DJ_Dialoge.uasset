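; BP_DJ_Dialoge is a citizen dialogue Blueprint, named for a DJ, that talks when the player comes near.
; On BeginPlay it binds handlers to the player detection enter and exit events.
; Entering detection calls Speak on its SCTextSystem, and leaving calls StopSpeak.
; The construction script only runs the parent's version.
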(event Custom|Begin%20to
  (params (Character :type BP%20Playable%20Character%20Object%20Reference))
  (Default|Speak (Variables|Default|GetSC_TextSystem)))

(event Custom|End%20to
  (params (Character :type BP%20Playable%20Character%20Object%20Reference))
  (Default|StopSpeak (Variables|Default|GetSC_TextSystem)))

(event EventBeginPlay
  (|CallParentFunction)
  (EventDispatchers|BindEventtoOnPlayerEnterDetection (delegate Custom|Begin%20to))
  (EventDispatchers|BindEventtoOnPlayerExitsDetection (delegate Custom|End%20to)))

(event Collision|EventActorBeginOverlap
  (params (OtherActor :type Actor%20Object%20Reference)))

(event EventTick
  (params (DeltaSeconds :type Float%20%28single-precision%29)))

(fn ConstructionScript
  (|CallParentFunction))