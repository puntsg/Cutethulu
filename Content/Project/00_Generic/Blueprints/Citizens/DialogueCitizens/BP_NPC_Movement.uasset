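; Citizen NPC Blueprint that moves on the navmesh, reacts to nearby players, assigns a transformation class on interact and swaps materials between Cute and Horror worlds.
; Detection and interaction volumes track the player, optionally only Taki, fire dispatchers, register the NPC as interactable and toggle an overlay outline.
; AIMoveTo drives random roaming, targeted moves, return to spawn and looping patrol.
; FacePlayer re-calls itself each tick to smoothly turn toward the detected player.
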(event OnComponentBeginOverlap(DetectionArea)
  (params (OverlappedComponent :type Primitive%20Component%20Object%20Reference) (OtherActor :type Actor%20Object%20Reference) (OtherComp :type Primitive%20Component%20Object%20Reference) (OtherBodyIndex :type Integer) (bFromSweep :type Boolean) (SweepResult :type Hit%20Result%20Structure%20%28by%20ref%29))
  ;[0.15 0.15 0.15 0.5] Colliders
  ;;[0.15 0.15 0.15 0.5] On Overlap events
  (bind _asbp_playable_character (Utilities|Casting|CastToBP_PlayableCharacter OtherActor))
  (if (Variables|PlayableCharacterRelated|detection|GetOnlyInteractWithTaki)
    (Variables|PlayableCharacterRelated|detection|SetDetectedCharacter (.AsBP%20Player%20Default%20Taki (Utilities|Casting|CastToBP_PlayerDefault_Taki _asbp_playable_character)))
    (else
      (Variables|PlayableCharacterRelated|detection|SetDetectedCharacter _asbp_playable_character)))
  (Default|CallOnPlayerEnterDetection (Variables|PlayableCharacterRelated|detection|GetDetectedCharacter)))

(event OnComponentEndOverlap(DetectionArea)
  (params (OverlappedComponent :type Primitive%20Component%20Object%20Reference) (OtherActor :type Actor%20Object%20Reference) (OtherComp :type Primitive%20Component%20Object%20Reference) (OtherBodyIndex :type Integer))
  ;[0.15 0.15 0.15 0.5] Colliders
  ;;[0.15 0.15 0.15 0.5] On Overlap events
  (bind _asbp_playable_character (Utilities|Casting|CastToBP_PlayableCharacter OtherActor))
  (Variables|PlayableCharacterRelated|detection|SetDetectedCharacter 0)
  (Default|CallOnPlayerExitsDetection _asbp_playable_character))

(event OnComponentBeginOverlap(InteractionArea)
  (params (OverlappedComponent :type Primitive%20Component%20Object%20Reference) (OtherActor :type Actor%20Object%20Reference) (OtherComp :type Primitive%20Component%20Object%20Reference) (OtherBodyIndex :type Integer) (bFromSweep :type Boolean) (SweepResult :type Hit%20Result%20Structure%20%28by%20ref%29))
  ;[0.15 0.15 0.15 0.5] Colliders
  ;;[0.15 0.15 0.15 0.5] On Overlap events
  (bind _asbp_playable_character (Utilities|Casting|CastToBP_PlayableCharacter OtherActor))
  (if (Variables|PlayableCharacterRelated|detection|GetOnlyInteractWithTaki)
    (Variables|PlayableCharacterRelated|detection|SetNearbyPlayer (.bSuccess (Utilities|Casting|CastToBP_PlayerDefault_Taki _asbp_playable_character)))
    (else
      (Variables|PlayableCharacterRelated|detection|SetNearbyPlayer true)))
  (Default|CallOnPlayerNear _asbp_playable_character)
  (Variables|/Game/Project/00_Generic/Blueprints/PlayableCharacters/BP_PlayableCharacter.BP_PlayableCharacter_C|SetCurrentInteractive _asbp_playable_character self)
  (CallFunction|SetOutliner (Variables|Outliner|GetOutlineOnAproach))
  (if (Variables|PlayableCharacterRelated|Looking|GetLookAtPlayer)
    (CallFunction|FacePlayer)))

(event OnComponentEndOverlap(InteractionArea)
  (params (OverlappedComponent :type Primitive%20Component%20Object%20Reference) (OtherActor :type Actor%20Object%20Reference) (OtherComp :type Primitive%20Component%20Object%20Reference) (OtherBodyIndex :type Integer))
  ;[0.15 0.15 0.15 0.5] Colliders
  ;;[0.15 0.15 0.15 0.5] On Overlap events
  (bind _asbp_playable_character (Utilities|Casting|CastToBP_PlayableCharacter OtherActor))
  (Variables|PlayableCharacterRelated|detection|SetDetectedCharacter 0)
  (Variables|PlayableCharacterRelated|detection|SetNearbyPlayer false)
  (Default|CallOnPlayerFlees _asbp_playable_character)
  (CallFunction|SetOutliner false)
  (Variables|/Game/Project/00_Generic/Blueprints/PlayableCharacters/BP_PlayableCharacter.BP_PlayableCharacter_C|SetCurrentInteractive _asbp_playable_character 0))

(event Custom|SetOutliner
  (params (Enabled :type Boolean))
  (bind _outlinerinstance (Variables|Outliner|GetOutlinerInstance))
  ;[0.15 0.15 0.15 0.5] Custom Events
  ;;[0.15 0.15 0.15 0.5] Outliner
  (if Enabled
    (Rendering|Material|SetScalarParameterValue _outlinerinstance "Thickness" 5.0 :!class /Script/Engine.MaterialInstanceDynamic)
    (else
      (Rendering|Material|SetScalarParameterValue _outlinerinstance "Thickness" 0.0 :!class /Script/Engine.MaterialInstanceDynamic))))

(event Custom|Return%20to%20start%20point
  ;[0.15 0.15 0.15 0.5] Custom Events
  ;;[0.15 0.15 0.15 0.5] Movement Events
  (bind _output_get (Variables|AIMoveParams|SetDestinyLocation (Variables|InitialValues|GetSpawnPosition)))
  (AI|AIMoveTo self _output_get 0 2.5e+02 false
    (:OnSuccess
      (Default|CallOnReturnedtoOriginalPos))
    (:OnFail
      (Default|CallOnAgentFailReachingTarget))))

(event Custom|Go%20to%20position
  (params (NewTargetLocation :type Vector))
  ;[0.15 0.15 0.15 0.5] Custom Events
  ;;[0.15 0.15 0.15 0.5] Movement Events
  (Variables|AIMoveParams|SetDestinyLocation NewTargetLocation)
  (AI|AIMoveTo self (Variables|AIMoveParams|GetDestinyLocation) 0 2.5e+02 false
    (:OnSuccess
      (Default|CallOnAgentReachTarget))
    (:OnFail
      (Default|CallOnAgentFailReachingTarget))))

(event Custom|MoveAgent
  (params (Radius :type Float%20%28double-precision%29) (StartFromInitialPosition :type Boolean))
  ;[0.15 0.15 0.15 0.5] Custom Events
  ;;[0.15 0.15 0.15 0.5] Movement Events
  (if StartFromInitialPosition
    (Variables|AIMoveParams|SetDestinyLocation (.RandomLocation (AI|Navigation|GetRandomReachablePointinRadius (Variables|InitialValues|GetSpawnPosition) Radius 0 0)))
    (else
      (Variables|AIMoveParams|SetDestinyLocation (.RandomLocation (AI|Navigation|GetRandomReachablePointinRadius (Transformation|GetActorLocation) Radius 0 0)))))
  (AI|AIMoveTo self (Variables|AIMoveParams|GetDestinyLocation) 0 2.5e+02 false
    (:OnSuccess
      (Default|CallOnAgentReachTarget))
    (:OnFail
      (Default|CallOnAgentFailReachingTarget))))

(event Custom|FacePlayer
  ;[0.15 0.15 0.15 0.5] Custom Events
  ;;[0.15 0.15 0.15 0.5] Look at event
  (if (and (Utilities|IsValid (Variables|PlayableCharacterRelated|detection|GetDetectedCharacter)) (Variables|PlayableCharacterRelated|Looking|GetLookAtPlayer))
    (Transformation|SetActorRotation (Math|Rotator|MakeRotator 0.0 0.0 (.yaw (Math|Interpolation|RInterpTo (Transformation|GetActorRotation) (Math|Rotator|FindLookatRotation (Transformation|GetActorLocation) (Transformation|GetActorLocation (Variables|PlayableCharacterRelated|detection|GetDetectedCharacter))) (Utilities|Time|GetWorldDeltaSeconds) 15.0))))
    (Utilities|FlowControl|DelayUntilNextTick)
    (CallFunction|FacePlayer)))

(event Custom|Patrol
  ;[0.15 0.15 0.15 0.5] Custom Events
  ;;[0.15 0.15 0.15 0.5] Movement Events
  (AI|AIMoveTo 0 (Utilities|Array|Get(acopy) (Variables|AIMoveParams|GetPatrolPoints) (Variables|AIMoveParams|GetCurrentPointIndex)) 0 2.5e+02 false
    (:OnSuccess
      (bind _result (Math|Integer|IncrementInt (Variables|AIMoveParams|GetCurrentPointIndex))
        (:%20%20
          (if (> _result (Utilities|Array|Length (Variables|AIMoveParams|GetPatrolPoints)))
            (Variables|AIMoveParams|SetCurrentPointIndex 0))
          (CallFunction|Patrol))))))

(event EventBeginPlay
  ;[0.15 0.15 0.15 0.5] BeginPlay
  (Variables|InitialValues|SetSpawnPosition (Transformation|GetActorLocation))
  (Variables|InitialValues|SetSpawnRotation (Transformation|GetActorRotation))
  (bind _returnvalue (Rendering|Material|CreateDynamicMaterialInstance (Variables|Outliner|GetOutlinerMaterial) "None" "None" :!class /Script/Engine.KismetMaterialLibrary))
  (bind _output_get (Variables|Outliner|SetOutlinerInstance _returnvalue))
  (Rendering|Material|SetOverlayMaterial (Variables|Character|GetMesh) _output_get :!class /Script/Engine.MeshComponent))

(event EventOnHorrorLoaded
  ;[0.15 0.15 0.15 0.5] Interfaces
  ;;[0.15 0.15 0.15 0.5] Change Materials on world load
  (Rendering|Material|SetMaterial (Variables|Character|GetMesh) 0 (Variables|Default|GetHorror%20Material)))

(event EventOnCuteLoaded
  ;[0.15 0.15 0.15 0.5] Interfaces
  ;;[0.15 0.15 0.15 0.5] Change Materials on world load
  (Rendering|Material|SetMaterial (Variables|Character|GetMesh) 0 (Variables|Default|GetCute%20Material)))

(event EventOnInteract
  (params (InteractedPlayer :type BP%20Playable%20Character%20Object%20Reference))
  ;[0.15 0.15 0.15 0.5] Interfaces
  ;;[0.15 0.15 0.15 0.5] Assign transformation class on interact
  (Default|AssignTransform (.AsYako%20Taki%20Game%20Mode (Utilities|Casting|CastToYakoTakiGameMode (Game|GetGameMode))) (Variables|PlayableCharacterRelated|Transformation|GetTransform%20Class)))

(fn ConstructionScript
  (bind _transformationeffect (Variables|Default|GetTransformationEffect))
  (if (Variables|PlayableCharacterRelated|Transformation|GetCanGiveTransformation)
    (Components|Activation|SetAutoActivate _transformationeffect true)
    (else
      (Components|Activation|SetAutoActivate _transformationeffect false))))