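; Illumination citizen Blueprint that switches the character's look between a cute and a horror version.
; On the cute-loaded and horror-loaded events, it assigns the matching fire Niagara effect to the Head component, resetting parameter overrides.
; The same events swap the skeletal mesh's head and body materials to that version.
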(event EventBeginPlay
  (|CallParentFunction) ; This node is disabled and will not be called.\nDrag off pins to build functionality.
)

(event Collision|EventActorBeginOverlap
  (params (OtherActor :type Actor%20Object%20Reference))
  (|CallParentFunction OtherActor) ; This node is disabled and will not be called.\nDrag off pins to build functionality.
)

(event EventTick
  (params (DeltaSeconds :type Float%20%28single-precision%29))
  (|CallParentFunction DeltaSeconds) ; This node is disabled and will not be called.\nDrag off pins to build functionality.
)

(event EventOnCuteLoaded
  (bind _skeletalmesh (Variables|Default|GetSkeletalMesh))
  (Class|NiagaraComponent|SetAsset (Variables|Default|GetHead) "/Game/Project/00_Generic/Assets/VFX/FireHead/FXS_FireCitizen_c.FXS_FireCitizen_c" true)
  (Rendering|Material|SetMaterial _skeletalmesh 0 "/Game/Project/00_Generic/Assets/Citizens/Candle/MI_Head_c.MI_Head_c")
  (Rendering|Material|SetMaterial _skeletalmesh 1 "/Game/Project/00_Generic/Assets/Citizens/Candle/MI_Body_c.MI_Body_c"))

(event EventOnHorrorLoaded
  (bind _skeletalmesh (Variables|Default|GetSkeletalMesh))
  (Class|NiagaraComponent|SetAsset (Variables|Default|GetHead) "/Game/Project/00_Generic/Assets/VFX/FireHead/FXS_FireCitizen_h.FXS_FireCitizen_h" true)
  (Rendering|Material|SetMaterial _skeletalmesh 0 "/Game/Project/00_Generic/Assets/Citizens/Candle/MI_Head_h.MI_Head_h")
  (Rendering|Material|SetMaterial _skeletalmesh 1 "/Game/Project/00_Generic/Assets/Citizens/Candle/MI_Body_h.MI_Body_h"))

(fn ConstructionScript
  (|CallParentFunction))