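; AC_InputBuffer is an actor component that buffers a single player input for later execution, keeping only the latest one rather than a queue.
; StoreNextInput saves a valid Input Action with a timestamp.
; ExecuteNextAction asks the owner via interface whether buffering is allowed and checks the BufferTime window, then replays the action through Enhanced Input injection on player 0 with a fixed value, and clears it.
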(event Custom|ExecuteNextAction
  (bind _returnvalue (Utilities|Time|GetGameTimeinSeconds))
  (bind _inputstoredtime (Variables|Default|GetInputStoredTime))
  ;[0.15 0.15 0.15 0.5] Use a Interface to Input buffer and not a Queue because we just want store a one Input and can change the condition to activate input Buffer for BP_DJ
  (bind _bool (Class|BIBufferExecutable|CanExecuteBuffer(Message) (Components|GetOwner)))
  (Development|PrintString (Utilities|String|Append "Game: " (Utilities|String|ToString(Float) _returnvalue)))
  (Development|PrintString (Utilities|String|Append "Stored: " (Utilities|String|ToString(Float) _inputstoredtime)))
  (if (and _bool (<= (- _returnvalue _inputstoredtime) (Variables|Default|GetBuffer%20Time)))
    (Class|EnhancedInputSubsystemInterface|InjectInputVectorforAction (PlayerController|LocalPlayerSubsystems|GetEnhancedInputLocalPlayerSubsystem (Game|GetPlayerController 0)) (Variables|Default|GetInputToStore) "20.000000,20.000000,20.000000")
    (Variables|Default|SetInputToStore 0)
    (else
      (Variables|Default|SetInputToStore 0))))

(fn StoreNextInput
  (params (InputToStore :type Input%20Action%20Object%20Reference) (Input%20Value :type Input%20Action%20Value%20Structure))
  ;[0.15 0.15 0.15 0.5] Store Input and inicialize the Input stored time
  (Utilities|IsValid InputToStore
    (:Is%20Valid
      (Variables|Default|SetInputToStore InputToStore)
      (Variables|Default|SetInputStoredTime (Utilities|Time|GetGameTimeinSeconds)))
    (:Is%20Not%20Valid
      (Variables|Default|SetInputToStore 0))))