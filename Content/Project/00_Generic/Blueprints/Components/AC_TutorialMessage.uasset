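; Tutorial message component that shows an on-screen tutorial and dismisses it when its tutorial key is pressed.
; InitializeTutorial takes the player controller's shared widget, fills it with content blocks from the DT_TutorialsEntries row named by TutorialName, and shows it.
; A player-controller key event hides the widget on a match and unbinds itself, while FinishTutorial hides it and clears the reference.
; CreateText and CreateImage are empty, with their default-block logic disconnected.
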(event Custom|CheckTutorialComplete
  (params (Input :type Input%20Action%20Object%20Reference))
  ;[0.15 0.15 0.15 0.5] Check if input press is the same to complete the tutorial
  (if (== Input (Variables|Default|GetTutorial%20Key))
    (bind _wbp_tutorial_reference (Variables|Default|GetWBP_Tutorial%20Reference)
      (:then
        (Default|HideWidget _wbp_tutorial_reference)
        (EventDispatchers|UnbindEventfromOnTutorialKeyPressed (.AsBP%20Player%20Controller (Utilities|Casting|CastToBP_PlayerController (Game|GetPlayerController 0))) (delegate Custom|CheckTutorialComplete))
        (Variables|Default|GetWBP_Tutorial%20Reference
          (:then)
          (:else)))
      (:else))))

(event EventTick
  (params (DeltaSeconds :type Float%20%28single-precision%29)))

(event EventBeginPlay
  ;[0.15 0.15 0.15 0.5] Check if input press is the same to complete the tutorial
  (EventDispatchers|BindEventtoOnTutorialKeyPressed (.AsBP%20Player%20Controller (Utilities|Casting|CastToBP_PlayerController (Game|GetPlayerController 0))) (delegate Custom|CheckTutorialComplete)))

(fn SetWidgetContent
  (params (Name :type Name))
  ;[0.15 0.15 0.15 0.5] Pass the content of Blueprint to widget
  (bind _asbp_player_controller (Utilities|Casting|CastToBP_PlayerController (Game|GetPlayerController 0)))
  (bind _wbp_tutorial_ref (Variables|/Game/Project/00_Generic/Blueprints/PlayerController/BP_PlayerController.BP_PlayerController_C|GetWBP%20Tutorial%20Ref _asbp_player_controller)
    (:then
      (bind _output_get (Variables|Default|SetWBP_Tutorial%20Reference _wbp_tutorial_ref))
      (bind _returnvalue (Utilities|GetDataTableRow "/Game/Project/00_Generic/Blueprints/Tables/DT_TutorialsEntries.DT_TutorialsEntries" Name)
        (:then
          (Variables|/Game/Project/00_Generic/Blueprints/UI_HUD/WBP_TutorialMessages.WBP_TutorialMessages_C|SetVertical%20Box%20Blocks _output_get (.tutorialContents (Utilities|Struct|BreakTutorialEntry _returnvalue))))))
    (:else)))

(fn CreateText
  ;[0.15 0.15 0.15 0.5] Add the Text with parameters default in blocks array
)

(fn CreateImage
  ;[0.15 0.15 0.15 0.5] Add the Image with parameters default in blocks array
)

(fn InitializeTutorial
  ;[0.15 0.15 0.15 0.5] Initialize the tutorial
  (Variables|Default|GetWBP_Tutorial%20Reference
    (:then)
    (:else
      (CallFunction|SetWidgetContent (Variables|Default|GetTutorialName))
      (Default|ShowWidget&UpdateWrap (Variables|Default|GetWBP_Tutorial%20Reference)))))

(fn FinishTutorial
  (bind _wbp_tutorial_reference (Variables|Default|GetWBP_Tutorial%20Reference)
    (:then
      (Default|HideWidget _wbp_tutorial_reference)
      (Variables|Default|SetWBP_Tutorial%20Reference 0))
    (:else)))