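; Scene component that gives its owning actor a screen-space dialogue widget and drives a talking face.
; On BeginPlay it creates the widget hidden, plus a dynamic material from the owner's static mesh, rebuilt when the Horror or Cute world loads.
; Speak shows the widget or advances dialogue; NextText sends each line, sets its face-index parameter, then auto-advances after a length-based delay.
; StopSpeak resets the index and plays another widget animation.
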(event Custom|NextText
  ;[0.15 0.15 0.15 0.5] Custom Events
  ;;[0.15 0.15 0.15 0.5] Advance the position in struct array with Text and Face Index, and send the message to Interface
  (if (and (< (Variables|Default|GetDialogueIndex) (Utilities|Array|Length (Variables|Default|GetDialogues))) (Variables|Default|GetIsSpeaking))
    (bind _output_get (Variables|Default|SetCurrentMessage (.text (Utilities|Array|Get(acopy) (Variables|Default|GetDialogues) (Variables|Default|GetDialogueIndex)))))
    (Class|BISpeakable|Talk(Message) (Variables|Default|GetWidgetReference) _output_get)
    (Rendering|Material|SetScalarParameterValue (Variables|Default|GetDynamic%20Material%20Ref) (Variables|Default|GetMI%20Parameter%20Name) (.faceindex (Utilities|Array|Get(acopy) (Variables|Default|GetDialogues) (Variables|Default|GetDialogueIndex))) :!class /Script/Engine.MaterialInstanceDynamic)
    (bind _output_get_2 (Variables|Default|SetDialogueIndex (+ (Variables|Default|GetDialogueIndex) 1)))
    (if (not (>= _output_get_2 (Utilities|Array|Length (Variables|Default|GetDialogues))))
      (Utilities|FlowControl|Delay (* (Utilities|String|Len (Utilities|String|ToString(Text) (Variables|Default|GetCurrentMessage))) 0.12))
      (CallFunction|NextText))))

(event Custom|Recharge%20Dynamic%20Material
  (bind _returnvalue (Components|GetOwner))
  (bind _returnvalue_2 (Actor|GetComponentbyClass _returnvalue "/Script/Engine.StaticMeshComponent"))
  ;[0.15 0.15 0.15 0.5] Custom Events
  ;;[0.15 0.15 0.15 0.5] Recharge Dynamic material to World change
  (bind _returnvalue_3 (Rendering|Material|CreateDynamicMaterialInstance _returnvalue_2 0 (Rendering|Material|GetMaterial _returnvalue_2 0) "FaceIndex" :!class /Script/Engine.PrimitiveComponent))
  (Variables|Default|SetDynamic%20Material%20Ref _returnvalue_3))

(event EventBeginPlay
  ;[0.15 0.15 0.15 0.5] Setup variables and Widget in Scene
  (bind _returnvalue (Game|AddComponentbyClass (Components|GetOwner) "/Script/UMG.WidgetComponent" false))
  (bind _output_get (Variables|Default|SetWidgetComponentReference _returnvalue))
  (Transformation|AttachComponentToComponent _output_get self "None" "KeepRelative" "KeepRelative" "KeepRelative" true)
  (Class|WidgetComponent|SetWidgetSpace (Variables|Default|GetWidgetComponentReference) "Screen")
  (bind _returnvalue_2 (UserInterface|CreateWidget (Variables|Default|GetWidgetClass) (Game|GetPlayerController 0)))
  (Variables|Default|SetWidgetReference _returnvalue_2)
  (UserInterface|SetWidget (Variables|Default|GetWidgetComponentReference) (Variables|Default|GetWidgetReference))
  (Widget|SetVisibility (Variables|Default|GetWidgetReference) "Hidden")
  (CallFunction|RechargeDynamicMaterial))

(event EventOnHorrorLoaded
  ;[0.15 0.15 0.15 0.5] Recharge MDI on World loaded
  (CallFunction|RechargeDynamicMaterial))

(event EventOnCuteLoaded
  ;[0.15 0.15 0.15 0.5] Recharge MDI on World loaded
  (CallFunction|RechargeDynamicMaterial))

(fn Speak
  (bind _widgetreference (Variables|Default|GetWidgetReference))
  ;[0.15 0.15 0.15 0.5] Check array messages and is speaking to do a Next Text or Show WBP
  (if (> (Utilities|Array|Length (Variables|Default|GetDialogues)) 0)
    (if (Variables|Default|GetIsSpeaking)
      (CallFunction|NextText)
      (else
        (Variables|Default|SetDialogueIndex 0)
        (Variables|Default|SetIsSpeaking true)
        (Widget|SetVisibility _widgetreference "SelfHitTestInvisible")
        (Class|BISpeakable|DialogueAnimation(Message) _widgetreference "NewEnumerator1")
        (CallFunction|NextText)))))

(fn StopSpeak
  ;[0.15 0.15 0.15 0.5] Stop Dialogue
  (if (Variables|Default|GetIsSpeaking)
    (Variables|Default|SetDialogueIndex 0)
    (Variables|Default|SetIsSpeaking false)
    (Class|BISpeakable|DialogueAnimation(Message) (Variables|Default|GetWidgetReference) "NewEnumerator0")))