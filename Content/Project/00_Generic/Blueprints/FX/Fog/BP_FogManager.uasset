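; Level fog manager that fades a fog effect and turns the player back when they go too deep.
; On BeginPlay it puts a dynamic M_Fog material on FogActor and binds the overlaps of every BP_FogTrigger and BP_DeepFogTrigger.
; Fog triggers fade opacity and count overlaps, saving the player's transform on first entry.
; Deep triggers lock controls, thicken fog, teleport the player to that spot facing back, then restore controls.
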(event Custom|FogActivatorsSetter
  (bind _returnvalue (Rendering|Material|CreateDynamicMaterialInstance "/Game/Project/00_Generic/Assets/VFX/Fog/M_Fog.M_Fog" "None" "None" :!class /Script/Engine.KismetMaterialLibrary))
  (bind _output_get (Variables|Default|SetFogMaterialInstance _returnvalue))
  (Rendering|Material|SetMaterial (Variables|/Script/Engine.StaticMeshActor|GetStaticMeshComponent (Variables|Default|GetFogActor)) 0 _output_get)
  (Rendering|Material|SetScalarParameterValue _output_get "Opacidad" 0.0 :!class /Script/Engine.MaterialInstanceDynamic)
  (bind _outactors (Actor|GetAllActorsOfClass "/Game/Project/00_Generic/Blueprints/FX/Fog/BP_FogTrigger.BP_FogTrigger_C"))
  (for _array_element _outactors
    (Collision|AssignOnComponentBeginOverlap (Variables|/Game/Project/00_Generic/Blueprints/FX/Fog/BP_FogTrigger.BP_FogTrigger_C|GetBox _array_element) (delegate Custom|OnComponentBeginOverlap_Event))
    (Collision|AssignOnComponentEndOverlap (Variables|/Game/Project/00_Generic/Blueprints/FX/Fog/BP_FogTrigger.BP_FogTrigger_C|GetBox _array_element) (delegate Custom|OnComponentEndOverlap_Event)))
  (bind _outactors_2 (Actor|GetAllActorsOfClass "/Game/Project/00_Generic/Blueprints/FX/Fog/BP_DeepFogTrigger.BP_DeepFogTrigger_C"))
  (for _array_element_2 _outactors_2
    ;[0.15 0.15 0.15 0.5] Restores player
    (Collision|AssignOnComponentBeginOverlap (Variables|/Game/Project/00_Generic/Blueprints/FX/Fog/BP_DeepFogTrigger.BP_DeepFogTrigger_C|GetBox _array_element_2) (delegate Custom|OnComponentBeginOverlap_Event_0))))

(event Custom|OnComponentBeginOverlap_Event
  (params (OverlappedComponent :type Primitive%20Component%20Object%20Reference) (OtherActor :type Actor%20Object%20Reference) (OtherComp :type Primitive%20Component%20Object%20Reference) (OtherBodyIndex :type Integer) (bFromSweep :type Boolean) (SweepResult :type Hit%20Result%20Structure%20%28by%20ref%29))
  ;[0.15 0.15 0.15 0.5] Manages if player switches between fog colliders
  (bind _asbp_playable_character (Utilities|Casting|CastToBP_PlayableCharacter OtherActor))
  (CallFunction|TrySetReturnPosition _asbp_playable_character)
  (bind _result (Math|Integer|IncrementInt (Variables|Default|GetFog%20Boxes%20Collied))
    (:%20%20
      (Development|PrintString (Utilities|String|Append "Enter fog: " (Utilities|String|ToString(Integer) _result)))
      (bind _fogvalue (Timeline|FogEffeectTimeline Reverse)
        (:Update
          (Rendering|Material|SetScalarParameterValue (Variables|Default|GetFogMaterialInstance) "Opacidad" (Math|Float|Lerp 0.0 0.2 _fogvalue) :!class /Script/Engine.MaterialInstanceDynamic))))))

(event Custom|OnComponentEndOverlap_Event
  (params (OverlappedComponent :type Primitive%20Component%20Object%20Reference) (OtherActor :type Actor%20Object%20Reference) (OtherComp :type Primitive%20Component%20Object%20Reference) (OtherBodyIndex :type Integer))
  ;[0.15 0.15 0.15 0.5] Manages if player switches between fog colliders
  (Utilities|Casting|CastToBP_PlayableCharacter OtherActor)
  (bind _result (Math|Integer|DecrementInt (Variables|Default|GetFog%20Boxes%20Collied))
    (:%20%20
      (Development|PrintString (Utilities|String|Append "Exit fog: " (Utilities|String|ToString(Integer) _result)))
      (bind _fogvalue (Timeline|FogEffeectTimeline Play)
        (:Update
          (Rendering|Material|SetScalarParameterValue (Variables|Default|GetFogMaterialInstance) "Opacidad" (Math|Float|Lerp 0.0 0.2 _fogvalue) :!class /Script/Engine.MaterialInstanceDynamic))))))

(event Custom|TrySetReturnPosition
  (params (Character :type BP%20Playable%20Character%20Object%20Reference))
  ;[0.15 0.15 0.15 0.5] If player hass not collied with any, saves rotation and position
  (if (== (Variables|Default|GetFog%20Boxes%20Collied) 0)
    (Variables|Default|SetPlayerEnterLocation (Transformation|GetActorLocation Character))
    (Variables|Default|SetPlayerEnterRotation (Transformation|GetActorRotation Character))))

(event Custom|OnComponentBeginOverlap_Event_0
  (params (OverlappedComponent :type Primitive%20Component%20Object%20Reference) (OtherActor :type Actor%20Object%20Reference) (OtherComp :type Primitive%20Component%20Object%20Reference) (OtherBodyIndex :type Integer) (bFromSweep :type Boolean) (SweepResult :type Hit%20Result%20Structure%20%28by%20ref%29))
  (bind _playerenterrotation (Variables|Default|GetPlayerEnterRotation))
  (bind _returnvalue (+ (.yaw _playerenterrotation) 1.8e+02))
  (bind _returnvalue_2 (Math|Rotator|MakeRotator (.roll _playerenterrotation) (.pitch _playerenterrotation) _returnvalue))
  ;[0.15 0.15 0.15 0.5] Restores player
  (bind _asbp_playable_character (Utilities|Casting|CastToBP_PlayableCharacter OtherActor))
  (Variables|/Game/Project/00_Generic/Blueprints/PlayableCharacters/BP_PlayableCharacter.BP_PlayableCharacter_C|SetCanExecuteTransform _asbp_playable_character false)
  (Default|SetCanMoveandJump _asbp_playable_character false)
  (Variables|/Game/Project/00_Generic/Blueprints/PlayableCharacters/BP_PlayableCharacter.BP_PlayableCharacter_C|SetCanRotateCamera _asbp_playable_character false)
  (bind _value (Timeline|DeepFogTimeline PlayFromStart)
    (:Update
      (Rendering|Material|SetScalarParameterValue (Variables|Default|GetFogMaterialInstance) "Opacidad" (Math|Float|Lerp 0.2 0.8 _value) :!class /Script/Engine.MaterialInstanceDynamic))
    (:Finished
      (Pawn|SetControlRotation (Pawn|GetController _asbp_playable_character) _returnvalue_2)
      (Utilities|FlowControl|Delay 0.275)
      (Transformation|SetActorLocationAndRotation _asbp_playable_character (Variables|Default|GetPlayerEnterLocation) _returnvalue_2 false true)
      (Variables|/Game/Project/00_Generic/Blueprints/PlayableCharacters/BP_PlayableCharacter.BP_PlayableCharacter_C|SetCanExecuteTransform _asbp_playable_character true)
      (Default|SetCanMoveandJump _asbp_playable_character true)
      (Variables|/Game/Project/00_Generic/Blueprints/PlayableCharacters/BP_PlayableCharacter.BP_PlayableCharacter_C|SetCanRotateCamera _asbp_playable_character true)
      (Timeline|ToNormalTimeline Play
        (:Update
          (Rendering|Material|SetScalarParameterValue (Variables|Default|GetFogMaterialInstance) "Opacidad" 0.0 :!class /Script/Engine.MaterialInstanceDynamic))))))

(event EventBeginPlay
  (CallFunction|FogActivatorsSetter))

(fn ConstructionScript)