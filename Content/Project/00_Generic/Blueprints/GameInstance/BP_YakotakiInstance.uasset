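; Game instance for Yakotaki that holds state and services for saves, settings, screen fades and respawn checkpoints.
; On Init it loads or creates the player save, applies user settings and saved volumes through audio buses, a VCA and sound mix overrides, and creates a hidden fade widget.
; It tracks the active checkpoint and returns its spawn transform, falling back to the level's default start, then the first PlayerStart.
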(event EventInit
  (Saving|LoadSaveFile)
  (CallFunction|LoadApplySavedSettings)
  (Variables|Default|SetMainMenuWidgetClass "/Game/Project/00_Generic/Blueprints/UI_HUD/WBP_MainMenu.WBP_MainMenu_C")
  (Variables|Default|GetFadeWRef
    (:then)
    (:else
      (bind _returnvalue (UserInterface|CreateWidget "/Game/Project/00_Generic/Blueprints/UI_HUD/WBP_Fade.WBP_Fade_C"))
      (Variables|Default|SetFadeWRef _returnvalue)
      (Widget|SetVisibility _returnvalue "Hidden"))))

(fn Show/HidePrintString
  (if (Variables|Default|GetShowStrings)
    (Development|ExecuteConsoleCommand "Enableallscreenmessages" 0)
    (else
      (Development|ExecuteConsoleCommand "Disableallscreenmessages" 0))))

(fn Fadein
  (bind _fadewref (Variables|Default|GetFadeWRef))
  (Widget|SetVisibility _fadewref "Visible")
  (Default|PlayFadein _fadewref))

(fn FadeOut
  (Default|PlayFadeOut (Variables|Default|GetFadeWRef)))

(fn SetCheckpoint
  (params (NewCheckpoint :type BP%20Chek%20Points%20Horror%20Object%20Reference))
  (Utilities|IsValid (Variables|Default|GetCurrentActiveCheckpoint)
    (:Is%20Valid
      _)
    (:Is%20Not%20Valid
      _))
  (bind _output_get (Variables|Default|SetCurrentActiveCheckpoint NewCheckpoint))
  (Default|FlagUp _output_get))

(fn GetCheckpointLocationandRotation
  (bind _returnvalue (Class|DualLevelFunctionLibrary|GetDualLevel))
  (bind _currentactivecheckpoint (Variables|Default|GetCurrentActiveCheckpoint))
  (bind _defaultplayerstart (Variables|/Script/Yakotaki.DualLevel|GetDefaultPlayerStart _returnvalue))
  (bind _spawndirection (Variables|/Game/Project/00_Generic/Blueprints/Others/BP_ChekPoints_Horror.BP_ChekPoints_Horror_C|GetSpawnDirection _currentactivecheckpoint))
  (Utilities|IsValid _currentactivecheckpoint
    (:Is%20Valid
      (LocalVariables|SetTargetLocation (Transformation|GetWorldLocation _spawndirection))
      (LocalVariables|SetTargetRotation (Transformation|GetWorldRotation _spawndirection))
      (return (LocalVariables|GetTargetLocation) (LocalVariables|GetTargetRotation)))
    (:Is%20Not%20Valid
      (Utilities|IsValid _defaultplayerstart
        (:Is%20Valid
          (LocalVariables|SetTargetLocation (Transformation|GetActorLocation _defaultplayerstart))
          (LocalVariables|SetTargetRotation (Transformation|GetActorRotation _defaultplayerstart))
          (return (LocalVariables|GetTargetLocation) (LocalVariables|GetTargetRotation)))
        (:Is%20Not%20Valid
          (bind _outactors (Actor|GetAllActorsOfClass "/Script/Engine.PlayerStart"))
          (LocalVariables|SetTargetLocation (Transformation|GetActorLocation (Utilities|Array|Get(acopy) _outactors)))
          (LocalVariables|SetTargetRotation (Transformation|GetActorRotation (Utilities|Array|Get(acopy) _outactors)))
          (return (LocalVariables|GetTargetLocation) (LocalVariables|GetTargetRotation)))))))

(fn LoadApplySavedSettings
  (bind _returnvalue (Settings|GetGameUserSettings))
  (Class|GameUserSettings|ApplySettings _returnvalue false)
  (bind _returnvalue_2 (SaveGame|LoadGamefromSlot "GameSettings"))
  (bind _asoptions_save_game (Utilities|Casting|CastToOptionsSaveGame _returnvalue_2))
  (Class|FMODBlueprintStatics|BusSetVolume "/Game/FMOD/Buses/Music.Music" (/ (Variables|/Game/Project/00_Generic/Blueprints/SaveGame/OptionsSaveGame.OptionsSaveGame_C|GetMusicVolume _asoptions_save_game) 1e+02))
  (Audio|SetSoundMixClassOverride "/Game/Project/00_Generic/Blueprints/SoundClass/GameSoundMix.GameSoundMix" "/Game/Project/00_Generic/Blueprints/SoundClass/GameMusic.GameMusic" (/ (Variables|/Game/Project/00_Generic/Blueprints/SaveGame/OptionsSaveGame.OptionsSaveGame_C|GetMusicVolume _asoptions_save_game) 1e+02) 1.0 1.0 true)
  (Class|FMODBlueprintStatics|BusSetVolume "/Game/FMOD/Buses/SFX.SFX" (/ (Variables|/Game/Project/00_Generic/Blueprints/SaveGame/OptionsSaveGame.OptionsSaveGame_C|GetFXVolume _asoptions_save_game) 1e+02))
  (Audio|SetSoundMixClassOverride "/Game/Project/00_Generic/Blueprints/SoundClass/GameSoundMix.GameSoundMix" "/Game/Project/00_Generic/Blueprints/SoundClass/GameMusic.GameMusic" (/ (Variables|/Game/Project/00_Generic/Blueprints/SaveGame/OptionsSaveGame.OptionsSaveGame_C|GetFXVolume _asoptions_save_game) 1e+02) 1.0 1.0 true)
  (Class|FMODBlueprintStatics|VCASetVolume "/Game/FMOD/VCAs/General.General" (/ (Variables|/Game/Project/00_Generic/Blueprints/SaveGame/OptionsSaveGame.OptionsSaveGame_C|GetGeneralSound _asoptions_save_game) 1e+02))
  (Audio|SetSoundMixClassOverride "/Game/Project/00_Generic/Blueprints/SoundClass/GameSoundMix.GameSoundMix" 0 (/ (Variables|/Game/Project/00_Generic/Blueprints/SaveGame/OptionsSaveGame.OptionsSaveGame_C|GetGeneralSound _asoptions_save_game) 1e+02) 1.0 1.0 true))

(fn LoadSaveFile
  (bind _returnvalue (SaveGame|LoadGamefromSlot "player"))
  (Utilities|IsValid _returnvalue
    (:Is%20Valid
      (bind _asyakotaki_save_game (Utilities|Casting|CastToYakotakiSaveGame _returnvalue)
        (:then
          (Variables|Default|SetSaveFile _asyakotaki_save_game))
        (:CastFailed
          (bind _returnvalue_2 (SaveGame|CreateSaveGameObject "/Script/Yakotaki.YakotakiSaveGame" :!label _label))
          (Variables|Default|SetSaveFile _returnvalue_2))))
    (:Is%20Not%20Valid
      (goto _label))))

(fn SaveGameFile
  (bind _savefile (Variables|Default|GetSaveFile))
  (Utilities|IsValid _savefile
    (:Is%20Valid
      (SaveGame|SaveGametoSlot _savefile "player"))))