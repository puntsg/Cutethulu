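; Main menu game mode that creates the main and options menu widgets and applies saved settings on BeginPlay.
; Options starts hidden; two events swap visibility and enabled state between the menus and hand UINav focus to the active widget.
; Settings loading applies user settings, then sets sound mix volumes from the GameSettings save slot.
; The saved volumes are crossed: MusicVolume drives the SFX class and FXVolume drives music.
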(event Custom|OptionsToMenu
  (bind _optionsmenu (Variables|Default|GetOptionsMenu))
  (bind _menu (Variables|Default|Getmenu))
  ;[0.15 0.15 0.15 0.5] Open/close options menu
  (Widget|SetIsEnabled _optionsmenu false)
  (Widget|SetVisibility _optionsmenu "Hidden")
  (Widget|SetIsEnabled _menu true)
  (Widget|SetVisibility _menu "Visible")
  (Class|UINavPCComponent|SetActiveWidget (Actor|GetComponentbyClass (Game|GetPlayerController 0) "/Script/UINavigation.UINavPCComponent") _menu))

(event Custom|MenuToOptions
  (bind _optionsmenu (Variables|Default|GetOptionsMenu))
  (bind _menu (Variables|Default|Getmenu))
  ;[0.15 0.15 0.15 0.5] Open/close options menu
  (Widget|SetIsEnabled _optionsmenu true)
  (Widget|SetVisibility _optionsmenu "Visible")
  (Default|SetOptionsMenuVisibility _optionsmenu true false false false false)
  (Widget|SetIsEnabled _menu false)
  (Widget|SetVisibility _menu "Hidden")
  (Class|UINavPCComponent|SetActiveWidget (Actor|GetComponentbyClass (Game|GetPlayerController 0) "/Script/UINavigation.UINavPCComponent") _optionsmenu))

(event Custom|Load%20game%20settings
  ;[0.15 0.15 0.15 0.5] Load graphics and audio settings
  (bind _returnvalue (Settings|GetGameUserSettings))
  (Class|GameUserSettings|ApplySettings _returnvalue false)
  (bind _returnvalue_2 (SaveGame|LoadGamefromSlot "GameSettings"))
  (bind _asoptions_save_game (Utilities|Casting|CastToOptionsSaveGame _returnvalue_2))
  (Audio|SetSoundMixClassOverride "/Game/Project/00_Generic/Blueprints/SoundClass/GameSoundMix.GameSoundMix" "/Game/Project/00_Generic/Blueprints/SoundClass/GameSFX.GameSFX" (/ (Variables|/Game/Project/00_Generic/Blueprints/SaveGame/OptionsSaveGame.OptionsSaveGame_C|GetMusicVolume _asoptions_save_game) 1e+02) 1.0 1.0 true)
  (Audio|SetSoundMixClassOverride "/Game/Project/00_Generic/Blueprints/SoundClass/GameSoundMix.GameSoundMix" "/Game/Project/00_Generic/Blueprints/SoundClass/GameMusic.GameMusic" (/ (Variables|/Game/Project/00_Generic/Blueprints/SaveGame/OptionsSaveGame.OptionsSaveGame_C|GetFXVolume _asoptions_save_game) 1e+02) 1.0 1.0 true)
  (Audio|PushSoundMixModifier "/Game/Project/00_Generic/Blueprints/SoundClass/GameSoundMix.GameSoundMix"))

(event EventBeginPlay
  ;[0.15 0.15 0.15 0.5] Init main menu
  (bind _returnvalue (UserInterface|CreateWidget "/Game/Project/00_Generic/Blueprints/UI_HUD/WBP_MainMenu.WBP_MainMenu_C"))
  (bind _output_get (Variables|Default|Setmenu _returnvalue))
  (UserInterface|Viewport|AddtoViewport _output_get 0)
  (bind _returnvalue_2 (UserInterface|CreateWidget "/Game/Project/00_Generic/Blueprints/UI_HUD/WBP_OptionsMenu.WBP_OptionsMenu_C"))
  (bind _output_get_2 (Variables|Default|SetOptionsMenu _returnvalue_2))
  (Widget|SetVisibility _output_get_2 "Hidden")
  (UserInterface|Viewport|AddtoViewport _output_get_2 0)
  (CallFunction|LoadGameSettings))

(fn ConstructionScript)