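; Game mode that sets up the player HUD, collectables widget and loading screen, and coordinates creature transformations and world healing.
; AssignTransform finds or spawns a creature, triggering the pawn's Transform, while transform events refresh HUD icons.
; HealWorld locks player control, darkens the world through a player-positioned material parameter collection, swaps the dual level, then reverses the fade on load.
; PlayerTransition blends the menu camera into the follow camera and changes music.
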(event Custom|OnPlayerTransform_Event
  (params (CurrentPlayableCharacter :type BP%20Playable%20Character%20Object%20Reference) (CharacterToTransform :type BP%20Playable%20Character%20Object%20Reference))
  (bind _playerui (Variables|UI|GetPlayerUI))
  (Utilities|Casting|CastToBP_PlayerDefault_Taki CurrentPlayableCharacter
    (:then
      _)
    (:CastFailed
      (Variables|Gameplay|SetTransformation CurrentPlayableCharacter)))
  (bind _output_get (Variables|Gameplay|SetCurrentCharacter CharacterToTransform))
  ;[0.15 0.15 0.15 0.5] Assign icons to hud
  (Default|AssignCurrentCreatureIcon (Variables|UI|GetPlayerUI) (.transformationicon (Variables|/Game/Project/00_Generic/Blueprints/PlayableCharacters/BP_PlayableCharacter.BP_PlayableCharacter_C|GetCharacterData _output_get)))
  (if (!= (Utilities|GetClass (Variables|Gameplay|GetCurrentCharacter)) (Utilities|GetClass (Variables|Gameplay|GetTransformation)))
    (Default|AssignTransformationCreatureIcon _playerui (.transformationicon (Variables|/Game/Project/00_Generic/Blueprints/PlayableCharacters/BP_PlayableCharacter.BP_PlayableCharacter_C|GetCharacterData (Variables|Gameplay|GetTransformation))))
    (else
      (Default|AssignTransformationCreatureIcon _playerui "/Game/Project/00_Generic/Assets/UI_Textures/T_Icon_empty.T_Icon_empty"))))

(event Custom|ResetTransformations)

(event Custom|OnTransformAcquired_Event
  (params (AcquiredTransform :type BP%20Playable%20Character%20Object%20Reference))
  (bind _returnvalue (Game|Player|GetPlayerPawn 0))
  (bind _asbp_playable_character (Utilities|Casting|CastToBP_PlayableCharacter _returnvalue))
  (bind _cantransform (Default|CanTransform _asbp_playable_character))
  (if _cantransform
    (Default|Transform _asbp_playable_character AcquiredTransform)))

(event Custom|PlayerTransition
  (bind _returnvalue (Game|GetPlayerController 0))
  (bind _returnvalue_2 (Game|Player|GetPlayerPawn 0))
  (bind _currentsoundplayer (Variables|Default|GetCurrentSoundPlayer))
  (bind _cameramainmenu (Variables|Default|GetcameraMainMenu))
  (bind _newtrack_0 (Timeline|Timeline Play)
    (:Update
      (bind _asbp_player_default_taki (Utilities|Casting|CastToBP_PlayerDefault_Taki (Game|Player|GetPlayerPawn 0)))
      (Transformation|SetWorldTransform _cameramainmenu (Math|Transform|Lerp(Transform) (Transformation|GetWorldTransform _cameramainmenu) (Transformation|GetWorldTransform (Variables|/Game/Project/00_Generic/Blueprints/PlayableCharacters/BP_PlayableCharacter.BP_PlayableCharacter_C|GetFollowCamera _asbp_player_default_taki)) _newtrack_0) true false)
      (Class|CameraComponent|SetPostProcessBlendWeight (Variables|Default|GetcameraMainMenu) _newtrack_0)
      (Audio|Components|Audio|FadeOut _currentsoundplayer 0.2 0.0 "Linear" :!class /Script/Engine.AudioComponent)
      (Utilities|FlowControl|Delay 0.2)
      (Audio|Components|Audio|SetSound _currentsoundplayer "/Game/Project/00_Generic/Assets/Sounds/SoundWaves_Cues/SW_CuteMusic.SW_CuteMusic"))
    (:Finished
      (Input|EnableInput _returnvalue _returnvalue)
      (Transformation|ResetRelativeTransform (Variables|/Game/Project/00_Generic/Blueprints/PlayableCharacters/BP_PlayableCharacter.BP_PlayableCharacter_C|GetFollowCamera _asbp_player_default_taki))
      (Components|Activation|SetActive (Variables|Default|GetcameraMainMenu) false false)
      (Utilities|Casting|CastToBP_PlayerDefault_Taki _returnvalue_2)
      (Game|Player|SetViewTargetwithBlend (Game|GetPlayerController 0) _returnvalue_2 0.0 "VTBlend_Linear" 0.0 false))))

(event EventBeginPlay
  (CallFunction|SetLoadingScreen)
  (Rendering|Material|SetScalarParameterValue "/Game/Project/00_Generic/Assets/Materials/MaterialParameterValues/MPC_LoadingEffect.MPC_LoadingEffect" "DarknessAmount" 0.0 :!class /Script/Engine.KismetMaterialLibrary)
  (if (Variables|Debug|GetShowFPS)
    (Development|ExecuteConsoleCommand "stat fps" 0))
  (DebugFunctions|Show/HidePrintString)
  (bind _returnvalue (UserInterface|CreateWidget "/Game/Project/00_Generic/Blueprints/UI_HUD/WBP_Player.WBP_Player_C"))
  (bind _output_get (Variables|UI|SetPlayerUI _returnvalue))
  (UserInterface|Viewport|AddtoViewport _output_get 0)
  (Variables|Gameplay|SetCurrentCharacter (.AsBP%20Player%20Default%20Taki (Utilities|Casting|CastToBP_PlayerDefault_Taki (Game|Player|GetPlayerPawn 0))))
  (CallFunction|ResetTransformations)
  (UIFunctions|ShowPlayerUI true)
  (bind _asbp_cutethulu_instance (Utilities|Casting|CastToBP_CutethuluInstance (Game|GetGameInstance)))
  (UserInterface|Viewport|AddtoViewport (Variables|/Game/Project/00_Generic/Blueprints/Others/BP_CutethuluInstance.BP_CutethuluInstance_C|GetFadeWRef _asbp_cutethulu_instance) 0)
  (EventDispatchers|AssignOnPlayerTransform (delegate Custom|OnPlayerTransform_Event))
  (bind _returnvalue_2 (UserInterface|CreateWidget "/Game/Project/00_Generic/Blueprints/UI_HUD/WBP_LevelCollectables.WBP_LevelCollectables_C"))
  (bind _output_get_2 (Variables|UI|SetCollectablesWidget _returnvalue_2))
  (UserInterface|Viewport|AddtoViewport _returnvalue_2 0)
  (CallFunction|CollectablesWidgetFadeOut)
  (EventDispatchers|AssignOnTransformAcquired (delegate Custom|OnTransformAcquired_Event)))

(event Custom|HealWorld
  (bind _returnvalue (Class|DualLevelFunctionLibrary|GetDualLevel))
  (EventDispatchers|UnbindEventfromOnCuteLoaded _returnvalue (delegate Custom|FadeoutWorld))
  (EventDispatchers|BindEventtoOnCuteLoaded _returnvalue (delegate Custom|FadeoutWorld))
  (CallFunction|FadeinWorld))

(event Custom|SetLoadingScreen
  (bind _returnvalue (Class|DualLevelFunctionLibrary|GetDualLevel))
  (EventDispatchers|AssignOnAnyLoad _returnvalue (delegate Custom|OnAnyLoad_Event))
  (EventDispatchers|AssignOnAnyLoaded _returnvalue (delegate Custom|OnAnyLoaded_Event)))

(event Custom|FadeoutWorld
  (bind _returnvalue (Game|Player|GetPlayerPawn 0))
  (bind _asbp_playable_character (Utilities|Casting|CastToBP_PlayableCharacter _returnvalue))
  (bind (_direction _darkness) (Timeline|LevelFadingTimeline Reverse)
    (:Update
      (Rendering|Material|SetScalarParameterValue "/Game/Project/00_Generic/Assets/Materials/MaterialParameterValues/MPC_LoadingEffect.MPC_LoadingEffect" "DarknessAmount" _darkness :!class /Script/Engine.KismetMaterialLibrary)
      (Rendering|Material|SetVectorParameterValue "/Game/Project/00_Generic/Assets/Materials/MaterialParameterValues/MPC_LoadingEffect.MPC_LoadingEffect" "PlayerWorldPos" (Math|Conversions|ToLinearColor(Vector) (+ (Transformation|GetActorLocation (Game|Player|GetPlayerPawn 0)) "100.000000,-88.000000,88.000000")) :!class /Script/Engine.KismetMaterialLibrary))
    (:Finished
      (if (Utilities|Enum|Equal(Enum) _direction "Backward")
        (Default|SetCanMoveandJump _asbp_playable_character (Utilities|Enum|Equal(Enum) _direction "Backward"))
        (Variables|/Game/Project/00_Generic/Blueprints/PlayableCharacters/BP_PlayableCharacter.BP_PlayableCharacter_C|SetCanExecuteTransform _asbp_playable_character true)
        (Variables|/Game/Project/00_Generic/Blueprints/PlayableCharacters/BP_PlayableCharacter.BP_PlayableCharacter_C|SetCanRotateCamera _asbp_playable_character true)
        (bind _asbp_player_controller (Utilities|Casting|CastToBP_PlayerController (Game|GetPlayerController 0)))
        (Default|ShowLevelUI _asbp_player_controller)
        (else
          (Class|DualLevel|SwapLevel (Class|DualLevelFunctionLibrary|GetDualLevel)))))))

(event Custom|OnAnyLoad_Event
  (Utilities|IsValid (Variables|UI|GetLoading%20Screen)
    (:Is%20Not%20Valid
      (bind _returnvalue (UserInterface|CreateWidget "/Game/Project/00_Generic/Blueprints/UI_HUD/WBP_LoadingScreen.WBP_LoadingScreen_C"))
      (bind _output_get (Variables|UI|SetLoading%20Screen _returnvalue))
      (UserInterface|Viewport|AddtoViewport _output_get 0))))

(event Custom|OnAnyLoaded_Event
  (Widget|RemovefromParent (Variables|UI|GetLoading%20Screen))
  (EventDispatchers|UnbindEventfromOnAnyLoad (Class|DualLevelFunctionLibrary|GetDualLevel) (delegate Custom|OnAnyLoad_Event)))

(event Custom|FadeInWorld
  (bind _returnvalue (Game|Player|GetPlayerPawn 0))
  (bind _returnvalue_2 (Game|Player|GetPlayerPawn 0))
  (bind _asbp_playable_character (Utilities|Casting|CastToBP_PlayableCharacter _returnvalue))
  (bind _asbp_playable_character_2 (Utilities|Casting|CastToBP_PlayableCharacter _returnvalue_2))
  (Default|SetCanMoveandJump _asbp_playable_character false)
  (Variables|/Game/Project/00_Generic/Blueprints/PlayableCharacters/BP_PlayableCharacter.BP_PlayableCharacter_C|SetCanRotateCamera _asbp_playable_character false)
  (Variables|/Game/Project/00_Generic/Blueprints/PlayableCharacters/BP_PlayableCharacter.BP_PlayableCharacter_C|SetCanExecuteTransform _asbp_playable_character false)
  (bind (_direction _darkness) (Timeline|LevelFadingTimeline Play)
    (:Update
      (Rendering|Material|SetScalarParameterValue "/Game/Project/00_Generic/Assets/Materials/MaterialParameterValues/MPC_LoadingEffect.MPC_LoadingEffect" "DarknessAmount" _darkness :!class /Script/Engine.KismetMaterialLibrary)
      (Rendering|Material|SetVectorParameterValue "/Game/Project/00_Generic/Assets/Materials/MaterialParameterValues/MPC_LoadingEffect.MPC_LoadingEffect" "PlayerWorldPos" (Math|Conversions|ToLinearColor(Vector) (+ (Transformation|GetActorLocation (Game|Player|GetPlayerPawn 0)) "100.000000,-88.000000,88.000000")) :!class /Script/Engine.KismetMaterialLibrary))
    (:Finished
      (if (Utilities|Enum|Equal(Enum) _direction "Backward")
        (Default|SetCanMoveandJump _asbp_playable_character_2 (Utilities|Enum|Equal(Enum) _direction "Backward"))
        (Variables|/Game/Project/00_Generic/Blueprints/PlayableCharacters/BP_PlayableCharacter.BP_PlayableCharacter_C|SetCanExecuteTransform _asbp_playable_character_2 true)
        (Variables|/Game/Project/00_Generic/Blueprints/PlayableCharacters/BP_PlayableCharacter.BP_PlayableCharacter_C|SetCanRotateCamera _asbp_playable_character_2 true)
        (bind _asbp_player_controller (Utilities|Casting|CastToBP_PlayerController (Game|GetPlayerController 0)))
        (Default|ShowLevelUI _asbp_player_controller)
        (else
          (Class|DualLevel|SwapLevel (Class|DualLevelFunctionLibrary|GetDualLevel)))))))

(event Custom|CollectablesWidgetFadeOut
  (bind (_direction _alpha) (Timeline|CollectablesWidgetOpacity Reverse)
    (:Update
      (Widget|SetRenderOpacity (Variables|UI|GetCollectablesWidget) _alpha))
    (:Finished
      (if (Utilities|Enum|Equal(Enum) _direction "Forward")
        (Utilities|FlowControl|Delay 1e+01)
        (CallFunction|CollectablesWidgetFadeOut)))))

(event Custom|CollectablesWidgetsFadeIn
  (bind (_direction _alpha) (Timeline|CollectablesWidgetOpacity Play)
    (:Update
      (Widget|SetRenderOpacity (Variables|UI|GetCollectablesWidget) _alpha))
    (:Finished
      (if (Utilities|Enum|Equal(Enum) _direction "Forward")
        (Utilities|FlowControl|Delay 1e+01)
        (CallFunction|CollectablesWidgetFadeOut)))))

(fn ConstructionScript)

(fn Show/HidePrintString
  (if (Variables|Debug|GetShowStrings)
    (Development|ExecuteConsoleCommand "Enableallscreenmessages" 0)
    (else
      (Development|ExecuteConsoleCommand "Disableallscreenmessages" 0))))

(fn ShowPlayerUI
  (params (IsVisible%28PlayerUI%29 :type Boolean))
  (bind _playerui (Variables|UI|GetPlayerUI))
  (if IsVisible%28PlayerUI%29
    (Widget|SetVisibility _playerui "Visible")
    (else
      (Widget|SetVisibility _playerui "Collapsed"))))

(fn Fadein
  (bind _fadewref (Variables|UI|GetFadeWRef))
  (Widget|SetVisibility _fadewref "Visible")
  (UserInterface|Animation|PlayAnimation _fadewref (Variables|/Game/Project/00_Generic/Blueprints/UI_HUD/WBP_Fade.WBP_Fade_C|GetFadeIn _fadewref) 0.0 1 "Forward" 1.0 false))

(fn FadeOut
  (bind _fadewref (Variables|UI|GetFadeWRef))
  (Widget|SetVisibility _fadewref "Hidden")
  (UserInterface|Animation|PlayAnimation _fadewref (Variables|/Game/Project/00_Generic/Blueprints/UI_HUD/WBP_Fade.WBP_Fade_C|GetFadeOut _fadewref) 0.0 1 "Forward" 1.0 false))

(fn GetCharacterfromClass
  (params (Character%20class :type BP%20Playable%20Character%20Class%20Reference) (Spawn%20new%20if%20not%20found :type Boolean))
  (bind _outactors (Actor|GetAllActorsOfClass Character%20class))
  (if (Utilities|Array|IsEmpty _outactors)
    (if Spawn%20new%20if%20not%20found
      (bind _returnvalue (Game|SpawnActorfromClass Character%20class (Transformation|GetActorTransform (Game|Player|GetPlayerPawn 0)) "Undefined" "MultiplyWithRoot" 0 0))
      (return _returnvalue true)
      (else
        (return 0 false)))
    (else
      (return (Utilities|Array|Get(acopy) _outactors) true))))

(fn AssignTransform
  (params (CharacterClass :type BP%20Playable%20Character%20Class%20Reference))
  (if (!= (Utilities|GetClass (Variables|Gameplay|GetTransformation)) CharacterClass)
    (bind _returnedcharacter (GameFunctions|GetCharacterfromClass CharacterClass true))
    (bind _output_get (Variables|Gameplay|SetTransformation _returnedcharacter))
    (Default|CallOnTransformAcquired _output_get)))

(fn SwapCreaturetoTransform
  (bind _output_get (LocalVariables|SetTemp 0)))