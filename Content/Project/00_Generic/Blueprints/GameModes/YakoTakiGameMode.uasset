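; Game mode for YakoTaki that manages player character transformations, world healing and the camera transition from main menu to gameplay.
; Characters are cached by class and spawned on demand; AssignTransform sets the pending Transformation, and dispatcher handlers trigger transforms and refresh UI icons.
; HealWorld drives a darkness timeline through a material parameter collection around the player, swaps the dual level, then reverses once the cute level loads.
; Dual-level load events control when the player UI appears.
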(event Custom|OnPlayerTransform_Event
  (params (CurrentPlayableCharacter :type BP%20Playable%20Character%20Object%20Reference) (CharacterToTransform :type BP%20Playable%20Character%20Object%20Reference))
  (Variables|Gameplay|SetCurrentCharacter CharacterToTransform)
  (if (!= (Utilities|GetClass CurrentPlayableCharacter) "/Game/Project/00_Generic/Blueprints/PlayableCharacters/BP_PlayerDefault_Taki.BP_PlayerDefault_Taki_C")
    (Variables|Gameplay|SetTransformation CurrentPlayableCharacter)
    (else
      (Variables|Gameplay|SetTransformation 0)))
  (Default|UpdateIcons (Variables|/Game/Project/00_Generic/Blueprints/PlayerController/BP_PlayerController.BP_PlayerController_C|GetPlayerUI (.AsBP%20Player%20Controller (Utilities|Casting|CastToBP_PlayerController (Game|GetPlayerController 0))))))

(event Custom|NotifyAllCharsLanded
  (params (OnLandedActor :type Actor%20Object%20Reference))
  (bind _values (Utilities|Map|Values (Variables|Gameplay|GetSavedCharacters)))
  (for _array_element _values
    (Variables|/Game/Project/00_Generic/Blueprints/PlayableCharacters/BP_PlayableCharacter.BP_PlayableCharacter_C|SetHasLanded _array_element (not (and (.bSuccess (Utilities|Casting|CastToBP_PlayerDJ _array_element)) (.bSuccess (Utilities|Casting|CastToBP_Platform_DJ OnLandedActor)))))))

(event Custom|OnTransformAcquired_Event
  (params (AcquiredTransform :type BP%20Playable%20Character%20Object%20Reference))
  (bind _currentcharacter (Variables|Gameplay|GetCurrentCharacter))
  (Default|UpdateIcons (Variables|/Game/Project/00_Generic/Blueprints/PlayerController/BP_PlayerController.BP_PlayerController_C|GetPlayerUI (.AsBP%20Player%20Controller (Utilities|Casting|CastToBP_PlayerController (Game|GetPlayerController 0)))))
  (bind _cantransform (Default|CanTransform _currentcharacter false))
  (if _cantransform
    (Default|Transform _currentcharacter (Variables|Gameplay|GetTransformation))))

(event Custom|RestoreActors
  (bind _outactors (Actor|GetAllActorswithInterface "/Script/Yakotaki.RestorationInterface"))
  (for _array_element _outactors
    (Class|RestorationInterface|RestoreObject(Message) _array_element)))

(event Custom|PlayerTransition
  (bind _returnvalue (Game|GetPlayerController 0))
  (bind _returnvalue_2 (Game|Player|GetPlayerPawn 0))
  (bind _currentsoundplayer (Variables|Default|GetCurrentSoundPlayer))
  (bind _cameramainmenu (Variables|Default|GetcameraMainMenu))
  (bind _newtrack_0 (Timeline|Timeline Play)
    (:Update
      (bind _asbp_player_default_taki (Utilities|Casting|CastToBP_PlayerDefault_Taki (Game|Player|GetPlayerPawn 0)))
      (Transformation|SetWorldTransform _cameramainmenu (Math|Transform|Lerp(Transform) (Transformation|GetWorldTransform _cameramainmenu) (Transformation|GetWorldTransform (Variables|/Game/Project/00_Generic/Blueprints/PlayableCharacters/BP_PlayableCharacter.BP_PlayableCharacter_C|GetFollowCamera _asbp_player_default_taki)) _newtrack_0) true false)
      (Class|CameraComponent|SetPostProcessBlendWeight (Variables|Default|GetcameraMainMenu) _newtrack_0)
      (Audio|Components|Audio|FadeOut _currentsoundplayer 0.2 0.0 "Linear" :!class /Script/Engine.AudioComponent)
      (Utilities|FlowControl|Delay 0.2)
      (Audio|Components|Audio|SetSound _currentsoundplayer "/Game/Project/00_Generic/Assets/Sounds/SoundWaves_Cues/SW_CuteMusic.SW_CuteMusic"))
    (:Finished
      (Input|EnableInput _returnvalue _returnvalue)
      (Transformation|ResetRelativeTransform (Variables|/Game/Project/00_Generic/Blueprints/PlayableCharacters/BP_PlayableCharacter.BP_PlayableCharacter_C|GetFollowCamera _asbp_player_default_taki))
      (Components|Activation|SetActive (Variables|Default|GetcameraMainMenu) false false)
      (Utilities|Casting|CastToBP_PlayerDefault_Taki _returnvalue_2)
      (Game|Player|SetViewTargetwithBlend (Game|GetPlayerController 0) _returnvalue_2 0.0 "VTBlend_Linear" 0.0 false))))

(event EventBeginPlay
  (CallFunction|SetLoadingScreen)
  (Rendering|Material|SetScalarParameterValue "/Game/Project/00_Generic/Assets/Materials/MaterialParameterValues/MPC_LoadingEffect.MPC_LoadingEffect" "DarknessAmount" 0.0 :!class /Script/Engine.KismetMaterialLibrary)
  (if (Variables|Debug|GetShowFPS)
    (Development|ExecuteConsoleCommand "stat fps" 0))
  (DebugFunctions|Show/HidePrintString)
  (bind _output_get (Variables|Gameplay|SetCurrentCharacter (.AsBP%20Player%20Default%20Taki (Utilities|Casting|CastToBP_PlayerDefault_Taki (Game|Player|GetPlayerPawn 0)))))
  (Utilities|Map|Add (Variables|Gameplay|GetSavedCharacters) (Utilities|GetClass _output_get) _output_get)
  (EventDispatchers|AssignOnPlayerTransform (delegate Custom|OnPlayerTransform_Event))
  (EventDispatchers|AssignOnTransformAcquired (delegate Custom|OnTransformAcquired_Event)))

(event Custom|HealWorld
  (bind _returnvalue (Class|DualLevelFunctionLibrary|GetDualLevel))
  ;[0.15 0.15 0.15 0.5] World "healing"
  (EventDispatchers|UnbindEventfromOnCuteLoaded _returnvalue (delegate Custom|FadeoutWorld))
  (EventDispatchers|BindEventtoOnCuteLoaded _returnvalue (delegate Custom|FadeoutWorld))
  (CallFunction|FadeinWorld))

(event Custom|SetLoadingScreen
  ;[0.15 0.15 0.15 0.5] Enables loading screen and disables it when streamed level is loaded
  (EventDispatchers|AssignOnAnyLoaded (Class|DualLevelFunctionLibrary|GetDualLevel) (delegate Custom|OnAnyLoaded_Event)))

(event Custom|OnInitialSequenceComplete_Event
  ;[0.15 0.15 0.15 0.5] Enables loading screen and disables it when streamed level is loaded
  (Default|ShowPlayerUI (.AsBP%20Player%20Controller (Utilities|Casting|CastToBP_PlayerController (Game|GetPlayerController 0))) true)
  (EventDispatchers|UnbindEventfromOnInitialSequenceComplete (Class|DualLevelFunctionLibrary|GetDualLevel) (delegate Custom|OnInitialSequenceComplete_Event)))

(event Custom|FadeoutWorld
  (bind _returnvalue (Game|Player|GetPlayerPawn 0))
  (bind _asbp_playable_character (Utilities|Casting|CastToBP_PlayableCharacter _returnvalue))
  ;[0.15 0.15 0.15 0.5] World "healing"
  (bind (_direction _darkness) (Timeline|LevelFadingTimeline Reverse)
    (:Update
      (Rendering|Material|SetScalarParameterValue "/Game/Project/00_Generic/Assets/Materials/MaterialParameterValues/MPC_LoadingEffect.MPC_LoadingEffect" "DarknessAmount" _darkness :!class /Script/Engine.KismetMaterialLibrary)
      (Rendering|Material|SetVectorParameterValue "/Game/Project/00_Generic/Assets/Materials/MaterialParameterValues/MPC_LoadingEffect.MPC_LoadingEffect" "PlayerWorldPos" (Math|Conversions|ToLinearColor(Vector) (+ (Transformation|GetActorLocation (Game|Player|GetPlayerPawn 0)) "100.000000,-88.000000,88.000000")) :!class /Script/Engine.KismetMaterialLibrary))
    (:Finished
      (if (Utilities|Enum|Equal(Enum) _direction "Backward")
        (Default|SetCanMoveandJump _asbp_playable_character (Utilities|Enum|Equal(Enum) _direction "Backward"))
        (Variables|/Game/Project/00_Generic/Blueprints/PlayableCharacters/BP_PlayableCharacter.BP_PlayableCharacter_C|SetCanExecuteTransform _asbp_playable_character true)
        (Variables|/Game/Project/00_Generic/Blueprints/PlayableCharacters/BP_PlayableCharacter.BP_PlayableCharacter_C|SetCanRotateCamera _asbp_playable_character true)
        (if (!= (Variables|/Script/Yakotaki.DualLevel|GetLevelID (Class|DualLevelFunctionLibrary|GetDualLevel)) 0)
          (bind _returnvalue_2 (UserInterface|CreateWidget "/Game/Project/00_Generic/Blueprints/UI_HUD/WBP_PortalFragments.WBP_PortalFragments_C"))
          (bind _output_get (Variables|UI|SetPortal%20fragmentsUI _returnvalue_2))
          (UserInterface|Viewport|AddtoViewport _output_get 0))
        (else
          (Class|DualLevel|SwapLevel (Class|DualLevelFunctionLibrary|GetDualLevel)))))))

(event Custom|OnAnyLoaded_Event
  ;[0.15 0.15 0.15 0.5] Enables loading screen and disables it when streamed level is loaded
  (if (Utilities|Enum|Equal(Enum) (Variables|/Script/Yakotaki.DualLevel|GetloadedState (Class|DualLevelFunctionLibrary|GetDualLevel)) "CUTE")
    (Default|ShowPlayerUI (.AsBP%20Player%20Controller (Utilities|Casting|CastToBP_PlayerController (Game|GetPlayerController 0))) true)
    (else
      (EventDispatchers|AssignOnInitialSequenceComplete (Class|DualLevelFunctionLibrary|GetDualLevel) (delegate Custom|OnInitialSequenceComplete_Event))))
  (EventDispatchers|UnbindEventfromOnAnyLoaded (Class|DualLevelFunctionLibrary|GetDualLevel) (delegate Custom|OnAnyLoaded_Event)))

(event Custom|FadeInWorld
  (bind _returnvalue (Game|Player|GetPlayerPawn 0))
  (bind _returnvalue_2 (Game|Player|GetPlayerPawn 0))
  (bind _asbp_playable_character (Utilities|Casting|CastToBP_PlayableCharacter _returnvalue))
  (bind _asbp_playable_character_2 (Utilities|Casting|CastToBP_PlayableCharacter _returnvalue_2))
  ;[0.15 0.15 0.15 0.5] World "healing"
  (Default|SetCanMoveandJump _asbp_playable_character false)
  (Variables|/Game/Project/00_Generic/Blueprints/PlayableCharacters/BP_PlayableCharacter.BP_PlayableCharacter_C|SetCanRotateCamera _asbp_playable_character true)
  (Variables|/Game/Project/00_Generic/Blueprints/PlayableCharacters/BP_PlayableCharacter.BP_PlayableCharacter_C|SetCanExecuteTransform _asbp_playable_character false)
  (bind (_direction _darkness) (Timeline|LevelFadingTimeline Play)
    (:Update
      (Rendering|Material|SetScalarParameterValue "/Game/Project/00_Generic/Assets/Materials/MaterialParameterValues/MPC_LoadingEffect.MPC_LoadingEffect" "DarknessAmount" _darkness :!class /Script/Engine.KismetMaterialLibrary)
      (Rendering|Material|SetVectorParameterValue "/Game/Project/00_Generic/Assets/Materials/MaterialParameterValues/MPC_LoadingEffect.MPC_LoadingEffect" "PlayerWorldPos" (Math|Conversions|ToLinearColor(Vector) (+ (Transformation|GetActorLocation (Game|Player|GetPlayerPawn 0)) "100.000000,-88.000000,88.000000")) :!class /Script/Engine.KismetMaterialLibrary))
    (:Finished
      (if (Utilities|Enum|Equal(Enum) _direction "Backward")
        (Default|SetCanMoveandJump _asbp_playable_character_2 (Utilities|Enum|Equal(Enum) _direction "Backward"))
        (Variables|/Game/Project/00_Generic/Blueprints/PlayableCharacters/BP_PlayableCharacter.BP_PlayableCharacter_C|SetCanExecuteTransform _asbp_playable_character_2 true)
        (Variables|/Game/Project/00_Generic/Blueprints/PlayableCharacters/BP_PlayableCharacter.BP_PlayableCharacter_C|SetCanRotateCamera _asbp_playable_character_2 true)
        (if (!= (Variables|/Script/Yakotaki.DualLevel|GetLevelID (Class|DualLevelFunctionLibrary|GetDualLevel)) 0)
          (bind _returnvalue_3 (UserInterface|CreateWidget "/Game/Project/00_Generic/Blueprints/UI_HUD/WBP_PortalFragments.WBP_PortalFragments_C"))
          (bind _output_get (Variables|UI|SetPortal%20fragmentsUI _returnvalue_3))
          (UserInterface|Viewport|AddtoViewport _output_get 0))
        (else
          (Class|DualLevel|SwapLevel (Class|DualLevelFunctionLibrary|GetDualLevel)))))))

(fn ConstructionScript)

(fn Show/HidePrintString
  (if (Variables|Debug|GetShowStrings)
    (Development|ExecuteConsoleCommand "Enableallscreenmessages" 0)
    (else
      (Development|ExecuteConsoleCommand "Disableallscreenmessages" 0))))

(fn GetCharacterfromClass
  (params (Character%20class :type BP%20Playable%20Character%20Class%20Reference) (Spawn%20new%20if%20not%20found :type Boolean))
  (bind _savedcharacters (Variables|Gameplay|GetSavedCharacters))
  (bind (_value _returnvalue) (Utilities|Map|Find _savedcharacters Character%20class))
  (if _returnvalue
    (return _value _returnvalue)
    (else
      (bind _outactors (Actor|GetAllActorsOfClass Character%20class))
      (if (Utilities|Array|IsEmpty _outactors)
        (if Spawn%20new%20if%20not%20found
          (bind _returnvalue_2 (Game|SpawnActorfromClass Character%20class (Transformation|GetActorTransform (Game|Player|GetPlayerPawn 0)) "Undefined" "MultiplyWithRoot" 0 0))
          (Utilities|Map|Add (Variables|Gameplay|GetSavedCharacters) Character%20class _returnvalue_2)
          (return _returnvalue_2 true)
          (else
            (return 0 false)))
        (else
          (return (Utilities|Array|Get(acopy) _outactors) true))))))

(fn AssignTransform
  (params (CharacterClass :type BP%20Playable%20Character%20Class%20Reference))
  (if (and (!= (Utilities|GetClass (Variables|Gameplay|GetCurrentCharacter)) CharacterClass) (!= CharacterClass (Utilities|GetClass (Variables|Gameplay|GetTransformation))))
    (bind _returnedcharacter (GameFunctions|GetCharacterfromClass CharacterClass true))
    (bind _output_get (Variables|Gameplay|SetTransformation _returnedcharacter))
    (Default|CallOnTransformAcquired _output_get)
    (elif (not (!= CharacterClass (Utilities|GetClass (Variables|Gameplay|GetTransformation))))
      (bind _returnedcharacter_2 (GameFunctions|GetCharacterfromClass CharacterClass true))
      (Default|Transform (.AsBP%20Playable%20Character (Utilities|Casting|CastToBP_PlayableCharacter (Game|Player|GetPlayerPawn 0))) _returnedcharacter_2))))