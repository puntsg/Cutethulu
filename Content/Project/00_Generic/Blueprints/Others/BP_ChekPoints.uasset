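; BP_ChekPoints is a checkpoint trigger that records the player's latest checkpoint location.
; When a BP_PlayableCharacter overlaps its Box, SetChekPoints writes the actor's own location to LastCheckPointLocation on BP_CutethuluInstance, the game instance.
; Shortly after BeginPlay it also checks whether the player already stands inside the Box, covering a start point placed within the trigger.
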(event OnComponentBeginOverlap(Box)
  (params (OverlappedComponent :type Primitive%20Component%20Object%20Reference) (OtherActor :type Actor%20Object%20Reference) (OtherComp :type Primitive%20Component%20Object%20Reference) (OtherBodyIndex :type Integer) (bFromSweep :type Boolean) (SweepResult :type Hit%20Result%20Structure%20%28by%20ref%29))
  ;[0.15 0.15 0.15 0.5] Colliders
  ;;[0.15 0.15 0.15 0.5] Set the checkpoint when player collision with collider
  (Utilities|Casting|CastToBP_PlayableCharacter OtherActor)
  (CallFunction|SetChekPoints))

(event EventBeginPlay
  ;[0.15 0.15 0.15 0.5] Check if PlayerStart is inside of trigger and set checkpoint
  (Utilities|FlowControl|Delay 0.1)
  (if (Collision|IsOverlappingActor (Variables|Default|GetBox) (Game|GetPlayerCharacter 0) :!class /Script/Engine.PrimitiveComponent)
    (CallFunction|SetChekPoints)))

(event Collision|EventActorBeginOverlap
  (params (OtherActor :type Actor%20Object%20Reference)))

(event EventTick
  (params (DeltaSeconds :type Float%20%28single-precision%29)))

(fn ConstructionScript)

(fn SetChekPoints
  ;[0.15 0.15 0.15 0.5] Update the checkpoint position
  (bind _asbp_cutethulu_instance (Utilities|Casting|CastToBP_CutethuluInstance (Game|GetGameInstance)))
  (Variables|/Game/Project/00_Generic/Blueprints/Others/BP_CutethuluInstance.BP_CutethuluInstance_C|SetLastCheckPointLocation _asbp_cutethulu_instance (Transformation|GetActorLocation)))