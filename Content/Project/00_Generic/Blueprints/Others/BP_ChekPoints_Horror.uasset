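; Checkpoint actor with an animated flag that registers itself with BP_YakotakiInstance when a BP_PlayableCharacter overlaps its box.
; Any overlap sets Arrive, before the character cast.
; The flag starts on a looping stopped animation; a separate Flagup event, not called in this graph, plays the down animation once, then switches to a looped one after a delay.
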(event OnComponentBeginOverlap(Box)
  (params (OverlappedComponent :type Primitive%20Component%20Object%20Reference) (OtherActor :type Actor%20Object%20Reference) (OtherComp :type Primitive%20Component%20Object%20Reference) (OtherBodyIndex :type Integer) (bFromSweep :type Boolean) (SweepResult :type Hit%20Result%20Structure%20%28by%20ref%29))
  ;[0.15 0.15 0.15 0.5] Colliders
  ;;[0.15 0.15 0.15 0.5] Set the checkpoint when player collision with collider
  (Variables|Default|SetArrive true)
  (Utilities|Casting|CastToBP_PlayableCharacter OtherActor)
  (Default|SetCheckpoint (.AsBP%20Yakotaki%20Instance (Utilities|Casting|CastToBP_YakotakiInstance (Game|GetGameInstance))) self))

(event Custom|Flag%20up
  ;[0.15 0.15 0.15 0.5] Flag animation
  (Utilities|FlowControl|DoOnce false
    (:Completed
      (Utilities|FlowControl|Sequence
        (:then_0
          (Audio|Components|Audio|Stop (Variables|Default|GetSK_Flag))
          (Components|Animation|PlayAnimation (Variables|Default|GetSK_Flag) "/Game/Project/02_WinterWonderland/Assets/Models/Flag/A_Down.A_Down" false))
        (:then_1
          (Utilities|FlowControl|Delay 3.0)
          (Variables|Default|SetIsLooping true)
          (Components|Animation|PlayAnimation (Variables|Default|GetSK_Flag) "/Game/Project/02_WinterWonderland/Assets/Models/Flag/A_Looped.A_Looped" true))))))

(event EventBeginPlay
  ;[0.15 0.15 0.15 0.5] Check if PlayerStart is inside of trigger and set checkpoint
  (Variables|Default|SetStartPosition (Variables|/Script/Engine.SceneComponent|GetRelativeLocation (Variables|Default|GetFlag)))
  (Components|Animation|PlayAnimation (Variables|Default|GetSK_Flag) "/Game/Project/02_WinterWonderland/Assets/Models/Flag/A_Stopped.A_Stopped" true))

(fn ConstructionScript)