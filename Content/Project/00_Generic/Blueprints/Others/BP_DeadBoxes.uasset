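; Kill volume that sends the player back to the last checkpoint when they overlap its box.
; On overlap it locks movement and input, insta-kills and fully heals the player, then calls a Teleport event.
; Teleport fades through BP_YakotakiInstance, waits a second, moves the player to LastCheckPointLocation and stops momentum.
; The delay sits inside that event, so controls return and the IsSpawning guard clears before the move happens.
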(event OnComponentBeginOverlap(Box)
  (params (OverlappedComponent :type Primitive%20Component%20Object%20Reference) (OtherActor :type Actor%20Object%20Reference) (OtherComp :type Primitive%20Component%20Object%20Reference) (OtherBodyIndex :type Integer) (bFromSweep :type Boolean) (SweepResult :type Hit%20Result%20Structure%20%28by%20ref%29))
  ;[0.15 0.15 0.15 0.5] Collisions
  ;;[0.15 0.15 0.15 0.5] Teleport player is not Spawning and is collisioning
  (if (not (Variables|Default|GetIsSpawning))
    (bind _asbp_playable_character (Utilities|Casting|CastToBP_PlayableCharacter OtherActor))
    (Variables|Default|SetIsSpawning true)
    (bind _player_controller (CallFunction|DisableMovementandKillPlayer _asbp_playable_character))
    (CallFunction|Teleport _asbp_playable_character)
    (CallFunction|RefillandEnableMovement _player_controller _asbp_playable_character)
    (Variables|Default|SetIsSpawning false)))

(event Custom|Teleport
  (params (Player :type BP%20Playable%20Character%20Object%20Reference))
  ;[0.15 0.15 0.15 0.5] Teleport the player to checkpoint
  (bind _asbp_yakotaki_instance (Utilities|Casting|CastToBP_YakotakiInstance (Game|GetGameInstance)))
  (Default|Fadein _asbp_yakotaki_instance)
  (Utilities|FlowControl|Delay 1.0)
  (Transformation|Teleport Player (Variables|/Game/Project/00_Generic/Blueprints/GameInstance/BP_YakotakiInstance.BP_YakotakiInstance_C|GetLastCheckPointLocation _asbp_yakotaki_instance) "0, 0, 0")
  (Default|FadeOut _asbp_yakotaki_instance)
  (Components|Movement|StopMovementImmediately (Variables|/Script/Engine.Character|GetCharacterMovement (Game|GetPlayerCharacter 0))))

(fn ConstructionScript)

(fn DisableMovementandKillPlayer
  (params (Playable%20Character :type BP%20Playable%20Character%20Object%20Reference))
  (bind _returnvalue (Game|GetPlayerController 0))
  (bind _advancedhealthbehaviour (Variables|/Game/Project/00_Generic/Blueprints/PlayableCharacters/BP_PlayableCharacter.BP_PlayableCharacter_C|GetAdvancedHealthBehaviour Playable%20Character))
  ;[0.15 0.15 0.15 0.5] Disable movement and kill Player to reset his Heal
  (Default|SetCanMoveandJump Playable%20Character false)
  (Default|SetActive Playable%20Character false)
  (Class|AdvancedHealthBehaviour|InstaKill _advancedhealthbehaviour)
  (Class|AdvancedHealthBehaviour|MaxHeal _advancedhealthbehaviour)
  (Input|DisableInput Playable%20Character _returnvalue)
  (return _returnvalue))

(fn RefillandEnableMovement
  (params (Player%20Controller :type Player%20Controller%20Object%20Reference) (Playable%20Character :type BP%20Playable%20Character%20Object%20Reference))
  ;[0.15 0.15 0.15 0.5] Refill mechanics Refilleables and Enable movement
  (Input|EnableInput Playable%20Character Player%20Controller)
  (Default|SetActive Playable%20Character true)
  (Default|SetCanMoveandJump Playable%20Character true)
  (Variables|/Game/Project/00_Generic/Blueprints/PlayableCharacters/BP_PlayableCharacter.BP_PlayableCharacter_C|SetCanRotateCamera Playable%20Character true)
  (Class|AdvancedHealthBehaviour|MaxHeal (Variables|/Game/Project/00_Generic/Blueprints/PlayableCharacters/BP_PlayableCharacter.BP_PlayableCharacter_C|GetAdvancedHealthBehaviour Playable%20Character)))