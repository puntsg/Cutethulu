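; Development cheat actor that teleports the player to preset positions for testing.
; On BeginPlay it enables input from player controller 0.
; Number keys 1 through 0 each teleport player pawn 0 to an entry in the TPPositions array, offset from the actor's location, with zero rotation.
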(event EventBeginPlay
  ;[0.15 0.15 0.15 0.5] Enables inputs
  (Input|EnableInput (Game|GetPlayerController 0)))

(event Input|KeyboardEvents|0
  (params (Key :type Key%20Structure :default "None"))
  ;[0.15 0.15 0.15 0.5] Teleports
  (:Pressed
    (Transformation|Teleport (Game|Player|GetPlayerPawn 0) (+ (Utilities|Array|Get(acopy) (Variables|Default|GetTP%20Positions) 9) (Transformation|GetActorLocation)) "0, 0, 0")))

(event Input|KeyboardEvents|9
  (params (Key :type Key%20Structure :default "None"))
  ;[0.15 0.15 0.15 0.5] Teleports
  (:Pressed
    (Transformation|Teleport (Game|Player|GetPlayerPawn 0) (+ (Utilities|Array|Get(acopy) (Variables|Default|GetTP%20Positions) 8) (Transformation|GetActorLocation)) "0, 0, 0")))

(event Input|KeyboardEvents|1
  (params (Key :type Key%20Structure :default "None"))
  ;[0.15 0.15 0.15 0.5] Teleports
  (:Pressed
    (Transformation|Teleport (Game|Player|GetPlayerPawn 0) (+ (Utilities|Array|Get(acopy) (Variables|Default|GetTP%20Positions)) (Transformation|GetActorLocation)) "0, 0, 0")))

(event Input|KeyboardEvents|2
  (params (Key :type Key%20Structure :default "None"))
  ;[0.15 0.15 0.15 0.5] Teleports
  (:Pressed
    (Transformation|Teleport (Game|Player|GetPlayerPawn 0) (+ (Utilities|Array|Get(acopy) (Variables|Default|GetTP%20Positions) 1) (Transformation|GetActorLocation)) "0, 0, 0")))

(event Input|KeyboardEvents|3
  (params (Key :type Key%20Structure :default "None"))
  ;[0.15 0.15 0.15 0.5] Teleports
  (:Pressed
    (Transformation|Teleport (Game|Player|GetPlayerPawn 0) (+ (Utilities|Array|Get(acopy) (Variables|Default|GetTP%20Positions) 2) (Transformation|GetActorLocation)) "0, 0, 0")))

(event Input|KeyboardEvents|4
  (params (Key :type Key%20Structure :default "None"))
  ;[0.15 0.15 0.15 0.5] Teleports
  (:Pressed
    (Transformation|Teleport (Game|Player|GetPlayerPawn 0) (+ (Utilities|Array|Get(acopy) (Variables|Default|GetTP%20Positions) 3) (Transformation|GetActorLocation)) "0, 0, 0")))

(event Input|KeyboardEvents|5
  (params (Key :type Key%20Structure :default "None"))
  ;[0.15 0.15 0.15 0.5] Teleports
  (:Pressed
    (Transformation|Teleport (Game|Player|GetPlayerPawn 0) (+ (Utilities|Array|Get(acopy) (Variables|Default|GetTP%20Positions) 4) (Transformation|GetActorLocation)) "0, 0, 0")))

(event Input|KeyboardEvents|6
  (params (Key :type Key%20Structure :default "None"))
  ;[0.15 0.15 0.15 0.5] Teleports
  (:Pressed
    (Transformation|Teleport (Game|Player|GetPlayerPawn 0) (+ (Utilities|Array|Get(acopy) (Variables|Default|GetTP%20Positions) 5) (Transformation|GetActorLocation)) "0, 0, 0")))

(event Input|KeyboardEvents|7
  (params (Key :type Key%20Structure :default "None"))
  ;[0.15 0.15 0.15 0.5] Teleports
  (:Pressed
    (Transformation|Teleport (Game|Player|GetPlayerPawn 0) (+ (Utilities|Array|Get(acopy) (Variables|Default|GetTP%20Positions) 6) (Transformation|GetActorLocation)) "0, 0, 0")))

(event Input|KeyboardEvents|8
  (params (Key :type Key%20Structure :default "None"))
  ;[0.15 0.15 0.15 0.5] Teleports
  (:Pressed
    (Transformation|Teleport (Game|Player|GetPlayerPawn 0) (+ (Utilities|Array|Get(acopy) (Variables|Default|GetTP%20Positions) 7) (Transformation|GetActorLocation)) "0, 0, 0")))

(fn ConstructionScript)