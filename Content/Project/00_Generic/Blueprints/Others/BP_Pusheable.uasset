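; BP_Pusheable is an actor that can be shoved along a given direction when its Push event is called.
; Push stores the current location, offsets it by direction times PushForce, and moves the actor there with a timeline-driven lerp using a swept SetActorLocation.
; When an overlap on the Cube component ends, the Cube switches to physics simulation.
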(event OnComponentEndOverlap(Cube)
  (params (OverlappedComponent :type Primitive%20Component%20Object%20Reference) (OtherActor :type Actor%20Object%20Reference) (OtherComp :type Primitive%20Component%20Object%20Reference) (OtherBodyIndex :type Integer))
  (Physics|SetSimulatePhysics (Variables|Default|GetCube) true))

(event EventPush
  (params (Direccion :type Vector :default "0, 0, 0"))
  ;[0.15 0.15 0.15 0.5] Activates push
  (bind _output_get (Variables|Default|SetInitialPos (Transformation|GetActorLocation)))
  (Variables|Default|SetFinalPos (+ _output_get (* Direccion (Variables|Default|GetPushForce))))
  (bind _alpha (Timeline|PushTimeLine PlayFromStart)
    (:Update
      (bind _returnvalue (Math|Vector|Lerp(Vector) (Variables|Default|GetInitialPos) (Variables|Default|GetFinalPos) _alpha))
      (Transformation|SetActorLocation _returnvalue true false))))

(fn ConstructionScript)