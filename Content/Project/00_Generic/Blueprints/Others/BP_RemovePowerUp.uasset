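; BP_RemovePowerUp is a trigger volume that strips the player's current power-up transformation.
; When a BP_PlayableCharacter overlaps its box, it clears the Transformation stored in TestGameMode.
; A non-default character is transformed into BP_PlayerDefault_Taki, which the game mode finds or spawns.
; If the player is already Taki, it only refreshes the UI icons through the player controller.
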(event OnComponentBeginOverlap(Box)
  (params (OverlappedComponent :type Primitive%20Component%20Object%20Reference) (OtherActor :type Actor%20Object%20Reference) (OtherComp :type Primitive%20Component%20Object%20Reference) (OtherBodyIndex :type Integer) (bFromSweep :type Boolean) (SweepResult :type Hit%20Result%20Structure%20%28by%20ref%29))
  (bind _returnvalue (Game|GetGameMode))
  (bind _astest_game_mode (Utilities|Casting|CastToTestGameMode _returnvalue))
  (bind _asbp_playable_character (Utilities|Casting|CastToBP_PlayableCharacter OtherActor))
  (Variables|/Game/Project/00_Generic/Blueprints/GameModes/TestGameMode.TestGameMode_C|SetTransformation _astest_game_mode 0)
  (if (!= (Utilities|GetClass _asbp_playable_character) "/Game/Project/00_Generic/Blueprints/PlayableCharacters/BP_PlayerDefault_Taki.BP_PlayerDefault_Taki_C")
    (bind _returnedcharacter (Default|GetCharacterfromClass _astest_game_mode "/Game/Project/00_Generic/Blueprints/PlayableCharacters/BP_PlayerDefault_Taki.BP_PlayerDefault_Taki_C" true))
    (Default|Transform _asbp_playable_character _returnedcharacter)
    (else
      (Default|UpdateIcons (Variables|/Game/Project/00_Generic/Blueprints/PlayerController/BP_PlayerController.BP_PlayerController_C|GetPlayerUI (.AsBP%20Player%20Controller (Utilities|Casting|CastToBP_PlayerController (Game|GetPlayerController 0))))))))

(fn ConstructionScript)