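; BP_Seed is an interactable seed that heals the world when the player uses it.
; Its collider registers it as the player's CurrentInteractive and fades a prompt widget in and out through a Timeline.
; Interacting reverts the player to Taki, pausing briefly if needed, then plays an absorption effect and calls HealWorld on the game mode.
; Horror and cute load events swap the seed's material, while the FMOD-style sound nodes are left disconnected.
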(event OnComponentBeginOverlap(seed_collider)
  (params (OverlappedComponent :type Primitive%20Component%20Object%20Reference) (OtherActor :type Actor%20Object%20Reference) (OtherComp :type Primitive%20Component%20Object%20Reference) (OtherBodyIndex :type Integer) (bFromSweep :type Boolean) (SweepResult :type Hit%20Result%20Structure%20%28by%20ref%29))
  (bind _widget (Variables|Default|GetWidget))
  ;[0.15 0.15 0.15 0.5] Collision detection
  (bind _asbp_playable_character (Utilities|Casting|CastToBP_PlayableCharacter OtherActor))
  (Variables|Default|SetIsCollision true)
  (Variables|/Game/Project/00_Generic/Blueprints/PlayableCharacters/BP_PlayableCharacter.BP_PlayableCharacter_C|SetCurrentInteractive _asbp_playable_character self)
  (Development|SetHiddeninGame _widget false false)
  ;[0.15 0.15 0.15 0.5] Widget visibility timeline
  (bind (_direction _alfa) (Timeline|Timeline PlayFromStart)
    (:Update
      (Default|Alfa (.AsWBP%20Interactive (Utilities|Casting|CastToWBP_Interactive (UserInterface|GetWidget _widget))) _alfa))
    (:Finished
      (if (Utilities|Enum|Equal(Enum) _direction "Backward")
        (Development|SetHiddeninGame (Variables|Default|GetWidget) true false)))))

(event OnComponentEndOverlap(seed_collider)
  (params (OverlappedComponent :type Primitive%20Component%20Object%20Reference) (OtherActor :type Actor%20Object%20Reference) (OtherComp :type Primitive%20Component%20Object%20Reference) (OtherBodyIndex :type Integer))
  ;[0.15 0.15 0.15 0.5] Collision detection
  (bind _asbp_playable_character (Utilities|Casting|CastToBP_PlayableCharacter OtherActor))
  (Variables|Default|SetIsCollision false)
  (Variables|/Game/Project/00_Generic/Blueprints/PlayableCharacters/BP_PlayableCharacter.BP_PlayableCharacter_C|SetCurrentInteractive _asbp_playable_character 0)
  ;[0.15 0.15 0.15 0.5] Widget visibility timeline
  (bind (_direction _alfa) (Timeline|Timeline Reverse)
    (:Update
      (Default|Alfa (.AsWBP%20Interactive (Utilities|Casting|CastToWBP_Interactive (UserInterface|GetWidget (Variables|Default|GetWidget)))) _alfa))
    (:Finished
      (if (Utilities|Enum|Equal(Enum) _direction "Backward")
        (Development|SetHiddeninGame (Variables|Default|GetWidget) true false)))))

(event EventOnInteract
  (params (InteractedPlayer :type BP%20Playable%20Character%20Object%20Reference))
  (bind _returnvalue (Transformation|GetActorTransform))
  ;[0.15 0.15 0.15 0.5] Interaction
  (if (Variables|Default|GetIsCollision)
    (bind _hasuntransformed (CallFunction|Untransform))
    (if _hasuntransformed
      (Utilities|FlowControl|Delay 0.5))
    (bind _asyako_taki_game_mode (Utilities|Casting|CastToYakoTakiGameMode (Game|GetGameMode)))
    (Niagara|SpawnSystematLocation "/Game/Project/00_Generic/Assets/VFX/CopyHability/FXS_Absortion.FXS_Absortion" (.location _returnvalue) (.rotation _returnvalue) (* (.scale _returnvalue) "10.000000,10.000000,10.000000"))
    (Default|HealWorld _asyako_taki_game_mode)
    ;[0.15 0.15 0.15 0.5] Widget visibility timeline
    (bind (_direction _alfa) (Timeline|Timeline Reverse)
      (:Update
        (Default|Alfa (.AsWBP%20Interactive (Utilities|Casting|CastToWBP_Interactive (UserInterface|GetWidget (Variables|Default|GetWidget)))) _alfa))
      (:Finished
        (if (Utilities|Enum|Equal(Enum) _direction "Backward")
          (Development|SetHiddeninGame (Variables|Default|GetWidget) true false))))))

(event EventOnHorrorLoaded
  ;[0.15 0.15 0.15 0.5] Changing material
  (Rendering|Material|SetMaterial (Variables|Default|GetSeed) 0 "/Game/Project/00_Generic/Assets/Models/Seed/MI_seed_h.MI_seed_h"))

(event EventOnCuteLoaded
  ;[0.15 0.15 0.15 0.5] Changing material
  (Rendering|Material|SetMaterial (Variables|Default|GetSeed) 0 "/Game/Project/00_Generic/Assets/Models/Seed/MI_seed_c.MI_seed_c"))

(event EventBeginPlay)

(fn ConstructionScript)

(fn Untransform
  (bind _returnvalue (Game|GetGameMode))
  (bind _asyako_taki_game_mode (Utilities|Casting|CastToYakoTakiGameMode _returnvalue))
  ;[0.15 0.15 0.15 0.5] Checks if playable character
  (bind _asbp_playable_character (Utilities|Casting|CastToBP_PlayableCharacter (Game|Player|GetPlayerPawn 0)))
  (Variables|/Game/Project/00_Generic/Blueprints/GameModes/YakoTakiGameMode.YakoTakiGameMode_C|SetTransformation _asyako_taki_game_mode 0)
  (if (!= (Utilities|GetClass _asbp_playable_character) "/Game/Project/00_Generic/Blueprints/PlayableCharacters/BP_PlayerDefault_Taki.BP_PlayerDefault_Taki_C")
    ;[0.15 0.15 0.15 0.5] No taki -> turns into taki
    (bind _returnedcharacter (Default|GetCharacterfromClass _asyako_taki_game_mode "/Game/Project/00_Generic/Blueprints/PlayableCharacters/BP_PlayerDefault_Taki.BP_PlayerDefault_Taki_C" true))
    (Default|Transform _asbp_playable_character _returnedcharacter)
    (Variables|/Game/Project/00_Generic/Blueprints/GameModes/YakoTakiGameMode.YakoTakiGameMode_C|SetTransformation _asyako_taki_game_mode 0)
    (return true)
    (else
      ;[0.15 0.15 0.15 0.5] Updates UI if taki
      (Default|UpdateIcons (Variables|/Game/Project/00_Generic/Blueprints/PlayerController/BP_PlayerController.BP_PlayerController_C|GetPlayerUI (.AsBP%20Player%20Controller (Utilities|Casting|CastToBP_PlayerController (Game|GetPlayerController 0)))))
      (return false))))