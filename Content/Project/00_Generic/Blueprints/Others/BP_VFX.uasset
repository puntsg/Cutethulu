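; Collectible particle pickup that homes in on the player and records itself in the save game.
; Overlapping a BP_PlayableCharacter sets it as the follow target, which Tick chases with VInterpTo.
; Within DistanceToCollect it disables collision, swaps the idle particle for the picked effect and plays the Collected audio event.
; When that effect finishes, it increments CollectedParticles through BP_YakotakiInstance, saves, prints the total and destroys itself.
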(event OnComponentBeginOverlap(Collision)
  (params (OverlappedComponent :type Primitive%20Component%20Object%20Reference) (OtherActor :type Actor%20Object%20Reference) (OtherComp :type Primitive%20Component%20Object%20Reference) (OtherBodyIndex :type Integer) (bFromSweep :type Boolean) (SweepResult :type Hit%20Result%20Structure%20%28by%20ref%29))
  (bind _asbp_playable_character (Utilities|Casting|CastToBP_PlayableCharacter OtherActor))
  (Variables|Default|SetActorToFollow _asbp_playable_character))

(event OnSystemFinished(PickedParticle)
  (params (PSystem :type Niagara%20Component%20Object%20Reference))
  (bind _returnvalue (Game|GetGameInstance))
  (bind _asbp_yakotaki_instance (Utilities|Casting|CastToBP_YakotakiInstance _returnvalue))
  (bind _game_save_file (Variables|/Game/Project/00_Generic/Blueprints/GameInstance/BP_YakotakiInstance.BP_YakotakiInstance_C|GetGame%20Save%20File _asbp_yakotaki_instance))
  (bind _result (Math|Integer|IncrementInt (Variables|/Script/Yakotaki.YakotakiSaveGame|GetcollectedParticles _game_save_file))
    (:%20%20
      (bind _output_get (Variables|/Script/Yakotaki.YakotakiSaveGame|SetcollectedParticles _game_save_file _result))
      (Default|SaveGameFile _asbp_yakotaki_instance)
      (Development|PrintString (Utilities|String|ToString(Integer) _output_get))
      (Actor|DestroyActor))))

(event EventTick
  (params (DeltaSeconds :type Float%20%28single-precision%29))
  (bind _normalparticle (Variables|Default|GetNormalParticle))
  (Utilities|IsValid (Variables|Default|GetActorToFollow)
    (:Is%20Valid
      (Transformation|SetActorLocation (Math|Interpolation|VInterpTo (Transformation|GetActorLocation) (Transformation|GetActorLocation (Variables|Default|GetActorToFollow)) DeltaSeconds (Variables|Default|GetInterp%20Speed)) false false)
      (if (<= (Math|Vector|Distance(Vector) (Transformation|GetActorLocation (Variables|Default|GetActorToFollow)) (Transformation|GetActorLocation)) (Variables|Default|GetDistanceToCollect))
        (Collision|SetCollisionEnabled (Variables|Default|GetCollision) "NoCollision")
        (Rendering|SetVisibility _normalparticle false false)
        (Components|Activation|Deactivate _normalparticle)
        (Components|Activation|Activate (Variables|Default|GetPickedParticle) true)
        (Class|FMODBlueprintStatics|PlayEventAttached "/Game/FMOD/Events/One_Shots/SFX/Collectables/Collected.Collected" (Variables|Default|GetDefaultSceneRoot) "None" "0, 0, 0" "KeepRelativeOffset")
        (Variables|Default|SetActorToFollow 0)))))

(fn ConstructionScript)