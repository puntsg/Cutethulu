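; Playable DJ character whose airborne jump press spawns a BP_Platform_DJ ahead of it, replacing the previous one.
; Spawning requires a charge, a prior landing and no active coyote time; it clears the input buffer and briefly locks move and jump.
; The single charge refills on landing off its own platform type, on death, or on EnterTransform when a downward trace finds no such platform while grounded.
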(event OnDie(AdvancedHealthBehaviour)
  ;[0.15 0.15 0.15 0.5] Interfaces
  ;;[0.15 0.15 0.15 0.5] AdvanceHealthBehaviour
  (CallFunction|Refill))

(event Custom|Refill
  ;[0.15 0.15 0.15 0.5] Interfaces
  ;;[0.15 0.15 0.15 0.5] Refill Platforms
  (Variables|Default|SetPlatforms 1)
  (Variables|Default|SetHasLanded true))

(event Custom|Calculate%20Platform%20Movement%20Position
  (params (Platform :type BP%20Platform%20DJ%20Object%20Reference))
  (bind _returnvalue (Transformation|GetActorForwardVector))
  (bind _returnvalue_2 (Transformation|GetActorLocation))
  (bind _platform_distance (Variables|Default|GetPlatform%20Distance))
  (bind _returnvalue_3 (* _returnvalue _platform_distance))
  (bind _returnvalue_4 (+ _returnvalue_3 _returnvalue_2))
  ;[0.15 0.15 0.15 0.5] Custom Events
  ;;[0.15 0.15 0.15 0.5] Calculate the next position to platform after spawn and move it
  (Transformation|SetActorLocation Platform (Math|Vector|MakeVector (.x _returnvalue_4) (.y _returnvalue_4) (.z (Transformation|GetActorLocation Platform))) false false))

(event Custom|CustomEvent
  ;[0.15 0.15 0.15 0.5] Overrides
  ;;[0.15 0.15 0.15 0.5] DoubleJump + Create Platform
  ;;;[0.15 0.15 0.15 0.5] Creating Platform
  (CallFunction|SetCanMoveandJump true))

(event Input|EnhancedActionEvents|EnhancedInputActionIA_Jump
  (params (ActionValue :type Boolean) (ElapsedSeconds :type Float%20%28double-precision%29) (TriggeredSeconds :type Float%20%28double-precision%29) (InputAction :type Input%20Action%20Object%20Reference :default "/Game/ThirdPerson/Input/Actions/IA_Jump.IA_Jump"))
  ;[0.15 0.15 0.15 0.5] Overrides
  ;;[0.15 0.15 0.15 0.5] DoubleJump + Create Platform
  (:Started
    (if (Math|Boolean|ANDBoolean (> (Variables|Default|GetPlatforms) 0) (AI|Components|NavMovement|IsFalling (Variables|Character|GetCharacterMovement)) (not (Variables|Default|GetCanCoyoteTime)) (Variables|Default|GetHasLanded))
      ;;;[0.15 0.15 0.15 0.5] Creating Platform
      (bind _platformspawned (Variables|Default|GetPlatformSpawned)
        (:then
          (Default|DestroyBP _platformspawned))
        (:else
          _))
      (Variables|Default|SetHasLanded false)
      (bind _returnvalue (Game|SpawnActorfromClass "/Game/Project/00_Generic/Blueprints/Others/BP_Platform_DJ.BP_Platform_DJ_C" (Math|Transform|MakeTransform (Transformation|GetWorldLocation (Variables|Default|GetPlatformPosition)) "0, 0, 0" "1.000000,1.000000,1.000000") "Undefined" "MultiplyWithRoot" 0 0))
      (bind _output_get (Variables|Default|SetPlatformSpawned _returnvalue))
      (Variables|/Game/Project/00_Generic/Blueprints/Components/AC_InputBuffer.AC_InputBuffer_C|SetInputToStore (Variables|Default|GetAC_InputBuffer) 0)
      (CallFunction|CalculatePlatformMovementPosition _output_get)
      (CallFunction|SetCanMoveandJump false)
      (Variables|Default|SetPlatforms (- (Variables|Default|GetPlatforms) 1))
      (Utilities|Time|SetTimerbyEvent (delegate Custom|CustomEvent) 0.2))))

(event EventEnterTransform
  (bind _returnvalue (Transformation|GetActorLocation))
  ;[0.15 0.15 0.15 0.5] Interfaces
  (bind _outhit (Collision|LineTraceByChannel _returnvalue (- _returnvalue "0.000000,0.000000,200.000000") "TraceTypeQuery1" false 0 "ForDuration"))
  (if (and (not (AI|Components|NavMovement|IsFalling (Variables|Character|GetCharacterMovement))) (not (.bSuccess (Utilities|Casting|CastToBP_Platform_DJ (.hitactor _outhit)))))
    (CallFunction|Refill)))

(event EventOnLanded
  (params (Hit :type Hit%20Result%20Structure%20%28by%20ref%29))
  ;[0.15 0.15 0.15 0.5] Character Events
  ;;[0.15 0.15 0.15 0.5] Reset Platforms and Squash Stretch
  (CallFunction|SquashStretchLand)
  (if (.bSuccess (Utilities|Casting|CastToBP_Platform_DJ (.HitActor (Collision|BreakHitResult Hit))))
    _
    (else
      (CallFunction|Refill)))
  (|CallParentFunction Hit))

(fn ConstructionScript
  (|CallParentFunction))