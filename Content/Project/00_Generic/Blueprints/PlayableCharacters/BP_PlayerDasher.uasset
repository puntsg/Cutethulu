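; BP_PlayerDasher is a playable character whose sprint input triggers a dash along camera yaw using LaunchCharacter.
; Dashing is gated by cooldown, transformation state and an air-dash limit that resets on landing.
; One timeline squashes the mesh, re-enables dashing when finished and broadcasts cooldown progress to a player UI material.
; While dashing is on cooldown, PushCollider overlaps beyond a minimum distance send push messages along the character's forward vector.
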(event OnComponentBeginOverlap(PushCollider)
  (params (OverlappedComponent :type Primitive%20Component%20Object%20Reference) (OtherActor :type Actor%20Object%20Reference) (OtherComp :type Primitive%20Component%20Object%20Reference) (OtherBodyIndex :type Integer) (bFromSweep :type Boolean) (SweepResult :type Hit%20Result%20Structure%20%28by%20ref%29))
  (bind _returnvalue (Transformation|GetActorLocation))
  ;[0.15 0.15 0.15 0.5] Push/Destroy Objects
  (if (and (not (Variables|Default|GetCanDash)) (> (Math|Vector|Distance(Vector) (Math|Vector|MakeVector (.x (.location SweepResult)) (.y (.location SweepResult)) 0.0) (Math|Vector|MakeVector (.x _returnvalue) (.y _returnvalue) 0.0)) (Variables|Default|GetPushMinDistance)))
    (Class|BIPusheable|Push(Message) OtherActor (Transformation|GetActorForwardVector))))

(event Custom|Dash
  (bind _returnvalue (Transformation|GetActorScale3D))
  (bind _returnvalue_2 (Pawn|GetControlRotation :!class /Script/Engine.Pawn))
  (bind _returnvalue_3 (Math|Rotator|MakeRotator 0.0 0.0 (.yaw _returnvalue_2)))
  ;[0.15 0.15 0.15 0.5] Dash Skill
  (Variables|Default|SetCanDash false)
  (Audio|SpawnSoundatLocation "/Game/Project/00_Generic/Assets/Sounds/PlayerSounds/Dash/SFX_Player_Charge_Break_001.SFX_Player_Charge_Break_001" (.location (Transformation|GetActorTransform (Game|GetPlayerCharacter 0))) "0, 0, 0" 1.0 1.0 0.0 0 0)
  (Transformation|SetActorRotation _returnvalue_3)
  (Character|LaunchCharacter (* (Math|Vector|GetForwardVector _returnvalue_3) (Variables|Default|GetDash%20Impulse)) true true)
  (bind (_direction _cooldown _squash) (Timeline|TL_CooldownUI PlayFromStart)
    (:Update
      (Default|CallOnDashCooldownUpdate _cooldown)
      (Transformation|SetRelativeScale3D (Variables|Character|GetMesh) (Math|Vector|MakeVector _squash (.y _returnvalue) (.z _returnvalue))))
    (:Finished
      (Variables|Default|SetCanDash true))))

(event Custom|UpdateCooldownUI
  (params (Cooldown :type Float%20%28double-precision%29))
  (Rendering|Material|SetScalarParameterValue (Variables|/Game/Project/00_Generic/Blueprints/UI_HUD/WBP_Player.WBP_Player_C|GetCooldown%20MI (Variables|/Game/Project/00_Generic/Blueprints/PlayerController/BP_PlayerController.BP_PlayerController_C|GetPlayerUI (stale EventBeginPlay _asbp_player_controller))) "Cooldown" Cooldown :!class /Script/Engine.MaterialInstanceDynamic))

(event Input|EnhancedActionEvents|EnhancedInputActionIA_Sprint
  (params (ActionValue :type Boolean) (ElapsedSeconds :type Float%20%28double-precision%29) (TriggeredSeconds :type Float%20%28double-precision%29) (InputAction :type Input%20Action%20Object%20Reference :default "/Game/ThirdPerson/Input/Actions/IA_Sprint.IA_Sprint"))
  ;[0.15 0.15 0.15 0.5] Use the Ability of Dash
  (:Started
    (Utilities|Dash/InAirConditions
      (:True
        (CallFunction|Dash)))))

(event EventBeginPlay
  (|CallParentFunction)
  (bind _asbp_player_controller (Utilities|Casting|CastToBP_PlayerController (Game|GetPlayerController 0)))
  (EventDispatchers|BindEventtoOnDashCooldownUpdate (delegate Custom|UpdateCooldownUI)))

(event EventOnLanded
  (params (Hit :type Hit%20Result%20Structure%20%28by%20ref%29))
  ;[0.15 0.15 0.15 0.5] Reset DashesInAir on Land
  (Variables|Default|SetDashesInAir 0)
  (|CallParentFunction Hit))

(fn ConstructionScript
  (|CallParentFunction))