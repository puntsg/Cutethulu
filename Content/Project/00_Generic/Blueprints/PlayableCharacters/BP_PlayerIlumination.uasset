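; Playable character whose held ability emits light that affects surrounding actors.
; Holding IA_Ability enables a radius sphere and plays a timeline that drives point light intensity, walk speed and sphere scale together.
; Releasing reverses that timeline, switching the sphere's collision off once it finishes rewinding.
; Actors entering or leaving the sphere receive messages to start or stop receiving light.
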(event OnComponentBeginOverlap(IluminationRadiusSphere)
  (params (OverlappedComponent :type Primitive%20Component%20Object%20Reference) (OtherActor :type Actor%20Object%20Reference) (OtherComp :type Primitive%20Component%20Object%20Reference) (OtherBodyIndex :type Integer) (bFromSweep :type Boolean) (SweepResult :type Hit%20Result%20Structure%20%28by%20ref%29))
  ;[0.15 0.15 0.15 0.5] Colliders
  ;;[0.15 0.15 0.15 0.5] Illumination radius effect
  (Class|BILightReactive|OnLightReceived(Message) OtherActor))

(event OnComponentEndOverlap(IluminationRadiusSphere)
  (params (OverlappedComponent :type Primitive%20Component%20Object%20Reference) (OtherActor :type Actor%20Object%20Reference) (OtherComp :type Primitive%20Component%20Object%20Reference) (OtherBodyIndex :type Integer))
  ;[0.15 0.15 0.15 0.5] Colliders
  ;;[0.15 0.15 0.15 0.5] Illumination radius effect
  (Class|BILightReactive|OnStopReceivingLight(Message) OtherActor))

(event Input|EnhancedActionEvents|EnhancedInputActionIA_Ability
  (params (ActionValue :type Boolean) (ElapsedSeconds :type Float%20%28double-precision%29) (TriggeredSeconds :type Float%20%28double-precision%29) (InputAction :type Input%20Action%20Object%20Reference :default "/Game/ThirdPerson/Input/Actions/IA_Ability.IA_Ability"))
  ;[0.15 0.15 0.15 0.5] Overrides
  ;;[0.15 0.15 0.15 0.5] Illumination Skill
  (:Started
    (Collision|SetCollisionEnabled (Variables|Default|GetIluminationRadiusSphere) "QueryAndPhysics")
    (bind (_direction _ligting_intencity _speed _lightaffectradius) (Timeline|ParamsTimeline Play)
      (:Update
        (Rendering|Components|Light|SetIntensity (Variables|Default|GetPointLight) _ligting_intencity)
        (Variables|/Script/Engine.CharacterMovementComponent|SetMaxWalkSpeed (Variables|Character|GetCharacterMovement) _speed)
        (Transformation|SetRelativeScale3D (Variables|Default|GetIluminationRadiusSphere) _lightaffectradius))
      (:Finished
        (if (Utilities|Enum|Equal(Enum) _direction "Backward")
          (Collision|SetCollisionEnabled (Variables|Default|GetIluminationRadiusSphere) "NoCollision")))))
  (:Completed
    (Timeline|ParamsTimeline Reverse)))

(event EventBeginPlay)

(event Collision|EventActorBeginOverlap
  (params (OtherActor :type Actor%20Object%20Reference)))

(event EventTick
  (params (DeltaSeconds :type Float%20%28single-precision%29)))

(fn ConstructionScript
  (|CallParentFunction))