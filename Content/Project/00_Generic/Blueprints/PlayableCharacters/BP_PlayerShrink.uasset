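; BP_PlayerShrink is a playable character whose ability input toggles it between normal and shrunken size.
; Each toggle swaps jump velocity, walk speed, braking deceleration and gravity, while one timeline plays forward or in reverse to scale the actor uniformly.
; Input is ignored while transforming or mid-timeline, and CanExecuteTransform is true only after returning to normal size.
; Restoring sets braking deceleration to a hard-coded zero rather than a stored normal value.
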(event Input|EnhancedActionEvents|EnhancedInputActionIA_Ability
  (params (ActionValue :type Boolean) (ElapsedSeconds :type Float%20%28double-precision%29) (TriggeredSeconds :type Float%20%28double-precision%29) (InputAction :type Input%20Action%20Object%20Reference :default "/Game/ThirdPerson/Input/Actions/IA_Ability.IA_Ability"))
  (if (and (not (Variables|Default|GetisTransforming)) (not (Audio|Components|Audio|IsPlaying (Variables|Default|GetShrinkTimeline))))
    (if (not (Variables|Default|GetShrinked))
      (Variables|Default|SetShrinked true)
      (Variables|/Script/Engine.CharacterMovementComponent|SetJumpZVelocity (Variables|Character|GetCharacterMovement) (Variables|Default|GetNewJump))
      (Variables|/Script/Engine.CharacterMovementComponent|SetMaxWalkSpeed (Variables|Character|GetCharacterMovement) (Variables|Default|GetNewSpeed))
      (Variables|/Script/Engine.CharacterMovementComponent|SetBrakingDecelerationWalking (Variables|Character|GetCharacterMovement) (Variables|Default|GetNewDeceleration))
      (Variables|/Script/Engine.CharacterMovementComponent|SetGravityScale (Variables|Character|GetCharacterMovement) (Variables|Default|GetNewGravity))
      (bind _sizemultiplier (Timeline|ShrinkTimeline PlayFromStart)
        (:Update
          (Transformation|SetActorScale3D (Math|Vector|MakeVector _sizemultiplier _sizemultiplier _sizemultiplier)))
        (:Finished
          (Variables|Default|SetCanExecuteTransform (not (Variables|Default|GetShrinked)))))
      (else
        (Variables|Default|SetShrinked false)
        (Variables|/Script/Engine.CharacterMovementComponent|SetJumpZVelocity (Variables|Character|GetCharacterMovement) (Variables|Default|GetNormalJump))
        (Variables|/Script/Engine.CharacterMovementComponent|SetMaxWalkSpeed (Variables|Character|GetCharacterMovement) (Variables|Default|GetNormalSpeed))
        (Variables|/Script/Engine.CharacterMovementComponent|SetBrakingDecelerationWalking (Variables|Character|GetCharacterMovement) 0.0)
        (Variables|/Script/Engine.CharacterMovementComponent|SetGravityScale (Variables|Character|GetCharacterMovement) (Variables|Default|GetNormalGravity))
        (Timeline|ShrinkTimeline ReverseFromEnd)))))

(event EventBeginPlay
  (|CallParentFunction) ; This node is disabled and will not be called.\nDrag off pins to build functionality.
)

(fn ConstructionScript
  (|CallParentFunction))