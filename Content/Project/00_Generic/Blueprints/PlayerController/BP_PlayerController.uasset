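; Player controller that manages the game's UI widgets and pause entry, and sets rotation and view target on possession to avoid camera flicks.
; BeginPlay creates the initially hidden player UI, adds the game instance's fade widget to the viewport and creates the collectables widget.
; IA_Pause opens a pause menu, pauses the game and switches to UI-only input.
; A timeline temporarily fades in the collectables widget, while helper functions drive screen fades.
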(event Input|EnhancedActionEvents|EnhancedInputActionIA_Pause
  (params (ActionValue :type Boolean) (ElapsedSeconds :type Float%20%28double-precision%29) (TriggeredSeconds :type Float%20%28double-precision%29) (InputAction :type Input%20Action%20Object%20Reference :default "/Game/ThirdPerson/Input/Actions/IA_Pause.IA_Pause"))
  ;[0.15 0.15 0.15 0.5] Activates pause menu and UI/mouse mode
  (:Started
    (bind _returnvalue (UserInterface|CreateWidget "/Game/Project/00_Generic/Blueprints/UI_HUD/PauseMenu.PauseMenu_C"))
    (bind _output_get (Variables|UI|SetPauseMenu _returnvalue))
    (UserInterface|Viewport|AddtoViewport _output_get 0)
    (Game|SetGamePaused true)
    (Input|SetInputModeUIOnly self 0 "DoNotLock" false)
    (Variables|Default|SetbShowMouseCursor true)))

(event EventBeginPlay
  ;[0.15 0.15 0.15 0.5] Init UIs
  (bind _returnvalue (UserInterface|CreateWidget "/Game/Project/00_Generic/Blueprints/UI_HUD/WBP_Player.WBP_Player_C"))
  (bind _output_get (Variables|UI|SetPlayerUI _returnvalue))
  (UserInterface|Viewport|AddtoViewport _output_get 0)
  (UIFunctions|ShowPlayerUI false)
  (bind _asbp_cutethulu_instance (Utilities|Casting|CastToBP_YakotakiInstance (Game|GetGameInstance))
    (:then
      (Utilities|IsValid (Variables|/Game/Project/00_Generic/Blueprints/GameInstance/BP_YakotakiInstance.BP_YakotakiInstance_C|GetFadeWRef _asbp_cutethulu_instance)
        (:Is%20Valid
          (UserInterface|Viewport|AddtoViewport (Variables|/Game/Project/00_Generic/Blueprints/GameInstance/BP_YakotakiInstance.BP_YakotakiInstance_C|GetFadeWRef _asbp_cutethulu_instance) 0))))
    (:CastFailed
      _))
  (bind _returnvalue_2 (UserInterface|CreateWidget "/Game/Project/00_Generic/Blueprints/UI_HUD/WBP_LevelCollectables.WBP_LevelCollectables_C"))
  (bind _output_get_2 (Variables|UI|SetCollectablesWidget _returnvalue_2))
  (UserInterface|Viewport|AddtoViewport _output_get_2 0)
  (CallFunction|HideCollectablesWidget))

(event EventPossess
  (params (PossessedPawn :type Pawn%20Object%20Reference))
  ;[0.15 0.15 0.15 0.5] Force camera rotation on transform/posses to avoid flick
  (Pawn|SetControlRotation (Variables|Default|GetPrevRotation))
  (Game|Player|SetViewTargetwithBlend PossessedPawn 0.0 "VTBlend_Linear" 0.0 false))

(event Custom|HideCollectablesWidget
  ;[0.15 0.15 0.15 0.5] Shows temporaly collectables widget
  (bind (_direction _alpha) (Timeline|CollectablesWidgetAlphaTimeline Reverse)
    (:Update
      (Widget|SetRenderOpacity (Variables|UI|GetCollectablesWidget) _alpha))
    (:Finished
      (if (Utilities|Enum|Equal(Enum) _direction "Forward")
        (Utilities|FlowControl|Delay (Variables|Default|GetCollectables%20UI%20display%20time))
        (CallFunction|HideCollectablesWidget)))))

(event Custom|ShowCollectablesWidgets
  ;[0.15 0.15 0.15 0.5] Shows temporaly collectables widget
  (bind (_direction _alpha) (Timeline|CollectablesWidgetAlphaTimeline Play)
    (:Update
      (Widget|SetRenderOpacity (Variables|UI|GetCollectablesWidget) _alpha))
    (:Finished
      (if (Utilities|Enum|Equal(Enum) _direction "Forward")
        (Utilities|FlowControl|Delay (Variables|Default|GetCollectables%20UI%20display%20time))
        (CallFunction|HideCollectablesWidget)))))

(fn ConstructionScript)

(fn ShowPlayerUI
  (params (IsVisible%28PlayerUI%29 :type Boolean))
  (bind _playerui (Variables|UI|GetPlayerUI))
  (if IsVisible%28PlayerUI%29
    (Widget|SetVisibility _playerui "Visible")
    (else
      (Widget|SetVisibility _playerui "Collapsed"))))

(fn Fadein
  (bind _fadewref (Variables|UI|GetFadeWRef))
  (Widget|SetVisibility _fadewref "Visible")
  (UserInterface|Animation|PlayAnimation _fadewref (Variables|/Game/Project/00_Generic/Blueprints/UI_HUD/WBP_Fade.WBP_Fade_C|GetFadeIn _fadewref) 0.0 1 "Forward" 1.0 false))

(fn FadeOut
  (bind _fadewref (Variables|UI|GetFadeWRef))
  (Widget|SetVisibility _fadewref "Hidden")
  (UserInterface|Animation|PlayAnimation _fadewref (Variables|/Game/Project/00_Generic/Blueprints/UI_HUD/WBP_Fade.WBP_Fade_C|GetFadeOut _fadewref) 0.0 1 "Forward" 1.0 false))