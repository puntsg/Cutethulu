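; Dialogue citizen actor that speaks to the player through a text system component when they are nearby.
; A trigger collider starts speech when the playable character enters and stops it on exit, with a short delayed overlap check at BeginPlay for players already inside.
; World-load events swap the skeletal mesh material between horror and cute variants.
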(event OnComponentBeginOverlap(TextCollider)
  (params (OverlappedComponent :type Primitive%20Component%20Object%20Reference) (OtherActor :type Actor%20Object%20Reference) (OtherComp :type Primitive%20Component%20Object%20Reference) (OtherBodyIndex :type Integer) (bFromSweep :type Boolean) (SweepResult :type Hit%20Result%20Structure%20%28by%20ref%29))
  ;[0.15 0.15 0.15 0.5] Colliders to Start /End Dialogue
  (Utilities|Casting|CastToBP_PlayableCharacter OtherActor)
  (Default|Speak (Variables|Default|GetSC_TextSystem)))

(event OnComponentEndOverlap(TextCollider)
  (params (OverlappedComponent :type Primitive%20Component%20Object%20Reference) (OtherActor :type Actor%20Object%20Reference) (OtherComp :type Primitive%20Component%20Object%20Reference) (OtherBodyIndex :type Integer))
  ;[0.15 0.15 0.15 0.5] Colliders to Start /End Dialogue
  (Utilities|Casting|CastToBP_PlayableCharacter OtherActor)
  (Default|StopSpeak (Variables|Default|GetSC_TextSystem)))

(event EventBeginPlay
  (Utilities|FlowControl|Delay 0.1)
  (if (Collision|IsOverlappingActor (Variables|Default|GetTextCollider) (Game|GetPlayerCharacter 0) :!class /Script/Engine.PrimitiveComponent)
    (Default|Speak (Variables|Default|GetSC_TextSystem))))

(event Collision|EventActorBeginOverlap
  (params (OtherActor :type Actor%20Object%20Reference)))

(event EventTick
  (params (DeltaSeconds :type Float%20%28single-precision%29)))

(event EventOnHorrorLoaded
  ;[0.15 0.15 0.15 0.5] Change Materials on world load
  (Rendering|Material|SetMaterial (Variables|Default|GetSkeletalMesh) 0 (Variables|Default|GetMaterial%20Horror)))

(event EventOnCuteLoaded
  ;[0.15 0.15 0.15 0.5] Change Materials on world load
  (Rendering|Material|SetMaterial (Variables|Default|GetSkeletalMesh) 0 (Variables|Default|GetMaterial%20Cute)))

(fn ConstructionScript)