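; BP_FollowerParticlesFX is an actor, named for particle effects, that follows the character the player controls.
; On BeginPlay it targets player pawn 0 and registers a callback with YakoTakiGameMode for player transform events.
; That callback switches the followed character to the one being transformed into.
; Tick moves the actor to that character's location every frame without sweep, copying position only rather than attaching.
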(event Custom|AssignParticlesToNewPawn
  (params (CurrentPlayableCharacter :type BP%20Playable%20Character%20Object%20Reference) (CharacterToTransform :type BP%20Playable%20Character%20Object%20Reference))
  ;[0.15 0.15 0.15 0.5] Assigna personatge al canviar/transformar
  (Variables|Default|SetCharacterToFollow CharacterToTransform))

(event EventBeginPlay
  ;[0.15 0.15 0.15 0.5] Assigna personatge al canviar/transformar
  (Variables|Default|SetCharacterToFollow (Game|Player|GetPlayerPawn 0))
  (EventDispatchers|AssignOnPlayerTransform (.AsYako%20Taki%20Game%20Mode (Utilities|Casting|CastToYakoTakiGameMode (Game|GetGameMode))) (delegate Custom|AssignParticlesToNewPawn)))

(event EventTick
  (params (DeltaSeconds :type Float%20%28single-precision%29))
  ;[0.15 0.15 0.15 0.5] Actualitza posició
  (Transformation|SetActorLocation (Transformation|GetActorLocation (Variables|Default|GetCharacterToFollow)) false false))

(fn ConstructionScript)