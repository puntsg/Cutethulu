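; BP_Fragment is a collectible portal piece that removes itself on BeginPlay if its level is already completed.
; It stays hidden and non-colliding until the Cute world loads, then a sequence moves it from seed to collect spot, enabling collision, effect and sound.
; Player overlap updates the fragment UI and plays a sequence to the portal, which is notified before the fragment destroys itself.
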(event OnComponentBeginOverlap(Sphere)
  (params (OverlappedComponent :type Primitive%20Component%20Object%20Reference) (OtherActor :type Actor%20Object%20Reference) (OtherComp :type Primitive%20Component%20Object%20Reference) (OtherBodyIndex :type Integer) (bFromSweep :type Boolean) (SweepResult :type Hit%20Result%20Structure%20%28by%20ref%29))
  (bind _audioplayer (Variables|Default|GetAudioPlayer))
  ;[0.15 0.15 0.15 0.5] Second animation ->to portal
  (Utilities|Casting|CastToBP_PlayableCharacter OtherActor)
  (if (and (not (Variables|State|GetCollected)) (Variables|State|GetCanBeCollected))
    (Variables|State|SetCanBeCollected false)
    (Variables|State|SetCollected true)
    (Default|OnFragmentCollectedEvent (Variables|/Game/Project/00_Generic/Blueprints/GameModes/YakoTakiGameMode.YakoTakiGameMode_C|GetPortal%20fragmentsUI (.AsYako%20Taki%20Game%20Mode (Utilities|Casting|CastToYakoTakiGameMode (Game|GetGameMode)))))
    (bind _returnvalue (Sequencer|Player|CreateLevelSequencePlayer (Variables|Sequences|GetToPortalSequence) (Utilities|Struct|MakeMovieSceneSequencePlaybackSettings false (Utilities|Struct|MakeMovieSceneSequenceLoopCount 0) (Utilities|Struct|MakeMovieSceneSequenceTickInterval 0.0 0.0 false false) 1.0 0.0 false false false false false false "None" true)))
    (bind _output_get (Variables|Sequences|SetLevelSequencePlayer _returnvalue))
    (Sequencer|Player|Play _output_get :!class /Script/MovieScene.MovieSceneSequencePlayer)
    (EventDispatchers|BindEventtoOnFinished _output_get (delegate Custom|CustomEvent))
    (Rendering|SetVisibility (Variables|Default|GetEffect) false false)
    (Audio|Components|Audio|Stop _audioplayer)
    (Audio|Components|Audio|SetSound _audioplayer "/Game/Project/00_Generic/Assets/Sounds/SFX/Objects/Portal/SFX_Collect_PortalPieces.SFX_Collect_PortalPieces")
    (Audio|Components|Audio|Play _audioplayer 0.0)))

(event Custom|CustomEvent
  ;[0.15 0.15 0.15 0.5] Second animation ->to portal
  (Development|PrintString "InPortal")
  (bind _outactors (Actor|GetAllActorsOfClass "/Game/Project/00_Generic/Blueprints/Scenario/BP_Portal.BP_Portal_C"))
  (Default|OnFragmentRecievedEvent (Utilities|Array|Get(acopy) _outactors))
  (Actor|DestroyActor))

(event Custom|OnFinished_Event
  ;[0.15 0.15 0.15 0.5] First animation seed->Collect location
  (Sequencer|Player|Stop (stale EventOnCuteLoaded _output_get) :!class /Script/MovieScene.MovieSceneSequencePlayer)
  (Collision|SetCollisionEnabled (Variables|Default|GetStaticMesh) "QueryAndPhysics")
  (Collision|SetCollisionEnabled (Variables|Default|GetSphere) "QueryOnly")
  (Development|PrintString "ReadyToCollect")
  (Variables|State|SetCanBeCollected true)
  (bind _returnvalue (Audio|SpawnSoundatLocation "/Game/Project/00_Generic/Assets/Sounds/SFX/Objects/Portal/Default_PortalPieces_1.Default_PortalPieces_1" (Transformation|GetActorLocation) "0, 0, 0" 1.0 1.0 0.0 "/USDCore/USDDefaultAttenuation.USDDefaultAttenuation" 0))
  (Variables|Default|SetAudioPlayer _returnvalue)
  (Rendering|SetVisibility (Variables|Default|GetEffect) true false))

(event EventOnHorrorLoaded
  ;[0.15 0.15 0.15 0.5] Check if level completed for destroy itself
  (Development|SetHiddeninGame (Variables|Default|GetStaticMesh) true true)
  (Collision|SetCollisionEnabled (Variables|Default|GetStaticMesh) "NoCollision")
  (Collision|SetCollisionEnabled (Variables|Default|GetSphere) "NoCollision"))

(event EventOnCuteLoaded
  ;[0.15 0.15 0.15 0.5] First animation seed->Collect location
  (Development|SetHiddeninGame (Variables|Default|GetStaticMesh) false true)
  (bind _returnvalue (Sequencer|Player|CreateLevelSequencePlayer (Variables|Sequences|GetFromSeedToDestinationSequence) (Utilities|Struct|MakeMovieSceneSequencePlaybackSettings false (Utilities|Struct|MakeMovieSceneSequenceLoopCount 0) (Utilities|Struct|MakeMovieSceneSequenceTickInterval 0.0 0.0 false false) 1.0 0.0 false false false false false false "None" true)))
  (bind _output_get (Variables|Sequences|SetLevelSequencePlayer _returnvalue))
  (Sequencer|Player|Play _output_get :!class /Script/MovieScene.MovieSceneSequencePlayer)
  (EventDispatchers|AssignOnFinished _output_get (delegate Custom|OnFinished_Event)))

(event EventBeginPlay
  ;[0.15 0.15 0.15 0.5] Check if level completed for destroy itself
  (bind _returnvalue (Class|DualLevel|IsLevelCompleted (Class|DualLevelFunctionLibrary|GetDualLevel)))
  (if _returnvalue
    (Actor|DestroyActor)
    (else
      (Development|SetHiddeninGame (Variables|Default|GetStaticMesh) true true)
      (Collision|SetCollisionEnabled (Variables|Default|GetStaticMesh) "NoCollision")
      (Collision|SetCollisionEnabled (Variables|Default|GetSphere) "NoCollision"))))

(fn ConstructionScript)