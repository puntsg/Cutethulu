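; Moving platform that reacts to light by switching its travel direction through waiting, reverse and braking flags.
; Losing light sets braking and starts a one-second timer that then switches the platform to reverse.
; Receiving light while that timer handle is valid clears it and sets forward travel.
; The graph only sets state, with no movement code of its own.
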(event Custom|GoBackwards
  (Variables|Default|Setbreaking false)
  (Variables|Default|Setreverse true)
  (Variables|Default|SetisWaiting false))

(event Custom|GoForward
  (Variables|Default|SetisWaiting false)
  (Variables|Default|Setreverse false)
  (Variables|Default|Setbreaking false))

(event EventOnLightReceived
  (bind _reversetimer (Variables|Default|GetReverseTimer))
  (if (Utilities|Time|IsValidTimerHandle _reversetimer)
    (Utilities|Time|ClearandInvalidateTimerbyHandle _reversetimer)
    (CallFunction|GoForward)))

(event EventOnStopReceivingLight
  (Variables|Default|Setbreaking true)
  (bind _returnvalue (Utilities|Time|SetTimerbyEvent (delegate Custom|GoBackwards) 1.0))
  (Variables|Default|SetReverseTimer _returnvalue))

(fn ConstructionScript)