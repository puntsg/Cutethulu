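; Light-reactive platform that becomes visible and solid when lit, and fades away when the light leaves.
; BeginPlay creates a dynamic material instance with zero opacity.
; Light interface events drive one opacity timeline: losing light plays it from start, receiving light reverses it at ten times the rate.
; Timeline updates enable mesh collision, which switches off only when the forward fade finishes.
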(event EventBeginPlay
  (bind _staticmesh (Variables|Default|GetStaticMesh))
  ;[0.15 0.15 0.15 0.5] BeginPlay
  ;;[0.15 0.15 0.15 0.5] Creation and assignation of Material Instance Dynamic
  (bind _returnvalue (Rendering|Material|CreateDynamicMaterialInstance _staticmesh 0 (Rendering|Material|GetMaterial _staticmesh (Variables|Default|GetMaterial%20index)) "None" :!class /Script/Engine.PrimitiveComponent))
  (bind _output_get (Variables|Default|SetMID _returnvalue))
  (Rendering|Material|SetMaterial (Variables|Default|GetStaticMesh) (Variables|Default|GetMaterial%20index) _output_get)
  (Rendering|Material|SetScalarParameterValue _output_get "Opacity" 0.0 :!class /Script/Engine.MaterialInstanceDynamic))

(event EventOnLightReceived
  (bind _tl_material_opacity (Variables|Default|GetTL_Material%20Opacity))
  ;[0.15 0.15 0.15 0.5] Interfaces
  ;;[0.15 0.15 0.15 0.5] On Light Received and Stop Receiving
  (bind (_direction _opacity) (Timeline|TL_Material%20Opacity Reverse)
    (:Update
      (switch Utilities|FlowControl|Switch|SwitchonETimelineDirection _direction
        (:Forward
          (Components|Timeline|SetPlayRate _tl_material_opacity 1.0))
        (:Backward
          (Components|Timeline|SetPlayRate _tl_material_opacity 1e+01)))
      (Rendering|Material|SetScalarParameterValue (Variables|Default|GetMID) "Opacity" _opacity :!class /Script/Engine.MaterialInstanceDynamic)
      (Collision|SetCollisionEnabled (Variables|Default|GetStaticMesh) "QueryAndPhysics"))
    (:Finished
      (switch Utilities|FlowControl|Switch|SwitchonETimelineDirection _direction
        (:Forward
          (Collision|SetCollisionEnabled (Variables|Default|GetStaticMesh) "NoCollision"))))))

(event EventOnStopReceivingLight
  (bind _tl_material_opacity (Variables|Default|GetTL_Material%20Opacity))
  ;[0.15 0.15 0.15 0.5] Interfaces
  ;;[0.15 0.15 0.15 0.5] On Light Received and Stop Receiving
  (bind (_direction _opacity) (Timeline|TL_Material%20Opacity PlayFromStart)
    (:Update
      (switch Utilities|FlowControl|Switch|SwitchonETimelineDirection _direction
        (:Forward
          (Components|Timeline|SetPlayRate _tl_material_opacity 1.0))
        (:Backward
          (Components|Timeline|SetPlayRate _tl_material_opacity 1e+01)))
      (Rendering|Material|SetScalarParameterValue (Variables|Default|GetMID) "Opacity" _opacity :!class /Script/Engine.MaterialInstanceDynamic)
      (Collision|SetCollisionEnabled (Variables|Default|GetStaticMesh) "QueryAndPhysics"))
    (:Finished
      (switch Utilities|FlowControl|Switch|SwitchonETimelineDirection _direction
        (:Forward
          (Collision|SetCollisionEnabled (Variables|Default|GetStaticMesh) "NoCollision"))))))

(fn ConstructionScript)