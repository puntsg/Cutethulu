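; BP_Ray is a scenario actor that renders a coloured ray mesh whose opacity depends on the player's distance.
; BeginPlay creates a dynamic instance of M_Cylinder on its static mesh and applies the colour and multiplier.
; Tick maps player pawn distance between MinDistance and MaxDistance to Opacity, so it fades out as the player approaches.
; Tick also reapplies both colours and prints the parameters for debugging.
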(event EventBeginPlay
  (Development|PrintString "Hello")
  (bind _returnvalue (Rendering|Material|CreateDynamicMaterialInstance (Variables|Default|GetStaticMesh) 0 "/Game/Project/00_Generic/Assets/VFX/Fragment/M_Cylinder.M_Cylinder" "None" :!class /Script/Engine.PrimitiveComponent))
  (bind _output_get (Variables|Default|SetMaterial _returnvalue))
  (Rendering|Material|SetVectorParameterValue _output_get "Colour" (Variables|Default|GetPrimaryColour) :!class /Script/Engine.MaterialInstanceDynamic)
  (Rendering|Material|SetVectorParameterValue _output_get "ColourMultiplier" (Variables|Default|GetColourMultiplier) :!class /Script/Engine.MaterialInstanceDynamic))

(event EventTick
  (params (DeltaSeconds :type Float%20%28single-precision%29))
  (bind _returnvalue (Game|Player|GetPlayerPawn 0))
  (bind _returnvalue_2 (Transformation|GetActorLocation))
  (bind _material (Variables|Default|GetMaterial))
  (bind _mindistance (Variables|Default|GetMinDistance))
  (bind _maxdistance (Variables|Default|GetMaxDistance))
  (bind _primarycolour (Variables|Default|GetPrimaryColour))
  (bind _colourmultiplier (Variables|Default|GetColourMultiplier))
  (bind _returnvalue_3 (Transformation|GetActorLocation _returnvalue))
  (bind _returnvalue_4 (Math|Vector|Distance(Vector) _returnvalue_3 _returnvalue_2))
  (bind _returnvalue_5 (Math|Float|MapRangeClamped _returnvalue_4 _mindistance _maxdistance 0.0 1.0))
  (Rendering|Material|SetScalarParameterValue _material "Opacity" _returnvalue_5 :!class /Script/Engine.MaterialInstanceDynamic)
  (Rendering|Material|SetVectorParameterValue _material "Colour" _primarycolour :!class /Script/Engine.MaterialInstanceDynamic)
  (Rendering|Material|SetVectorParameterValue _material "ColourMultiplier" _colourmultiplier :!class /Script/Engine.MaterialInstanceDynamic)
  (Development|PrintString (Utilities|String|Append "Setting " (Utilities|GetDisplayName _material) " params to: Distance:" (Utilities|String|ToString(Float) _returnvalue_5) "primary colour:" (Utilities|String|ToString(Integer) _primarycolour) "colour multiplier:" (Utilities|String|ToString(Integer) _colourmultiplier))))

(fn ConstructionScript)