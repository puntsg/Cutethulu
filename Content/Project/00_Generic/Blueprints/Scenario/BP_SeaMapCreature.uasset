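; Interactive sea map creature that loops along a spline route with squash-and-stretch animation, passing a transform class to the game mode on interaction.
; Tick accelerates or brakes it by player proximity, toggling Niagara particles at a speed threshold.
; Sphere overlap registers it as the player's interactive, shows an overlay outline and blends rotation to track the player, subject to an angle check.
; A second collider triggers speech; horror/cute world events swap materials.
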(event OnComponentBeginOverlap(TextCollision)
  (params (OverlappedComponent :type Primitive%20Component%20Object%20Reference) (OtherActor :type Actor%20Object%20Reference) (OtherComp :type Primitive%20Component%20Object%20Reference) (OtherBodyIndex :type Integer) (bFromSweep :type Boolean) (SweepResult :type Hit%20Result%20Structure%20%28by%20ref%29))
  ;[0.15 0.15 0.15 0.5] Colliders
  ;;[0.15 0.15 0.15 0.5] Start and End Citizens Dialogue
  (Utilities|Casting|CastToBP_PlayableCharacter OtherActor)
  (Default|Speak (Variables|Default|GetSC_TextSystem)))

(event OnComponentEndOverlap(Sphere)
  (params (OverlappedComponent :type Primitive%20Component%20Object%20Reference) (OtherActor :type Actor%20Object%20Reference) (OtherComp :type Primitive%20Component%20Object%20Reference) (OtherBodyIndex :type Integer))
  ;[0.15 0.15 0.15 0.5] Colliders
  ;;[0.15 0.15 0.15 0.5] Start and End Citizens Following
  (bind _asbp_playable_character (Utilities|Casting|CastToBP_PlayableCharacter OtherActor))
  (Variables|Default|SetCurrentRotation (Variables|/Script/Engine.SceneComponent|GetRelativeRotation (Variables|Default|GetCharacterOffset)))
  (Variables|/Game/Project/00_Generic/Blueprints/PlayableCharacters/BP_PlayableCharacter.BP_PlayableCharacter_C|SetCurrentInteractive _asbp_playable_character 0)
  (CallFunction|SetInteracted false)
  (CallFunction|StopFollowing))

(event OnComponentBeginOverlap(Sphere)
  (params (OverlappedComponent :type Primitive%20Component%20Object%20Reference) (OtherActor :type Actor%20Object%20Reference) (OtherComp :type Primitive%20Component%20Object%20Reference) (OtherBodyIndex :type Integer) (bFromSweep :type Boolean) (SweepResult :type Hit%20Result%20Structure%20%28by%20ref%29))
  ;[0.15 0.15 0.15 0.5] Colliders
  ;;[0.15 0.15 0.15 0.5] Start and End Citizens Following
  (bind _asbp_playable_character (Utilities|Casting|CastToBP_PlayableCharacter OtherActor))
  (Variables|Default|SetPlayer _asbp_playable_character)
  (Variables|Default|SetCurrentRotation (Variables|/Script/Engine.SceneComponent|GetRelativeRotation (Variables|Default|GetCharacterOffset)))
  (Variables|/Game/Project/00_Generic/Blueprints/PlayableCharacters/BP_PlayableCharacter.BP_PlayableCharacter_C|SetCurrentInteractive (Variables|Default|GetPlayer) self)
  (Utilities|Casting|CastToYakoTakiGameMode (Game|GetGameMode))
  (CallFunction|SetInteracted true)
  (CallFunction|Following))

(event OnComponentEndOverlap(TextCollision)
  (params (OverlappedComponent :type Primitive%20Component%20Object%20Reference) (OtherActor :type Actor%20Object%20Reference) (OtherComp :type Primitive%20Component%20Object%20Reference) (OtherBodyIndex :type Integer))
  ;[0.15 0.15 0.15 0.5] Colliders
  ;;[0.15 0.15 0.15 0.5] Start and End Citizens Dialogue
  (Utilities|Casting|CastToBP_PlayableCharacter OtherActor)
  (Default|StopSpeak (Variables|Default|GetSC_TextSystem)))

(event Custom|SetInteracted
  (params (NewState :type Boolean))
  (bind _outlinematerialinstance (Variables|InteractionParams|GetOutlineMaterialInstance))
  ;[0.15 0.15 0.15 0.5] Custom Events
  ;;[0.15 0.15 0.15 0.5] Add/Remove Outliner
  (bind _output_get (Variables|InteractionParams|SetIsPlayerNearby NewState))
  (if _output_get
    (Rendering|Material|SetScalarParameterValue _outlinematerialinstance "Thickness" 5.0 :!class /Script/Engine.MaterialInstanceDynamic)
    (else
      (Rendering|Material|SetScalarParameterValue _outlinematerialinstance "Thickness" 0.0 :!class /Script/Engine.MaterialInstanceDynamic))))

(event Custom|PlaySound
  ;[0.15 0.15 0.15 0.5] Custom Events
  (if (not (Variables|InteractionParams|GetIsPlayingSound))
    (Variables|InteractionParams|SetIsPlayingSound true)
    (bind _returnvalue (Audio|SpawnSoundatLocation (Variables|InteractionParams|GetSound) (Transformation|GetActorLocation) "0, 0, 0" 1.0 1.0 0.0 0 0))
    (EventDispatchers|AssignOnAudioFinished _returnvalue (delegate Custom|OnAudioFinished_Event))))

(event Custom|CalculateSpeed
  (bind _niagara (Variables|Default|GetNiagara))
  ;[0.15 0.15 0.15 0.5] Custom Events
  ;;[0.15 0.15 0.15 0.5] Calculate Speed if player is nearby or not
  (if (Variables|InteractionParams|GetIsPlayerNearby)
    (bind _output_get (Variables|SpeedParams|SetSpeed (- (Variables|SpeedParams|GetSpeed) (* (Utilities|Time|GetWorldDeltaSeconds) (Variables|SpeedParams|GetDeceleration)))))
    (if (< _output_get 0.0)
      (Variables|SpeedParams|SetSpeed 0.0))
    (else
      (Variables|SpeedParams|SetSpeed (+ (Variables|SpeedParams|GetSpeed) (* (Utilities|Time|GetWorldDeltaSeconds) (Variables|SpeedParams|GetAcceleration))))
      (if (< (Variables|SpeedParams|GetMaxSpeed) (Variables|SpeedParams|GetSpeed))
        (Variables|SpeedParams|SetSpeed (Variables|SpeedParams|GetMaxSpeed)))))
  (if (< (Variables|SpeedParams|GetSpeed) (Variables|Default|GetParticlesThreshold))
    (Components|Activation|Deactivate _niagara)
    (else
      (Components|Activation|Activate _niagara false))))

(event Custom|OnAudioFinished_Event
  ;[0.15 0.15 0.15 0.5] Custom Events
  (Variables|InteractionParams|SetIsPlayingSound false))

(event Custom|Stop%20Following
  ;[0.15 0.15 0.15 0.5] Custom Events
  ;;[0.15 0.15 0.15 0.5] Stop Following Player in axis X and Y
  (Variables|InteractionParams|SetlookAtTaki false)
  (bind _newtrack_0 (Timeline|LookNormalTimeline PlayFromStart)
    (:Update
      (if (Variables|InteractionParams|GetIsPlayerNearby)
        (Timeline|LookNormalTimeline Stop)
        (else
          (Transformation|SetWorldRotation (Variables|Default|GetCharacterOffset) (Math|Rotator|Lerp(Rotator) (Variables|Default|GetCurrentRotation) "0, 0, 0" _newtrack_0 true) false false))))))

(event Custom|Following
  (bind _returnvalue (Game|Player|GetPlayerPawn 0))
  (bind _characteroffset (Variables|Default|GetCharacterOffset))
  (bind _returnvalue_2 (Transformation|GetWorldLocation _characteroffset))
  (bind _returnvalue_3 (Transformation|GetActorLocation _returnvalue))
  ;[0.15 0.15 0.15 0.5] Custom Events
  ;;[0.15 0.15 0.15 0.5] Citizen follow Player in axis X and Y
  (bind _newtrack_0 (Timeline|LookAtTakiTimeline PlayFromStart)
    (:Update
      (if (Variables|InteractionParams|GetIsPlayerNearby)
        (Transformation|SetWorldRotation (Variables|Default|GetCharacterOffset) (Math|Rotator|Lerp(Rotator) (Variables|Default|GetCurrentRotation) (Math|Rotator|FindLookatRotation (Math|Vector|MakeVector (.x _returnvalue_3) (.y _returnvalue_3) 0.0) (Math|Vector|MakeVector (.x _returnvalue_2) (.y _returnvalue_2) 0.0)) _newtrack_0 true) false false)
        (else
          (Timeline|LookAtTakiTimeline Stop))))
    (:Finished
      (Variables|InteractionParams|SetlookAtTaki true))))

(event EventBeginPlay
  (bind _skeletalmesh (Variables|Default|GetSkeletalMesh))
  ;[0.15 0.15 0.15 0.5] Beginplay and Event Tick
  (bind _returnvalue (Rendering|Material|CreateDynamicMaterialInstance "/Game/Project/00_Generic/Assets/Materials/Outliner/M_Outliner.M_Outliner" "None" "None" :!class /Script/Engine.KismetMaterialLibrary))
  (bind _output_get (Variables|InteractionParams|SetOutlineMaterialInstance _returnvalue))
  (Rendering|Material|SetOverlayMaterial _skeletalmesh _output_get :!class /Script/Engine.MeshComponent)
  (Variables|Default|SetOriginal%20Scale (Transformation|GetWorldScale _skeletalmesh))
  (bind (_direction _zstretch) (Timeline|SquashStretchTimeline Play)
    (:Update
      (Transformation|SetRelativeScale3D (Variables|Default|GetSkeletalMesh) (Math|Vector|MakeVector (.x (Variables|Default|GetOriginal%20Scale)) (.y (Variables|Default|GetOriginal%20Scale)) (* _zstretch (.z (Variables|Default|GetOriginal%20Scale))))))
    (:Finished
      (if (Utilities|Enum|Equal(Enum) _direction "Backward")
        (Timeline|SquashStretchTimeline Play)
        (else
          (Timeline|SquashStretchTimeline ReverseFromEnd))))))

(event EventTick
  (params (DeltaSeconds :type Float%20%28single-precision%29))
  (bind _returnvalue (Game|Player|GetPlayerPawn 0))
  (bind _characteroffset (Variables|Default|GetCharacterOffset))
  (bind _returnvalue_2 (Transformation|GetActorLocation _returnvalue))
  (bind _returnvalue_3 (Transformation|GetWorldLocation _characteroffset))
  ;[0.15 0.15 0.15 0.5] Beginplay and Event Tick
  ;;[0.15 0.15 0.15 0.5] Update the Rotation and Spline position of SeaMapCreature
  (CallFunction|CalculateSpeed)
  (bind _output_get (Variables|SpeedParams|SetSplinePosition (+ (* DeltaSeconds (Variables|SpeedParams|GetSpeed)) (Variables|SpeedParams|GetSplinePosition))))
  (Transformation|SetRelativeLocationAndRotation (Variables|Default|GetCharacterOffset) (.location (Spline|GetTransformatDistanceAlongSpline (Variables|Default|GetMovementRoute) _output_get "Local" false)) (.rotation (Spline|GetTransformatDistanceAlongSpline (Variables|Default|GetMovementRoute) _output_get "Local" false)) false false)
  (if (>= (Variables|SpeedParams|GetSplinePosition) (Spline|GetSplineLength (Variables|Default|GetMovementRoute)))
    (Variables|SpeedParams|SetSplinePosition 0.0))
  (bind _newparam (CallFunction|KeepFollowingCondition))
  (if _newparam
    (Transformation|SetWorldRotation (Variables|Default|GetCharacterOffset) (Math|Rotator|FindLookatRotation (Math|Vector|MakeVector (.x _returnvalue_2) (.y _returnvalue_2) 0.0) (Math|Vector|MakeVector (.x _returnvalue_3) (.y _returnvalue_3) 0.0)) false false)))

(event EventOnHorrorLoaded
  ;[0.15 0.15 0.15 0.5] Interfaces
  ;;[0.15 0.15 0.15 0.5] Change Material On world Loaded
  (Rendering|Material|SetMaterial (Variables|Default|GetSkeletalMesh) 0 (Variables|Default|GetMaterial%20Horror)))

(event EventOnInteract
  (params (InteractedPlayer :type BP%20Playable%20Character%20Object%20Reference))
  ;[0.15 0.15 0.15 0.5] Interfaces
  (Default|AssignTransform (.AsYako%20Taki%20Game%20Mode (Utilities|Casting|CastToYakoTakiGameMode (Game|GetGameMode))) (Variables|TransformationParams|GetTransformClass)))

(event EventOnCuteLoaded
  ;[0.15 0.15 0.15 0.5] Interfaces
  ;;[0.15 0.15 0.15 0.5] Change Material On world Loaded
  (Rendering|Material|SetMaterial (Variables|Default|GetSkeletalMesh) 0 (Variables|Default|GetMaterial%20Cute)))

(fn ConstructionScript)

(fn KeepFollowingCondition
  ;[0.15 0.15 0.15 0.5] Check if player is X degrees down about Citizens
  (bind _player (Variables|Default|GetPlayer)
    (:then
      (return (and (Variables|InteractionParams|GetlookAtTaki) (>= (Math|Trig|RadiansToDegrees (Math|Trig|Acos(Degrees) (Math|Vector|DotProduct (Math|Vector|Normalize (- (Transformation|GetActorLocation _player) (Transformation|GetActorLocation))) "0.000000,0.000000,1.000000"))) (Variables|Default|GetDegrees%20To%20Keep%20Following)))))
    (:else)))