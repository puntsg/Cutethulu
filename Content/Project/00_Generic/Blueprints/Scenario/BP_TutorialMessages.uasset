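; BP_TutorialMessages is a trigger volume that starts and ends a tutorial message as the player enters and leaves its box.
; Entering initializes the ACTutorialMessage component, limited by a DoOnce, while a short delayed BeginPlay check also initializes it for players already inside.
; Leaving finishes the tutorial only if the game instance's save file does not already record that tutorial name as completed.
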(event OnComponentBeginOverlap(Box)
  (params (OverlappedComponent :type Primitive%20Component%20Object%20Reference) (OtherActor :type Actor%20Object%20Reference) (OtherComp :type Primitive%20Component%20Object%20Reference) (OtherBodyIndex :type Integer) (bFromSweep :type Boolean) (SweepResult :type Hit%20Result%20Structure%20%28by%20ref%29))
  ;[0.15 0.15 0.15 0.5] Colliders
  ;;[0.15 0.15 0.15 0.5] If Begin Overlap Start Tutorial
  (Utilities|Casting|CastToBP_PlayableCharacter OtherActor)
  (Utilities|FlowControl|DoOnce false
    (:Completed
      (Default|InitializeTutorial (Variables|Default|GetAC_TutorialMessage)))))

(event OnComponentEndOverlap(Box)
  (params (OverlappedComponent :type Primitive%20Component%20Object%20Reference) (OtherActor :type Actor%20Object%20Reference) (OtherComp :type Primitive%20Component%20Object%20Reference) (OtherBodyIndex :type Integer))
  (bind _ac_tutorialmessage (Variables|Default|GetAC_TutorialMessage))
  ;[0.15 0.15 0.15 0.5] Colliders
  ;;[0.15 0.15 0.15 0.5] If End Overlap End Tutorial
  (Utilities|Casting|CastToBP_PlayableCharacter OtherActor)
  (bind _returnvalue (Class|YakotakiSaveGame|GetifTutorialCompleted (Variables|/Game/Project/00_Generic/Blueprints/GameInstance/BP_YakotakiInstance.BP_YakotakiInstance_C|GetGame%20Save%20File (.AsBP%20Yakotaki%20Instance (Utilities|Casting|CastToBP_YakotakiInstance (Game|GetGameInstance)))) (Utilities|String|ToString(Name) (Variables|/Game/Project/00_Generic/Blueprints/Components/AC_TutorialMessage.AC_TutorialMessage_C|GetTutorialName _ac_tutorialmessage))))
  (if (not _returnvalue)
    (Default|FinishTutorial _ac_tutorialmessage)))

(event EventBeginPlay
  (Utilities|FlowControl|Delay 0.2)
  (if (Collision|IsOverlappingActor (Variables|Default|GetBox) (Game|GetPlayerCharacter 0) :!class /Script/Engine.PrimitiveComponent)
    (Default|InitializeTutorial (Variables|Default|GetAC_TutorialMessage))))

(fn ConstructionScript)