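; BP_Spikes is a spike obstacle that knocks a playable character away when it hits the Cone component.
; On hit, it calls Damage on the character's AdvancedHealthBehaviour with an amount of zero, then launches the character after a short delay.
; Launch velocity is the scaled direction from the actor's origin to the hit point, with each axis capped only from above by LaunchSpeedLimiter.
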(event OnComponentHit(Cone)
  (params (HitComponent :type Primitive%20Component%20Object%20Reference) (OtherActor :type Actor%20Object%20Reference) (OtherComp :type Primitive%20Component%20Object%20Reference) (NormalImpulse :type Vector :default "0, 0, 0") (Hit :type Hit%20Result%20Structure%20%28by%20ref%29))
  (bind _returnvalue (Transformation|GetActorLocation))
  (bind _launchmultiplier (Variables|Default|GetLaunchMultiplier))
  (bind _launchspeedlimiter (Variables|Default|GetLaunchSpeedLimiter))
  (bind _returnvalue_2 (- (.location Hit) _returnvalue))
  (bind _returnvalue_3 (Math|Vector|Normalize _returnvalue_2))
  (bind _returnvalue_4 (* _returnvalue_3 _launchmultiplier))
  (bind _asbp_playable_character (Utilities|Casting|CastToBP_PlayableCharacter OtherActor))
  (Class|AdvancedHealthBehaviour|Damage (Variables|/Game/Project/00_Generic/Blueprints/PlayableCharacters/BP_PlayableCharacter.BP_PlayableCharacter_C|GetAdvancedHealthBehaviour _asbp_playable_character) 0.0)
  (Utilities|FlowControl|Delay 0.25)
  (Character|LaunchCharacter _asbp_playable_character (Math|Vector|MakeVector (Math|Float|Min(Float) (.x _returnvalue_4) (.x _launchspeedlimiter)) (Math|Float|Min(Float) (.y _returnvalue_4) (.y _launchspeedlimiter)) (Math|Float|Min(Float) (.z _returnvalue_4) (.z _launchspeedlimiter))) false false))

(fn ConstructionScript)