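; Moving platform that travels along a spline route while its mesh loops back and forth on the UpDown timeline.
; Tick advances spline distance by speed and applies location and yaw to the offset component, layering route motion with the mesh animation.
; Follow Spline restarts from zero speed at the route's end; Ping Pong flags reverse travel.
; CalculateSpeed ramps speed toward a maximum, with a separate branch for braking.
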(event Custom|Accelerate
  (if (Variables|PlatformParams|GetReverse)
    (Variables|PlatformSpeedParams|SetSpeed 0.0)
    (else
      (Variables|PlatformSpeedParams|SetSpeed (Math|Float|Min(Float) (+ (Variables|PlatformSpeedParams|GetSpeed) (* (Utilities|Time|GetWorldDeltaSeconds) (Variables|PlatformSpeedParams|GetAcceleration))) (Variables|PlatformSpeedParams|GetMaxSpeed))))))

(event Custom|CalculateSpeed
  (if (Variables|PlatformParams|GetBreaking)
    (Variables|PlatformSpeedParams|SetSpeed (Math|Float|Min(Float) (- (Variables|PlatformSpeedParams|GetSpeed) (* (Utilities|Time|GetWorldDeltaSeconds) (Variables|PlatformSpeedParams|GetDeceleration))) 0.0))
    (else
      (Variables|PlatformSpeedParams|SetSpeed (Math|Float|Min(Float) (+ (Variables|PlatformSpeedParams|GetSpeed) (* (Utilities|Time|GetWorldDeltaSeconds) (Variables|PlatformSpeedParams|GetAcceleration))) (Variables|PlatformSpeedParams|GetMaxSpeed))))))

(event EventBeginPlay
  (bind (_direction _newtrack_1) (Timeline|UpDown PlayFromStart)
    (:Update
      (Transformation|SetRelativeLocation (Variables|Default|GetStaticMesh) _newtrack_1 false false))
    (:Finished
      (if (Utilities|Enum|Equal(Enum) _direction "Backward")
        (Timeline|UpDown Play)
        (else
          (Timeline|UpDown Reverse))))))

(event EventTick
  (params (DeltaSeconds :type Float%20%28single-precision%29))
  (bind _route (Variables|Default|GetRoute))
  (switch Utilities|FlowControl|Switch|SwitchonE_PlatformMovementEnum (Variables|PlatformParams|GetMovementType)
    (:NewEnumerator1
      (Variables|PlatformSpeedParams|SetSplinePosition (+ (* DeltaSeconds (Variables|PlatformSpeedParams|GetSpeed)) (Variables|PlatformSpeedParams|GetSplinePosition)) :!label _label))
    (:NewEnumerator3
      (if (not (Variables|PlatformParams|GetReverse))
        (goto _label)
        (else
          (bind _output_get (Variables|PlatformSpeedParams|SetSplinePosition (+ (* (* DeltaSeconds (Variables|PlatformSpeedParams|GetSpeed)) -1.0) (Variables|PlatformSpeedParams|GetSplinePosition))))
          (if (< _output_get 0.0)
            _
            (else
              (Variables|PlatformParams|SetReverse false)))))))
  (CallFunction|CalculateSpeed)
  (Transformation|SetRelativeLocationAndRotation (Variables|Default|GetPlatfomOffset) (.location (Spline|GetTransformatDistanceAlongSpline _route (Variables|PlatformSpeedParams|GetSplinePosition) "Local" false)) (Math|Rotator|MakeRotator 0.0 0.0 (.yaw (.rotation (Spline|GetTransformatDistanceAlongSpline _route (Variables|PlatformSpeedParams|GetSplinePosition) "Local" false)))) false false)
  (if (>= (Variables|PlatformSpeedParams|GetSplinePosition) (Spline|GetSplineLength _route))
    (if (Utilities|Enum|Equal(Enum) (Variables|PlatformParams|GetMovementType) "NewEnumerator3")
      (Variables|PlatformParams|SetReverse true)
      (Variables|PlatformSpeedParams|SetSplinePosition (Spline|GetSplineLength (Variables|Default|GetRoute)))
      (else
        (Variables|PlatformSpeedParams|SetSplinePosition 0.0)
        (Variables|PlatformSpeedParams|SetSpeed 0.0)))))

(fn ConstructionScript)