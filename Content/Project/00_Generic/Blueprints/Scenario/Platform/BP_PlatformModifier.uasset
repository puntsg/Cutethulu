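; BP_PlatformModifier is a trigger volume that changes the motion settings of moving platforms passing into it.
; When its Box begins overlapping a BP_Platform, it overwrites that platform's Speed, MaxSpeed and Acceleration.
; The platform's Reverse flag selects the value set: true applies the plain New values, while false applies the NewReverse values.
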(event OnComponentBeginOverlap(Box)
  (params (OverlappedComponent :type Primitive%20Component%20Object%20Reference) (OtherActor :type Actor%20Object%20Reference) (OtherComp :type Primitive%20Component%20Object%20Reference) (OtherBodyIndex :type Integer) (bFromSweep :type Boolean) (SweepResult :type Hit%20Result%20Structure%20%28by%20ref%29))
  (bind _asbp_platform (Utilities|Casting|CastToBP_Platform OtherActor))
  (if (Variables|/Game/Project/00_Generic/Blueprints/Scenario/Platform/BP_Platform.BP_Platform_C|GetReverse _asbp_platform)
    (Variables|/Game/Project/00_Generic/Blueprints/Scenario/Platform/BP_Platform.BP_Platform_C|SetSpeed _asbp_platform (Variables|Default|GetNewSpeed))
    (Variables|/Game/Project/00_Generic/Blueprints/Scenario/Platform/BP_Platform.BP_Platform_C|SetMaxSpeed _asbp_platform (Variables|Default|GetNewMaxSpeed))
    (Variables|/Game/Project/00_Generic/Blueprints/Scenario/Platform/BP_Platform.BP_Platform_C|SetAcceleration _asbp_platform (Variables|Default|GetNewAcceleration))
    (else
      (Variables|/Game/Project/00_Generic/Blueprints/Scenario/Platform/BP_Platform.BP_Platform_C|SetSpeed _asbp_platform (Variables|Default|GetNewReverseSpeed))
      (Variables|/Game/Project/00_Generic/Blueprints/Scenario/Platform/BP_Platform.BP_Platform_C|SetMaxSpeed _asbp_platform (Variables|Default|GetNewReverseMaxSpeed))
      (Variables|/Game/Project/00_Generic/Blueprints/Scenario/Platform/BP_Platform.BP_Platform_C|SetAcceleration _asbp_platform (Variables|Default|GetNewReverseAcceleration)))))

(event EventBeginPlay)

(event Collision|EventActorBeginOverlap
  (params (OtherActor :type Actor%20Object%20Reference)))

(event EventTick
  (params (DeltaSeconds :type Float%20%28single-precision%29)))

(fn ConstructionScript)