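; Test citizen NPC that walks toward a detected player and offers two interactions that assign transform character classes through TestGameMode.
; It binds its detection and proximity events on BeginPlay, moving to the player's location at detection, then returning to its start point and spawn rotation once the player exits.
; Proximity sets or clears the player's CurrentInteractive.
; Primary and secondary interactions each assign their own class, with secondary using slot 1.
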(event Custom|OnPlayerEnterDetection_Event
  (params (Character :type BP%20Playable%20Character%20Object%20Reference))
  (CallFunction|GotoPosition (Transformation|GetActorLocation Character)))

(event Custom|OnPlayerExitsDetection_Event
  (params (Character :type BP%20Playable%20Character%20Object%20Reference))
  (CallFunction|ReturntoStartPoint))

(event Custom|OnReturnedToOriginalPos_Event
  (Transformation|SetActorRotation (Variables|Default|GetSpawnRotation)))

(event Custom|OnPlayerNear_Event
  (params (Character :type BP%20Playable%20Character%20Object%20Reference))
  (Variables|/Game/Project/00_Generic/Bluprints/PlayableCharacters/BP_PlayableCharacter.BP_PlayableCharacter_C|SetCurrentInteractive Character self))

(event Custom|OnPlayerFlees_Event
  (params (Character :type BP%20Playable%20Character%20Object%20Reference))
  (Variables|/Game/Project/00_Generic/Bluprints/PlayableCharacters/BP_PlayableCharacter.BP_PlayableCharacter_C|SetCurrentInteractive Character 0))

(event EventBeginPlay
  (|CallParentFunction)
  (EventDispatchers|BindEventtoOnPlayerEnterDetection (delegate Custom|OnPlayerEnterDetection_Event))
  (EventDispatchers|AssignOnPlayerExitsDetection (delegate Custom|OnPlayerExitsDetection_Event))
  (EventDispatchers|AssignOnReturnedtoOriginalPos (delegate Custom|OnReturnedToOriginalPos_Event))
  (EventDispatchers|AssignOnPlayerNear (delegate Custom|OnPlayerNear_Event))
  (EventDispatchers|AssignOnPlayerFlees (delegate Custom|OnPlayerFlees_Event)))

(event EventOnSecondaryInteract
  (params (InteractedPlayer :type BP%20Playable%20Character%20Object%20Reference))
  (Default|AssignTransform (.AsTest%20Game%20Mode (Utilities|Casting|CastToTestGameMode (Game|GetGameMode))) (Variables|Default|GetAssigned%20class%20to%20transform_0) 1))

(event EventOnInteract
  (params (InteractedPlayer :type BP%20Playable%20Character%20Object%20Reference))
  (Default|AssignTransform (.AsTest%20Game%20Mode (Utilities|Casting|CastToTestGameMode (Game|GetGameMode))) (Variables|Default|GetAssigned%20class%20to%20transform)))

(fn ConstructionScript
  (|CallParentFunction))