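; Actor component that buffers a single player input action so it can be replayed later.
; StoreNextInput saves the given action while CanBeQueued is true, overwriting or clearing the slot, and returns that flag.
; ExecuteNextAction replays the stored action by injecting it into player 0's Enhanced Input subsystem, then empties the slot.
; Nothing in this graph sets CanBeQueued or triggers the replay.
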(event Custom|ExecuteNextAction
  (Class|EnhancedInputSubsystemInterface|InjectInputVectorforAction (PlayerController|LocalPlayerSubsystems|GetEnhancedInputLocalPlayerSubsystem (Game|GetPlayerController 0)) (Variables|Default|GetInputToStore) "0, 0, 0")
  (Variables|Default|SetInputToStore 0))

(event EventBeginPlay)

(event EventTick
  (params (DeltaSeconds :type Float%20%28single-precision%29)))

(fn StoreNextInput
  (params (InputToStore :type Input%20Action%20Object%20Reference))
  (if (Variables|Default|GetCan%20be%20Queued)
    (Utilities|IsValid InputToStore
      (:Is%20Valid
        (Variables|Default|SetInputToStore InputToStore)
        (return (Variables|Default|GetCan%20be%20Queued)))
      (:Is%20Not%20Valid
        (Variables|Default|SetInputToStore 0)
        (return (Variables|Default|GetCan%20be%20Queued))))
    (else
      (return (Variables|Default|GetCan%20be%20Queued)))))