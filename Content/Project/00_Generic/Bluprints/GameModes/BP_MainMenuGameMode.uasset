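; Main menu game mode that creates the main menu and options menu widgets and switches between them.
; On BeginPlay it adds both widgets to the viewport, with options hidden, and binds the Options and Return buttons to switch events.
; Each switch toggles visibility and enabled state on both widgets, and opening options also calls SetOptionsMenuVisibility on that widget.
; A FadeIn function is present but empty.
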(event Custom|OptionsToMenu
  (bind _optionsmenu (Variables|Default|GetOptionsMenu))
  (bind _menu (Variables|Default|Getmenu))
  (Widget|SetIsEnabled _optionsmenu false)
  (Widget|SetVisibility _optionsmenu "Hidden")
  (Widget|SetIsEnabled _menu true)
  (Widget|SetVisibility _menu "Visible"))

(event Custom|MenuToOptions
  (bind _optionsmenu (Variables|Default|GetOptionsMenu))
  (bind _menu (Variables|Default|Getmenu))
  (Widget|SetIsEnabled _optionsmenu true)
  (Widget|SetVisibility _optionsmenu "Visible")
  (Default|SetOptionsMenuVisibility _optionsmenu false false false false)
  (Widget|SetIsEnabled _menu false)
  (Widget|SetVisibility _menu "Hidden"))

(event EventBeginPlay
  (bind _returnvalue (UserInterface|CreateWidget "/Game/Project/00_Generic/Bluprints/UI_HUD/WBP_MainMenu.WBP_MainMenu_C"))
  (bind _output_get (Variables|Default|Setmenu _returnvalue))
  (UserInterface|Viewport|AddtoViewport _output_get 0)
  (bind _returnvalue_2 (UserInterface|CreateWidget "/Game/Project/00_Generic/Bluprints/UI_HUD/WBP_OptionsMenu.WBP_OptionsMenu_C"))
  (bind _output_get_2 (Variables|Default|SetOptionsMenu _returnvalue_2))
  (Widget|SetVisibility _output_get_2 "Hidden")
  (UserInterface|Viewport|AddtoViewport _output_get_2 0)
  (EventDispatchers|AssignOnClicked (Variables|/Game/Project/00_Generic/Bluprints/UI_HUD/WBP_OptionsMenu.WBP_OptionsMenu_C|GetReturnButton _output_get_2) (delegate Custom|OptionsToMenu))
  (EventDispatchers|AssignOnClicked (Variables|/Game/Project/00_Generic/Bluprints/UI_HUD/WBP_MainMenu.WBP_MainMenu_C|GetOPTIONS_button (Variables|Default|Getmenu)) (delegate Custom|MenuToOptions)))

(fn ConstructionScript)

(fn Fadein)