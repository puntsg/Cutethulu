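; BP_ChekPoints is a checkpoint actor that records where the player last reached.
; When a BP_PlayableCharacter overlaps its Box, it writes its own location to LastCheckPointLocation on BP_CutethuluInstance, the game instance.
; Shortly after BeginPlay it also checks whether the player already overlaps the Box and saves then, covering characters that start inside it.
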(event OnComponentBeginOverlap(Box)
  (params (OverlappedComponent :type Primitive%20Component%20Object%20Reference) (OtherActor :type Actor%20Object%20Reference) (OtherComp :type Primitive%20Component%20Object%20Reference) (OtherBodyIndex :type Integer) (bFromSweep :type Boolean) (SweepResult :type Hit%20Result%20Structure%20%28by%20ref%29))
  (Utilities|Casting|CastToBP_PlayableCharacter OtherActor)
  (CallFunction|SetChekPoints))

(event EventBeginPlay
  (Utilities|FlowControl|Delay 0.1)
  (if (Collision|IsOverlappingActor (Variables|Default|GetBox) (Game|GetPlayerCharacter 0) :!class /Script/Engine.PrimitiveComponent)
    (CallFunction|SetChekPoints)))

(event Collision|EventActorBeginOverlap
  (params (OtherActor :type Actor%20Object%20Reference)))

(event EventTick
  (params (DeltaSeconds :type Float%20%28single-precision%29)))

(fn ConstructionScript)

(fn SetChekPoints
  (bind _asbp_cutethulu_instance (Utilities|Casting|CastToBP_CutethuluInstance (Game|GetGameInstance)))
  (Variables|/Game/Project/00_Generic/Bluprints/Others/BP_CutethuluInstance.BP_CutethuluInstance_C|SetLastCheckPointLocation _asbp_cutethulu_instance (Transformation|GetActorLocation)))