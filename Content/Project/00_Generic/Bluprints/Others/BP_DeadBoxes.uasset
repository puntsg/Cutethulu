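; BP_DeadBoxes is a kill volume that sends the player back to the last checkpoint.
; On overlap, it disables and insta-kills the playable character, then possesses the first BP_PlayerDefault_Taki with input disabled.
; After a delayed fade, it teleports Taki to the checkpoint location stored in BP_CutethuluInstance.
; It then restores movement, camera and health, and resets transformations through TestGameMode.
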(event OnComponentBeginOverlap(Box)
  (params (OverlappedComponent :type Primitive%20Component%20Object%20Reference) (OtherActor :type Actor%20Object%20Reference) (OtherComp :type Primitive%20Component%20Object%20Reference) (OtherBodyIndex :type Integer) (bFromSweep :type Boolean) (SweepResult :type Hit%20Result%20Structure%20%28by%20ref%29))
  (bind _returnvalue (Game|GetPlayerController 0))
  (bind _asbp_playable_character (Utilities|Casting|CastToBP_PlayableCharacter OtherActor))
  (Default|SetCanMoveandJump _asbp_playable_character false)
  (Default|SetActive _asbp_playable_character false)
  (Class|AdvancedHealthBehaviour|InstaKill (Variables|/Game/Project/00_Generic/Bluprints/PlayableCharacters/BP_PlayableCharacter.BP_PlayableCharacter_C|GetAdvancedHealthBehaviour _asbp_playable_character))
  (Class|AdvancedHealthBehaviour|MaxHeal (Variables|/Game/Project/00_Generic/Bluprints/PlayableCharacters/BP_PlayableCharacter.BP_PlayableCharacter_C|GetAdvancedHealthBehaviour _asbp_playable_character))
  (Pawn|UnPossess _returnvalue)
  (bind _outactors (Actor|GetAllActorsOfClass "/Game/Project/00_Generic/Bluprints/PlayableCharacters/BP_PlayerDefault_Taki.BP_PlayerDefault_Taki_C"))
  (Pawn|Possess _returnvalue (Utilities|Array|Get(acopy) _outactors))
  (Input|DisableInput (Utilities|Array|Get(acopy) _outactors) _returnvalue)
  (bind _asbp_cutethulu_instance (Utilities|Casting|CastToBP_CutethuluInstance (Game|GetGameInstance)))
  (Default|Fadein _asbp_cutethulu_instance)
  (Utilities|FlowControl|Delay 1.0)
  (Transformation|Teleport (Utilities|Array|Get(acopy) _outactors) (Variables|/Game/Project/00_Generic/Bluprints/Others/BP_CutethuluInstance.BP_CutethuluInstance_C|GetLastCheckPointLocation _asbp_cutethulu_instance) "0, 0, 0")
  (Default|FadeOut _asbp_cutethulu_instance)
  (Components|Movement|StopMovementImmediately (Variables|/Script/Engine.Character|GetCharacterMovement (Game|GetPlayerCharacter 0)))
  (Input|EnableInput (Utilities|Array|Get(acopy) _outactors) _returnvalue)
  (Default|SetActive (Utilities|Array|Get(acopy) _outactors) true)
  (Default|SetCanMoveandJump (Utilities|Array|Get(acopy) _outactors) true)
  (Variables|/Game/Project/00_Generic/Bluprints/PlayableCharacters/BP_PlayableCharacter.BP_PlayableCharacter_C|SetCanRotateCamera (Utilities|Array|Get(acopy) _outactors) true)
  (Class|AdvancedHealthBehaviour|MaxHeal (Variables|/Game/Project/00_Generic/Bluprints/PlayableCharacters/BP_PlayableCharacter.BP_PlayableCharacter_C|GetAdvancedHealthBehaviour (Utilities|Array|Get(acopy) _outactors)))
  (Default|ResetTransformations (.AsTest%20Game%20Mode (Utilities|Casting|CastToTestGameMode (Game|GetGameMode)))))

(fn ConstructionScript)