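; Temporary platform for BP_PlayerDJ that grows in on spawn and removes itself after LifeTime.
; A timeline scales it from near zero toward its original size, enabling collision and starting the lifetime delay from its update.
; When the player stops overlapping the cylinder collision while not falling, it refills their platforms.
; End-overlap events are unbound before destruction, so despawning triggers no refill.
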(event OnComponentEndOverlap(CylinderCollision)
  (params (OverlappedComponent :type Primitive%20Component%20Object%20Reference) (OtherActor :type Actor%20Object%20Reference) (OtherComp :type Primitive%20Component%20Object%20Reference) (OtherBodyIndex :type Integer))
  (bind _asbp_player_dj (Utilities|Casting|CastToBP_PlayerDJ OtherActor))
  (if (Utilities|Enum|NotEqual(Enum) (Variables|/Script/Engine.CharacterMovementComponent|GetMovementMode (Variables|/Script/Engine.Character|GetCharacterMovement _asbp_player_dj)) "MOVE_Falling")
    (Default|RefillPlatforms _asbp_player_dj)))

(event EventBeginPlay
  (Variables|Default|SetBaseScale (Transformation|GetActorScale3D))
  (Transformation|SetActorScale3D "0.050000,0.050000,0.050000")
  (bind _scalevalue (Timeline|ScaleTimeline Play)
    (:Update
      (Transformation|SetActorScale3D (* _scalevalue (Variables|Default|GetBaseScale)))
      (Collision|SetActorEnableCollision true)
      (Utilities|FlowControl|Delay (Variables|Default|GetLifeTime))
      (EventDispatchers|UnbindallEventsfromOnComponentEndOverlap (Variables|Default|GetCylinderCollision))
      (Actor|DestroyActor))))

(event Collision|EventActorBeginOverlap
  (params (OtherActor :type Actor%20Object%20Reference)))

(event EventTick
  (params (DeltaSeconds :type Float%20%28single-precision%29)))

(fn ConstructionScript)