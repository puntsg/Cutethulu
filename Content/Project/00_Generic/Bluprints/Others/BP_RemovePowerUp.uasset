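; BP_RemovePowerUp is a trigger actor that strips the player's transformation power-up.
; When an actor overlaps its Box, a playable character that is not BP_PlayerDefault_Taki transforms back into the TestGameMode's OriginalCharacter.
; The overlap then has the game mode reset its transformations.
; An unconnected leftover chain for swapping to another creature and updating the transformation UI never runs.
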(event OnComponentBeginOverlap(Box)
  (params (OverlappedComponent :type Primitive%20Component%20Object%20Reference) (OtherActor :type Actor%20Object%20Reference) (OtherComp :type Primitive%20Component%20Object%20Reference) (OtherBodyIndex :type Integer) (bFromSweep :type Boolean) (SweepResult :type Hit%20Result%20Structure%20%28by%20ref%29))
  (bind _returnvalue (Game|GetGameMode))
  (bind _asbp_playable_character (Utilities|Casting|CastToBP_PlayableCharacter OtherActor))
  (bind _astest_game_mode (Utilities|Casting|CastToTestGameMode _returnvalue))
  (if (!= (Utilities|GetClass _asbp_playable_character) "/Game/Project/00_Generic/Bluprints/PlayableCharacters/BP_PlayerDefault_Taki.BP_PlayerDefault_Taki_C")
    (Default|Transform _asbp_playable_character (Variables|/Game/Project/00_Generic/Bluprints/GameModes/TestGameMode.TestGameMode_C|GetOriginalCharacter _astest_game_mode)))
  (Default|ResetTransformations _astest_game_mode))

(event EventBeginPlay)

(event Collision|EventActorBeginOverlap
  (params (OtherActor :type Actor%20Object%20Reference)))

(event EventTick
  (params (DeltaSeconds :type Float%20%28single-precision%29)))

(fn ConstructionScript)