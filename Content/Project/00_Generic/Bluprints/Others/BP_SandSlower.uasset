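; BP_SandSlower is a sand area that slows a playable character and visually sinks it while inside.
; When the character's capsule enters the box, it stores the mesh location, caps faster walk speeds at MoveInSand and plays the SandDrown timeline to lower only the mesh.
; Leaving restores the saved speed and reverses the timeline to raise the mesh.
; It tracks one character at a time, resetting the previous mesh on re-entry.
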(event OnComponentBeginOverlap(Box)
  (params (OverlappedComponent :type Primitive%20Component%20Object%20Reference) (OtherActor :type Actor%20Object%20Reference) (OtherComp :type Primitive%20Component%20Object%20Reference) (OtherBodyIndex :type Integer) (bFromSweep :type Boolean) (SweepResult :type Hit%20Result%20Structure%20%28by%20ref%29))
  (bind _asbp_playable_character (Utilities|Casting|CastToBP_PlayableCharacter OtherActor))
  (Utilities|Casting|CastToCapsuleComponent OtherComp)
  (Development|PrintString "Enter in sand")
  (Utilities|IsValid (Variables|Default|GetReferencedCharacter)
    (:Is%20Valid
      (Transformation|SetRelativeLocation (Variables|/Script/Engine.Character|GetMesh (Variables|Default|GetReferencedCharacter)) (Variables|Default|GetMesh%20Original%20Relative%20Location) false false)
      (Utilities|FlowControl|Sequence
        (:then_0)
        (:then_1
          _)))
    (:Is%20Not%20Valid
      _))
  (bind _output_get (Variables|Default|SetReferencedCharacter _asbp_playable_character))
  (Variables|Default|SetMesh%20Original%20Relative%20Location (Variables|/Script/Engine.SceneComponent|GetRelativeLocation (Variables|/Script/Engine.Character|GetMesh _output_get)))
  (Math|Float|CompareFloat (Variables|/Script/Engine.CharacterMovementComponent|GetMaxWalkSpeed (Variables|/Script/Engine.Character|GetCharacterMovement (Variables|Default|GetReferencedCharacter))) (Variables|Default|GetMove%20in%20sand)
    (:>
      (Variables|Default|SetOriginal%20Walk%20Speed (Variables|/Script/Engine.CharacterMovementComponent|GetMaxWalkSpeed (Variables|/Script/Engine.Character|GetCharacterMovement (Variables|Default|GetReferencedCharacter))))
      (Variables|/Script/Engine.CharacterMovementComponent|SetMaxWalkSpeed (Variables|/Script/Engine.Character|GetCharacterMovement (Variables|Default|GetReferencedCharacter)) (Variables|Default|GetMove%20in%20sand))
      (Development|PrintString "Playing drowning")
      (bind _drowningperc (Timeline|SandDrown Play)
        (:Update
          (Transformation|SetRelativeLocation (Variables|/Script/Engine.Character|GetMesh (Variables|Default|GetReferencedCharacter)) (Math|Vector|MakeVector (.x (Variables|Default|GetMesh%20Original%20Relative%20Location)) (.y (Variables|Default|GetMesh%20Original%20Relative%20Location)) (- (.z (Variables|Default|GetMesh%20Original%20Relative%20Location)) (* _drowningperc (Variables|Default|GetMaxDrowningDepth)))) false false))))))

(event OnComponentEndOverlap(Box)
  (params (OverlappedComponent :type Primitive%20Component%20Object%20Reference) (OtherActor :type Actor%20Object%20Reference) (OtherComp :type Primitive%20Component%20Object%20Reference) (OtherBodyIndex :type Integer))
  (bind _mesh_original_relative_location (Variables|Default|GetMesh%20Original%20Relative%20Location))
  (bind _asbp_playable_character (Utilities|Casting|CastToBP_PlayableCharacter OtherActor))
  (Utilities|Casting|CastToCapsuleComponent OtherComp)
  (Variables|/Script/Engine.CharacterMovementComponent|SetMaxWalkSpeed (Variables|/Script/Engine.Character|GetCharacterMovement _asbp_playable_character) (Variables|Default|GetOriginal%20Walk%20Speed))
  (Development|PrintString "Not drowning")
  (bind _drowningperc (Timeline|SandDrown Reverse)
    (:Update
      (Transformation|SetRelativeLocation (Variables|/Script/Engine.Character|GetMesh (Variables|Default|GetReferencedCharacter)) (Math|Vector|MakeVector (.x _mesh_original_relative_location) (.y _mesh_original_relative_location) (- (.z _mesh_original_relative_location) (* _drowningperc (Variables|Default|GetMaxDrowningDepth)))) false false))))

(fn ConstructionScript)