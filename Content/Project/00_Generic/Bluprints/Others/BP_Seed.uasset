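; BP_Seed is an interactable seed that heals the world through TestGameMode when the player uses it.
; Overlapping its collider registers it as the Taki player's CurrentInteractive and fades in a prompt widget via a timeline.
; Leaving clears that reference and fades the prompt out before hiding it; interacting also fades it out.
; Horror and Cute world-loaded events each set the seed mesh's material.
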(event OnComponentBeginOverlap(seed_collider)
  (params (OverlappedComponent :type Primitive%20Component%20Object%20Reference) (OtherActor :type Actor%20Object%20Reference) (OtherComp :type Primitive%20Component%20Object%20Reference) (OtherBodyIndex :type Integer) (bFromSweep :type Boolean) (SweepResult :type Hit%20Result%20Structure%20%28by%20ref%29))
  (bind _asbp_player_default_taki (Utilities|Casting|CastToBP_PlayerDefault_Taki OtherActor))
  (Variables|Default|SetIsCollision true)
  (Variables|/Game/Project/00_Generic/Bluprints/PlayableCharacters/BP_PlayableCharacter.BP_PlayableCharacter_C|SetCurrentInteractive _asbp_player_default_taki self)
  (Development|SetHiddeninGame (Variables|Default|GetWidget) false false)
  (bind _asinteractive (Utilities|Casting|CastToInteractive (UserInterface|GetWidget (Variables|Default|GetWidget))))
  (bind _alfa (Timeline|Timeline PlayFromStart)
    (:Update
      (Default|Alfa _asinteractive _alfa))))

(event OnComponentEndOverlap(seed_collider)
  (params (OverlappedComponent :type Primitive%20Component%20Object%20Reference) (OtherActor :type Actor%20Object%20Reference) (OtherComp :type Primitive%20Component%20Object%20Reference) (OtherBodyIndex :type Integer))
  (bind _asbp_player_default_taki (Utilities|Casting|CastToBP_PlayerDefault_Taki OtherActor))
  (Variables|Default|SetIsCollision false)
  (Variables|/Game/Project/00_Generic/Bluprints/PlayableCharacters/BP_PlayableCharacter.BP_PlayableCharacter_C|SetCurrentInteractive _asbp_player_default_taki 0)
  (bind _asinteractive (Utilities|Casting|CastToInteractive (UserInterface|GetWidget (Variables|Default|GetWidget))))
  (bind _alfa (Timeline|Timeline_0 Reverse)
    (:Update
      (Default|Alfa _asinteractive _alfa))
    (:Finished
      (Development|SetHiddeninGame (Variables|Default|GetWidget) true false))))

(event EventOnInteract
  (params (InteractedPlayer :type BP%20Playable%20Character%20Object%20Reference))
  (if (Variables|Default|GetIsCollision)
    (bind _astest_game_mode (Utilities|Casting|CastToTestGameMode (Game|GetGameMode)))
    (Default|HealWorld _astest_game_mode)
    (bind _asinteractive (Utilities|Casting|CastToInteractive (UserInterface|GetWidget (Variables|Default|GetWidget))))
    (bind _alfa (Timeline|Timeline_0 Reverse)
      (:Update
        (Default|Alfa _asinteractive _alfa))
      (:Finished
        (Development|SetHiddeninGame (Variables|Default|GetWidget) true false)))))

(event EventOnHorrorLoaded
  (Rendering|Material|SetMaterial (Variables|Default|GetSeed) 0 0))

(event EventOnCuteLoaded
  (Rendering|Material|SetMaterial (Variables|Default|GetSeed) 0 "/Engine/EditorLandscapeResources/SelectBrushMaterial_Selected.SelectBrushMaterial_Selected"))

(fn ConstructionScript)