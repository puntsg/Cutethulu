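; Player character Blueprint whose extra jump press, once jumps run out in midair, spawns a SpatterPlatform.
; The spawn spends a platform charge, can halve horizontal velocity, and uses a timeline lerp to slide the platform forward, scaled by X velocity.
; A jump timeline drives gravity scale; landing triggers squash-stretch, and non-platform surfaces refill charges and reset gravity.
; An interp-based movement branch is disabled, and Tick prints the platform target for debugging.
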(event Custom|RefillPlatforms
  ;[0.15 0.15 0.15 0.5] Refill Platforms
  (Variables|Default|SetPlatforms 1)
  (Variables|Default|SetJumpMaxCount 2)
  (Variables|Default|SetJumpCount 1))

(event Custom|Calculate%20Platform%20Movement%20Position
  (params (Platform :type Spatter%20Platform%20Object%20Reference))
  (bind _returnvalue (Transformation|GetActorForwardVector))
  (bind _returnvalue_2 (Transformation|GetActorLocation))
  (bind _vertical_offset (Variables|Default|GetVertical%20Offset))
  (bind _platform_distancev1 (Variables|Default|GetPlatform%20DistanceV1))
  (bind _returnvalue_3 (* _returnvalue _platform_distancev1))
  (bind _returnvalue_4 (+ _returnvalue_3 _returnvalue_2))
  (bind _returnvalue_5 (+ _returnvalue_4 (Math|Vector|MakeVector 0.0 0.0 _vertical_offset)))
  ;[0.15 0.15 0.15 0.5] Calculate the next position to platform after spawn and move it
  (if false
    (Variables|Default|SetPlatform%20Movement%20Final%20Position _returnvalue_5)
    (Collision|LineTraceByChannel (Transformation|GetActorLocation) _returnvalue_5 "TraceTypeQuery1" false 0 "None")
    (Transformation|SetActorLocation Platform (Math|Vector|MakeVector (.x (Math|Interpolation|VInterpTo (Transformation|GetActorLocation Platform) (Variables|Default|GetPlatform%20Movement%20Final%20Position) (stale EventTick DeltaSeconds) (Variables|Default|GetPlatformTimeMovement))) (.y (Math|Interpolation|VInterpTo (Transformation|GetActorLocation Platform) (Variables|Default|GetPlatform%20Movement%20Final%20Position) (stale EventTick DeltaSeconds) (Variables|Default|GetPlatformTimeMovement))) (.z (Transformation|GetActorLocation Platform))) true false)
    (else
      (Variables|Default|SetPlatform%20Movement%20Final%20Position (+ (* (Transformation|GetActorForwardVector) (* (Math|Vector|VectorLength (Math|Vector|MakeVector (.x (Transformation|GetVelocity)) 0.0 0.0)) (Variables|Default|GetPlatform%20DistanceV2))) (Transformation|GetActorLocation)))
      (bind _movement (Timeline|Timeline_2 PlayFromStart)
        (:Update
          (Transformation|SetActorLocation Platform (Math|Vector|MakeVector (.x (Math|Vector|Lerp(Vector) (Transformation|GetActorLocation Platform) (Variables|Default|GetPlatform%20Movement%20Final%20Position) _movement)) (.y (Math|Vector|Lerp(Vector) (Transformation|GetActorLocation Platform) (Variables|Default|GetPlatform%20Movement%20Final%20Position) _movement)) (.z (Transformation|GetActorLocation Platform))) true false))))))

(event Input|EnhancedActionEvents|EnhancedInputActionIA_Jump
  (params (ActionValue :type Boolean) (ElapsedSeconds :type Float%20%28double-precision%29) (TriggeredSeconds :type Float%20%28double-precision%29) (InputAction :type Input%20Action%20Object%20Reference :default "/Game/ThirdPerson/Input/Actions/IA_Jump.IA_Jump"))
  ;[0.15 0.15 0.15 0.5] DoubleJump + Create Platform
  (:Started
    (bind _condition (CallFunction|Jumps/PlatformComprovation))
    (if _condition
      (CallFunction|ReduceSpeedonCreatePlatform)
      ;;[0.15 0.15 0.15 0.5] Creating Platform
      (bind _returnvalue (Game|SpawnActorfromClass "/Game/Project/Blueprints/Others/SpatterPlatform.SpatterPlatform_C" (Math|Transform|MakeTransform (Transformation|GetWorldLocation (Variables|Default|GetPlatformPosition)) "0, 0, 0" "1.000000,1.000000,1.000000") "Undefined" "MultiplyWithRoot" 0 0))
      (CallFunction|CalculatePlatformMovementPosition _returnvalue)
      (Variables|Default|SetPlatforms (- (Variables|Default|GetPlatforms) 1))
      (Variables|Default|SetJumpCount 0)
      (Variables|Default|SetCanMove true)
      (Variables|Default|SetJumpMaxCount 1))))

(event EventOnJumped
  (bind _jump (Timeline|Timeline_1 PlayFromStart)
    (:Update
      (Variables|/Script/Engine.CharacterMovementComponent|SetGravityScale (Variables|Character|GetCharacterMovement) _jump))))

(event EventTick
  (params (DeltaSeconds :type Float%20%28single-precision%29))
  ;[0.15 0.15 0.15 0.5] Calculate the next position to platform after spawn and move it
  (Development|PrintString (Utilities|String|ToString(Vector) (Variables|Default|GetPlatform%20Movement%20Final%20Position))))

(event EventOnLanded
  (params (Hit :type Hit%20Result%20Structure%20%28by%20ref%29))
  (CallFunction|SquashStretchLand)
  (if (not (.bSuccess (Utilities|Casting|CastToSpatterPlatform (.hitactor Hit))))
    (CallFunction|RefillPlatforms)
    (Variables|/Script/Engine.CharacterMovementComponent|SetGravityScale (Variables|Character|GetCharacterMovement) 1.0)
    (bind _jump (Timeline|Timeline_1 Stop)
      (:Update
        (Variables|/Script/Engine.CharacterMovementComponent|SetGravityScale (Variables|Character|GetCharacterMovement) _jump)))))

(fn ConstructionScript
  (|CallParentFunction))

(fn Jumps/PlatformComprovation
  ;[0.15 0.15 0.15 0.5] Check Jumps and Platforms that Player can Spawn
  (if (>= (Variables|Default|GetJumpCount) (Variables|Default|GetJumpMaxCount))
    (return (and (> (Variables|Default|GetPlatforms) 0) (AI|Components|NavMovement|IsFalling (Variables|Character|GetCharacterMovement))))
    (else
      (Variables|Default|SetJumpCount (+ (Variables|Default|GetJumpCount) 1))
      (return false))))

(fn ReduceSpeedonCreatePlatform
  (bind _charactermovement (Variables|Character|GetCharacterMovement))
  ;[0.15 0.15 0.15 0.5] Reduce speed when is create the platform
  (if (Variables|Default|GetStop%20on%20create%20platform)
    (Variables|/Script/Engine.MovementComponent|SetVelocity _charactermovement (Math|Vector|MakeVector (* (.x (Variables|/Script/Engine.MovementComponent|GetVelocity _charactermovement)) 0.5) (* (.y (Variables|/Script/Engine.MovementComponent|GetVelocity _charactermovement)) 0.5) (.z (Variables|/Script/Engine.MovementComponent|GetVelocity _charactermovement))))
    (Variables|Default|SetCanMove false)))