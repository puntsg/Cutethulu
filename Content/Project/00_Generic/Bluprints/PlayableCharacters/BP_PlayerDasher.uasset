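; BP_PlayerDasher is a playable character whose ability is a forward dash that can push objects.
; The ability input launches it along its forward vector, allowed when off cooldown or when falling with air dashes left.
; Every dash increments the air-dash counter, which resets on landing.
; While on cooldown and past a minimum distance from the dash start, PushCollider overlaps call RecibirEmpuje on BI_Pusheable actors with the forward direction.
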(event OnComponentBeginOverlap(PushCollider)
  (params (OverlappedComponent :type Primitive%20Component%20Object%20Reference) (OtherActor :type Actor%20Object%20Reference) (OtherComp :type Primitive%20Component%20Object%20Reference) (OtherBodyIndex :type Integer) (bFromSweep :type Boolean) (SweepResult :type Hit%20Result%20Structure%20%28by%20ref%29))
  (bind _returnvalue (Transformation|GetActorLocation))
  (bind _dashstartlocation (Variables|Default|GetDashStartLocation))
  ;[0.15 0.15 0.15 0.5] Push/Destroy Objects
  (if (and (not (Variables|Default|GetCanDash)) (> (Math|Vector|Distance(Vector) (Math|Vector|MakeVector (.x _dashstartlocation) (.y _dashstartlocation) 0.0) (Math|Vector|MakeVector (.x _returnvalue) (.y _returnvalue) 0.0)) (Variables|Default|GetPushMinDistance)))
    (bind _asipusheable (Utilities|Casting|CastToBI_Pusheable OtherActor))
    (Default|RecibirEmpuje _asipusheable (Transformation|GetActorForwardVector))))

(event Custom|Dash
  ;[0.15 0.15 0.15 0.5] Dash Skill
  (Variables|Default|SetCanDash false)
  (Variables|Default|SetDashStartLocation (Transformation|GetActorLocation))
  (Character|LaunchCharacter (* (Transformation|GetActorForwardVector) (Variables|Default|GetDashForce)) true true)
  (Utilities|FlowControl|Delay (Variables|Default|GetCooldown))
  (Variables|Default|SetCanDash true))

(event Input|EnhancedActionEvents|EnhancedInputActionIA_Ability
  (params (ActionValue :type Boolean) (ElapsedSeconds :type Float%20%28double-precision%29) (TriggeredSeconds :type Float%20%28double-precision%29) (InputAction :type Input%20Action%20Object%20Reference :default "/Game/ThirdPerson/Input/Actions/IA_Ability.IA_Ability"))
  ;[0.15 0.15 0.15 0.5] Use the Ability of Dash
  (:Started
    (if (or (and (AI|Components|NavMovement|IsFalling (Variables|Character|GetCharacterMovement)) (< (Variables|Default|GetDashesInAir) (Variables|Default|GetMaxDashesInAir))) (Variables|Default|GetCanDash))
      (Variables|Default|SetDashesInAir (+ (Variables|Default|GetDashesInAir) 1))
      (CallFunction|Dash))))

(event EventBeginPlay
  (|CallParentFunction) ; This node is disabled and will not be called.\nDrag off pins to build functionality.
)

(event Collision|EventActorBeginOverlap
  (params (OtherActor :type Actor%20Object%20Reference)))

(event EventTick
  (params (DeltaSeconds :type Float%20%28single-precision%29))
  (|CallParentFunction DeltaSeconds))

(event EventOnLanded
  (params (Hit :type Hit%20Result%20Structure%20%28by%20ref%29))
  ;[0.15 0.15 0.15 0.5] Reset Dashes In Air on Land
  (Variables|Default|SetDashesInAir 0))

(fn ConstructionScript
  (|CallParentFunction))