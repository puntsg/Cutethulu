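; BP_PlayerDefault_Taki is a playable character Blueprint that handles Taki's interaction input.
; The ability and secondary ability Enhanced Input actions send primary or secondary interact messages to CurrentInteractive, passing the character, when that reference is valid.
; Both paths then share one Niagara spawn of NE_attack01 at the character's location.
; Construction defers to the parent class, and CurrentInteractive is not assigned in this graph.
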(event Input|EnhancedActionEvents|EnhancedInputActionIA_Ability
  (params (ActionValue :type Boolean) (ElapsedSeconds :type Float%20%28double-precision%29) (TriggeredSeconds :type Float%20%28double-precision%29) (InputAction :type Input%20Action%20Object%20Reference :default "/Game/ThirdPerson/Input/Actions/IA_Ability.IA_Ability"))
  (bind _currentinteractive (Variables|Default|GetCurrentInteractive))
  (:Started
    (Utilities|IsValid _currentinteractive
      (:Is%20Valid
        (Class|IInteractebol|OnInteract(Message) _currentinteractive self)
        (Niagara|SpawnSystematLocation "/Game/Knife_light/VFX/NE_attack01.NE_attack01" (Transformation|GetActorLocation))))))

(event Input|EnhancedActionEvents|EnhancedInputActionIA_SecondaryAbility
  (params (ActionValue :type Boolean) (ElapsedSeconds :type Float%20%28double-precision%29) (TriggeredSeconds :type Float%20%28double-precision%29) (InputAction :type Input%20Action%20Object%20Reference :default "/Game/ThirdPerson/Input/Actions/IA_SecondaryAbility.IA_SecondaryAbility"))
  (bind _currentinteractive (Variables|Default|GetCurrentInteractive))
  (Utilities|IsValid _currentinteractive
    (:Is%20Valid
      (Class|IInteractebol|OnSecondaryInteract(Message) _currentinteractive self)
      (Niagara|SpawnSystematLocation "/Game/Knife_light/VFX/NE_attack01.NE_attack01" (Transformation|GetActorLocation)))))

(event EventBeginPlay)

(event Collision|EventActorBeginOverlap
  (params (OtherActor :type Actor%20Object%20Reference)))

(fn ConstructionScript
  (|CallParentFunction))