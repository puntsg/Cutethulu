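; Interactive sea map creature that loops along a spline and assigns its TransformClass through TestGameMode when interacted with.
; When Taki enters its sphere, it registers as the current interactive, shows ability UI and an overlay outline, decelerates and turns toward the player.
; On exit it reverses this, and Niagara effects toggle on a speed threshold.
; A looping timeline squashes and stretches the mesh, while a separate collision triggers speech text.
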(event OnComponentBeginOverlap(TextCollision)
  (params (OverlappedComponent :type Primitive%20Component%20Object%20Reference) (OtherActor :type Actor%20Object%20Reference) (OtherComp :type Primitive%20Component%20Object%20Reference) (OtherBodyIndex :type Integer) (bFromSweep :type Boolean) (SweepResult :type Hit%20Result%20Structure%20%28by%20ref%29))
  (Utilities|Casting|CastToBP_PlayableCharacter OtherActor)
  (Default|Speak (Variables|Default|GetSC_TextSystem)))

(event OnComponentEndOverlap(Sphere)
  (params (OverlappedComponent :type Primitive%20Component%20Object%20Reference) (OtherActor :type Actor%20Object%20Reference) (OtherComp :type Primitive%20Component%20Object%20Reference) (OtherBodyIndex :type Integer))
  (bind _skeletalmesh (Variables|Default|GetSkeletalMesh))
  (bind _asbp_player_default_taki (Utilities|Casting|CastToBP_PlayerDefault_Taki OtherActor))
  (Default|SetUIAbilityState _asbp_player_default_taki false)
  (Variables|/Game/Project/00_Generic/Bluprints/PlayableCharacters/BP_PlayableCharacter.BP_PlayableCharacter_C|SetCurrentInteractive _asbp_player_default_taki 0)
  (Development|PrintString "setting current map creature to null")
  (CallFunction|SetInteracted false)
  (Variables|InteractionParams|SetlookAtTaki false)
  (bind _newtrack_0 (Timeline|LookNormalTimeline PlayFromStart)
    (:Update
      (if (Variables|InteractionParams|GetIsPlayerNearby)
        (Timeline|LookNormalTimeline Stop)
        (else
          (Transformation|SetRelativeRotation _skeletalmesh (Math|Rotator|Lerp(Rotator) (Variables|/Script/Engine.SceneComponent|GetRelativeRotation _skeletalmesh) "0.000000,180.000000,0.000000" _newtrack_0 true) false false))))))

(event OnComponentBeginOverlap(Sphere)
  (params (OverlappedComponent :type Primitive%20Component%20Object%20Reference) (OtherActor :type Actor%20Object%20Reference) (OtherComp :type Primitive%20Component%20Object%20Reference) (OtherBodyIndex :type Integer) (bFromSweep :type Boolean) (SweepResult :type Hit%20Result%20Structure%20%28by%20ref%29))
  (bind _skeletalmesh (Variables|Default|GetSkeletalMesh))
  (bind _asbp_player_default_taki (Utilities|Casting|CastToBP_PlayerDefault_Taki OtherActor))
  (Default|SetUIAbilityState _asbp_player_default_taki true)
  (Variables|/Game/Project/00_Generic/Bluprints/PlayableCharacters/BP_PlayableCharacter.BP_PlayableCharacter_C|SetCurrentInteractive _asbp_player_default_taki self)
  (bind _astest_game_mode (Utilities|Casting|CastToTestGameMode (Game|GetGameMode))
    (:then
      (Default|AbilityTuto (Variables|/Game/Project/00_Generic/Bluprints/GameModes/TestGameMode.TestGameMode_C|GetPlayerUI _astest_game_mode)))
    (:CastFailed
      _))
  (CallFunction|SetInteracted true)
  (bind _newtrack_0 (Timeline|LookAtTakiTimeline PlayFromStart)
    (:Update
      (if (Variables|InteractionParams|GetIsPlayerNearby)
        (Transformation|SetWorldRotation (Variables|Default|GetSkeletalMesh) (Math|Rotator|Lerp(Rotator) (Transformation|GetWorldRotation _skeletalmesh) (Math|Rotator|FindLookatRotation (Transformation|GetActorLocation (Game|Player|GetPlayerPawn 0)) (Transformation|GetWorldLocation _skeletalmesh)) _newtrack_0 true) false false)
        (else
          (Timeline|LookAtTakiTimeline Stop))))
    (:Finished
      (Variables|InteractionParams|SetlookAtTaki true))))

(event OnComponentEndOverlap(TextCollision)
  (params (OverlappedComponent :type Primitive%20Component%20Object%20Reference) (OtherActor :type Actor%20Object%20Reference) (OtherComp :type Primitive%20Component%20Object%20Reference) (OtherBodyIndex :type Integer))
  (Utilities|Casting|CastToBP_PlayableCharacter OtherActor)
  (Default|StopSpeak (Variables|Default|GetSC_TextSystem)))

(event Custom|SetInteracted
  (params (NewState :type Boolean))
  (bind _outlinematerialinstance (Variables|InteractionParams|GetOutlineMaterialInstance))
  (bind _output_get (Variables|InteractionParams|SetIsPlayerNearby NewState))
  (if _output_get
    (Rendering|Material|SetScalarParameterValue _outlinematerialinstance "Thickness" 5.0 :!class /Script/Engine.MaterialInstanceDynamic)
    (else
      (Rendering|Material|SetScalarParameterValue _outlinematerialinstance "Thickness" 0.0 :!class /Script/Engine.MaterialInstanceDynamic))))

(event Custom|PlaySound
  (if (not (Variables|InteractionParams|GetIsPlayingSound))
    (Variables|InteractionParams|SetIsPlayingSound true)
    (bind _returnvalue (Audio|SpawnSoundatLocation (Variables|InteractionParams|GetSound) (Transformation|GetActorLocation) "0, 0, 0" 1.0 1.0 0.0 0 0))
    (EventDispatchers|AssignOnAudioFinished _returnvalue (delegate Custom|OnAudioFinished_Event))))

(event Custom|CalculateSpeed
  (bind _niagara (Variables|Default|GetNiagara))
  (if (Variables|InteractionParams|GetIsPlayerNearby)
    (bind _output_get (Variables|SpeedParams|SetSpeed (- (Variables|SpeedParams|GetSpeed) (* (Utilities|Time|GetWorldDeltaSeconds) (Variables|SpeedParams|GetDeceleration)))))
    (if (< _output_get 0.0)
      (Variables|SpeedParams|SetSpeed 0.0))
    (else
      (Variables|SpeedParams|SetSpeed (+ (Variables|SpeedParams|GetSpeed) (* (Utilities|Time|GetWorldDeltaSeconds) (Variables|SpeedParams|GetAcceleration))))
      (if (< (Variables|SpeedParams|GetMaxSpeed) (Variables|SpeedParams|GetSpeed))
        (Variables|SpeedParams|SetSpeed (Variables|SpeedParams|GetMaxSpeed)))))
  (if (< (Variables|SpeedParams|GetSpeed) (Variables|Default|GetParticlesThreshold))
    (Components|Activation|Deactivate _niagara)
    (else
      (Components|Activation|Activate _niagara false))))

(event Custom|OnAudioFinished_Event
  (Variables|InteractionParams|SetIsPlayingSound false))

(event EventBeginPlay
  (bind _skeletalmesh (Variables|Default|GetSkeletalMesh))
  (bind _returnvalue (Rendering|Material|CreateDynamicMaterialInstance "/Game/Project/04_ProvisionalElements/Material/Outliner/M_Outliner.M_Outliner" "None" "None" :!class /Script/Engine.KismetMaterialLibrary))
  (bind _output_get (Variables|InteractionParams|SetOutlineMaterialInstance _returnvalue))
  (Rendering|Material|SetOverlayMaterial _skeletalmesh _output_get :!class /Script/Engine.MeshComponent)
  (Variables|Default|SetOriginal%20Scale (Transformation|GetWorldScale _skeletalmesh))
  (bind (_direction _zstretch) (Timeline|SquashStretchTimeline Play)
    (:Update
      (Transformation|SetRelativeScale3D (Variables|Default|GetSkeletalMesh) (Math|Vector|MakeVector (.x (Variables|Default|GetOriginal%20Scale)) (.y (Variables|Default|GetOriginal%20Scale)) (* _zstretch (.z (Variables|Default|GetOriginal%20Scale))))))
    (:Finished
      (if (Utilities|Enum|Equal(Enum) _direction "Backward")
        (Timeline|SquashStretchTimeline Play)
        (else
          (Timeline|SquashStretchTimeline ReverseFromEnd))))))

(event EventTick
  (params (DeltaSeconds :type Float%20%28single-precision%29))
  (CallFunction|CalculateSpeed)
  (bind _output_get (Variables|SpeedParams|SetSplinePosition (+ (* DeltaSeconds (Variables|SpeedParams|GetSpeed)) (Variables|SpeedParams|GetSplinePosition))))
  (Transformation|SetRelativeLocationAndRotation (Variables|Default|GetCharacterOffset) (.location (Spline|GetTransformatDistanceAlongSpline (Variables|Default|GetMovementRoute) _output_get "Local" false)) (.rotation (Spline|GetTransformatDistanceAlongSpline (Variables|Default|GetMovementRoute) _output_get "Local" false)) false false)
  (if (>= (Variables|SpeedParams|GetSplinePosition) (Spline|GetSplineLength (Variables|Default|GetMovementRoute)))
    (Variables|SpeedParams|SetSplinePosition 0.0))
  (if (Variables|InteractionParams|GetlookAtTaki)
    (Transformation|SetWorldRotation (Variables|Default|GetSkeletalMesh) (Math|Rotator|FindLookatRotation (Transformation|GetActorLocation (Game|Player|GetPlayerPawn 0)) (Transformation|GetWorldLocation (Variables|Default|GetSkeletalMesh))) false false)
    (Development|PrintString "I am looking at Taki")))

(event EventOnInteract
  (params (InteractedPlayer :type BP%20Playable%20Character%20Object%20Reference))
  (Default|AssignTransform (.AsTest%20Game%20Mode (Utilities|Casting|CastToTestGameMode (Game|GetGameMode))) (Variables|TransformationParams|GetTransformClass)))

(fn ConstructionScript)