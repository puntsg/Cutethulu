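; BP_WindZone is a box-volume hazard that pushes the playable character with a configurable wind force.
; Box overlap events store or clear a single BP_PlayableCharacter reference and print debug text on entry and exit.
; Each tick, it adds WindForce through the character's movement component when airborne, or also when grounded if AffectGroundedPlayer is set.
; On BeginPlay, it spawns an attenuated wind sound at the actor's location.
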(event OnComponentBeginOverlap(Box)
  (params (OverlappedComponent :type Primitive%20Component%20Object%20Reference) (OtherActor :type Actor%20Object%20Reference) (OtherComp :type Primitive%20Component%20Object%20Reference) (OtherBodyIndex :type Integer) (bFromSweep :type Boolean) (SweepResult :type Hit%20Result%20Structure%20%28by%20ref%29))
  (bind _asbp_playable_character (Utilities|Casting|CastToBP_PlayableCharacter OtherActor))
  (Variables|Default|SetColliedCharacter _asbp_playable_character)
  (Development|PrintText "Player entrered"))

(event OnComponentEndOverlap(Box)
  (params (OverlappedComponent :type Primitive%20Component%20Object%20Reference) (OtherActor :type Actor%20Object%20Reference) (OtherComp :type Primitive%20Component%20Object%20Reference) (OtherBodyIndex :type Integer))
  (Utilities|Casting|CastToBP_PlayableCharacter OtherActor)
  (Variables|Default|SetColliedCharacter 0)
  (Development|PrintText "Player exitted"))

(event EventBeginPlay
  (Audio|SpawnSoundatLocation "/Game/Project/00_Generic/Assets/Sounds/SoundWaves_Cues/SW_Wind.SW_Wind" (Transformation|GetActorLocation) "0, 0, 0" 1.0 1.0 0.0 "/USDCore/USDDefaultAttenuation.USDDefaultAttenuation" 0))

(event EventTick
  (params (DeltaSeconds :type Float%20%28single-precision%29))
  (bind _colliedcharacter (Variables|Default|GetColliedCharacter))
  (bind _charactermovement (Variables|/Script/Engine.Character|GetCharacterMovement _colliedcharacter))
  (bind _returnvalue (AI|Components|NavMovement|IsMovingonGround _charactermovement))
  (Utilities|IsValid _colliedcharacter
    (:Is%20Valid
      (if (or (not _returnvalue) (and _returnvalue (Variables|Default|GetAffectGroundedPlayer)))
        (Physics|AddForce _charactermovement (Variables|Default|GetWindForce))))))

(fn ConstructionScript)