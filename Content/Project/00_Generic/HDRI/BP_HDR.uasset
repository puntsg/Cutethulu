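; HDRI environment actor that drives sky, lighting, post process and height fog from exposed variables.
; All work happens in the Construction Script; the event graph is unused.
; One HDR texture feeds both the SkyLight cubemap, set while the light is briefly hidden, and a dynamic material instance of M_RealisticBlueSky on the sky sphere.
; It also pushes bloom, saturation and exposure settings to PostProcess and configures the ExponentialHeightFog.
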(event EventBeginPlay)

(event Collision|EventActorBeginOverlap
  (params (OtherActor :type Actor%20Object%20Reference)))

(event EventTick
  (params (DeltaSeconds :type Float%20%28single-precision%29)))

(fn ConstructionScript
  (bind _skylight (Variables|Default|GetSkyLight))
  (bind _exponentialheightfog (Variables|Default|GetExponentialHeightFog))
  (Rendering|SetVisibility (Variables|Default|GetSkyLight) false false)
  (Class|SkyLightComponent|SetCubemap _skylight (Variables|MainHDR|GetHDRTexture))
  (Rendering|Components|Light|SetIntensity _skylight (Variables|MainHDR|GetSkyLightIntensity))
  (Rendering|SetVisibility (Variables|Default|GetSkyLight) true false)
  (Utilities|IsValid (Variables|MainHDR|GetHDRMaterial)
    (:Is%20Valid
      _)
    (:Is%20Not%20Valid
      (bind _returnvalue (Rendering|Material|CreateDynamicMaterialInstance (Variables|Default|GetSM_SkySphere) 0 "/Game/Project/00_Generic/HDRI/M_RealisticBlueSky.M_RealisticBlueSky" "None" :!class /Script/Engine.PrimitiveComponent))
      (Variables|MainHDR|SetHDRMaterial _returnvalue)))
  (Rendering|Material|SetTextureParameterValue (Variables|MainHDR|GetHDRMaterial) "SkyTextureParameter" (Variables|MainHDR|GetHDRTexture))
  (Rendering|Material|SetScalarParameterValue (Variables|MainHDR|GetHDRMaterial) "SkyBrightness" (Variables|MainHDR|GetSkyTextureBrighness) :!class /Script/Engine.MaterialInstanceDynamic)
  ;[0.15 0.15 0.15 0.5] PostProcessParam
  (Utilities|Struct|SetmembersinPostProcessSettings (Variables|/Script/Engine.PostProcessComponent|GetSettings (Variables|Default|GetPostProcess)) (Variables|PostProcess-Bloom|GetMethod) (Variables|PostProcess|GetSaturation) (Variables|PostProcess-Bloom|GetIntensity) (Variables|PostProcess-Bloom|GetSize%20Scale) (Variables|PostProcess-Bloom|Get#%201%20Size) (Variables|PostProcess-Bloom|Get#%201%20Tint) (Variables|PostProcess|GetExposure%20Compensation) (Variables|PostProcess|GetMin%20EV100) (Variables|PostProcess|GetMax%20EV100))
  ;[0.15 0.15 0.15 0.5] FogParam
  (Class|ExponentialHeightFogComponent|SetFogDensity _exponentialheightfog (Variables|Fog|GetFogDensity))
  (Class|ExponentialHeightFogComponent|SetFogHeightFalloff _exponentialheightfog (Variables|Fog|GetFogFalloff))
  (Class|ExponentialHeightFogComponent|SetFogInscatteringColor _exponentialheightfog (* (Variables|Fog|GetFogColor) (Variables|Fog|GetFogColorIntensity)))
  (Class|ExponentialHeightFogComponent|SetFogMaxOpacity _exponentialheightfog (Variables|Fog|GetMaxOpacity))
  (Class|ExponentialHeightFogComponent|SetStartDistance _exponentialheightfog (Variables|Fog|GetStartDistance)))