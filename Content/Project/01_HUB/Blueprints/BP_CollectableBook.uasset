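; BP_CollectableBook is an interactable book that opens a collectable page UI.
; Its Box overlap registers it as the player's CurrentInteractive and fades in a prompt widget through a timeline, reversing and hiding it when the player leaves.
; OnInteract stops and locks player movement, shows WBP_CollectablePage with UI-only input and a mouse cursor, and fades out the prompt.
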(event OnComponentBeginOverlap(Box)
  (params (OverlappedComponent :type Primitive%20Component%20Object%20Reference) (OtherActor :type Actor%20Object%20Reference) (OtherComp :type Primitive%20Component%20Object%20Reference) (OtherBodyIndex :type Integer) (bFromSweep :type Boolean) (SweepResult :type Hit%20Result%20Structure%20%28by%20ref%29))
  (bind _widget (Variables|Default|GetWidget))
  (bind _asbp_playable_character (Utilities|Casting|CastToBP_PlayableCharacter OtherActor))
  (Variables|/Game/Project/00_Generic/Blueprints/PlayableCharacters/BP_PlayableCharacter.BP_PlayableCharacter_C|SetCurrentInteractive _asbp_playable_character self)
  (Development|SetHiddeninGame _widget false false)
  (bind (_direction _alpha) (Timeline|TL_HiddeText PlayFromStart)
    (:Update
      (Default|Alfa (.AsWBP%20Interactive (Utilities|Casting|CastToWBP_Interactive (UserInterface|GetWidget _widget))) _alpha))
    (:Finished
      (if (Utilities|Enum|Equal(Enum) _direction "Backward")
        (Development|SetHiddeninGame (Variables|Default|GetWidget) true false)))))

(event OnComponentEndOverlap(Box)
  (params (OverlappedComponent :type Primitive%20Component%20Object%20Reference) (OtherActor :type Actor%20Object%20Reference) (OtherComp :type Primitive%20Component%20Object%20Reference) (OtherBodyIndex :type Integer))
  (bind _asbp_playable_character (Utilities|Casting|CastToBP_PlayableCharacter OtherActor))
  (Variables|/Game/Project/00_Generic/Blueprints/PlayableCharacters/BP_PlayableCharacter.BP_PlayableCharacter_C|SetCurrentInteractive _asbp_playable_character 0)
  (bind (_direction _alpha) (Timeline|TL_HiddeText Reverse)
    (:Update
      (Default|Alfa (.AsWBP%20Interactive (Utilities|Casting|CastToWBP_Interactive (UserInterface|GetWidget (Variables|Default|GetWidget)))) _alpha))
    (:Finished
      (if (Utilities|Enum|Equal(Enum) _direction "Backward")
        (Development|SetHiddeninGame (Variables|Default|GetWidget) true false)))))

(event EventOnInteract
  (params (InteractedPlayer :type BP%20Playable%20Character%20Object%20Reference))
  (bind _returnvalue (Game|Player|GetPlayerPawn 0))
  (bind _returnvalue_2 (Game|GetPlayerController 0))
  (bind _asbp_playable_character (Utilities|Casting|CastToBP_PlayableCharacter _returnvalue))
  (Default|SetCanMoveandJump _asbp_playable_character false)
  (Components|Movement|StopMovementImmediately (Variables|/Script/Engine.Character|GetCharacterMovement _asbp_playable_character))
  (bind _returnvalue_3 (UserInterface|CreateWidget "/Game/Project/00_Generic/Blueprints/UI_HUD/WBP_CollectablePage.WBP_CollectablePage_C"))
  (UserInterface|Viewport|AddtoViewport _returnvalue_3 0)
  (Input|SetInputModeUIOnly _returnvalue_2 _returnvalue_3 "DoNotLock" false)
  (Variables|/Script/Engine.PlayerController|SetbShowMouseCursor _returnvalue_2 true)
  (bind (_direction _alpha) (Timeline|TL_HiddeText Reverse)
    (:Update
      (Default|Alfa (.AsWBP%20Interactive (Utilities|Casting|CastToWBP_Interactive (UserInterface|GetWidget (Variables|Default|GetWidget)))) _alpha))
    (:Finished
      (if (Utilities|Enum|Equal(Enum) _direction "Backward")
        (Development|SetHiddeninGame (Variables|Default|GetWidget) true false)))))

(fn ConstructionScript)