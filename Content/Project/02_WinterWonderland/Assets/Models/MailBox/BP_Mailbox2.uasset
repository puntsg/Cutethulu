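; Mailbox prop Blueprint for the Winter Wonderland project that switches its look between cute and horror versions.
; OnCuteLoaded and OnHorrorLoaded each swap material slot zero on the mailbox parts, letters and gift to the matching mailbox material instance.
; The post gets a bridge material instead, with a snow variant in the horror version.
; The construction script is empty.
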(event EventOnCuteLoaded
  (Rendering|Material|SetMaterial (Variables|Default|GetMailbox_base) 0 "/Game/Project/02_WinterWonderland/Assets/Models/MailBox/MI_Mailbox_c.MI_Mailbox_c")
  (Rendering|Material|SetMaterial (Variables|Default|GetPost) 0 "/Game/Project/02_WinterWonderland/Assets/Models/Bridge/MI_Bridge_c.MI_Bridge_c"))

(event EventOnHorrorLoaded
  (Rendering|Material|SetMaterial (Variables|Default|GetMailbox_base) 0 "/Game/Project/02_WinterWonderland/Assets/Models/MailBox/MI_Mailbox_h.MI_Mailbox_h")
  (Rendering|Material|SetMaterial (Variables|Default|GetPost) 0 "/Game/Project/02_WinterWonderland/Assets/Models/Bridge/MI_Bridge_h_snow.MI_Bridge_h_snow"))

(fn ConstructionScript)