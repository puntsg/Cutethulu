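; Brick path Blueprint for the Winter Wonderland town square that switches its look between cute and horror world states.
; It holds thirty Floor components laid out as the path.
; The OnCuteLoaded and OnHorrorLoaded events set material slot 0 on every floor piece to the cute or horror town square material instance.
; The construction script is empty.
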(event EventOnCuteLoaded
  (Rendering|Material|SetMaterial (Variables|Default|GetFloor8) 0 "/Game/Project/02_WinterWonderland/Assets/Models/TownSquare/MI_TownSquare_c.MI_TownSquare_c"))

(event EventOnHorrorLoaded
  (Rendering|Material|SetMaterial (Variables|Default|GetFloor22) 0 "/Game/Project/02_WinterWonderland/Assets/Models/TownSquare/MI_TownSquare_h.MI_TownSquare_h"))

(fn ConstructionScript)