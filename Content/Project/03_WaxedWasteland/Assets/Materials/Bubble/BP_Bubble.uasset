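; BP_Bubble is an actor with three bubble meshes that the player character can pop on contact.
; Each mesh's begin-overlap event casts the other actor to BP_PlayableCharacter, destroys that mesh component and activates a paired Niagara effect.
; The pairing crosses numbering: StaticMesh1 triggers Niagara2 and StaticMesh2 triggers Niagara1.
; Each mesh pops independently, and the actor itself is never destroyed.
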(event OnComponentBeginOverlap(StaticMesh)
  (params (OverlappedComponent :type Primitive%20Component%20Object%20Reference) (OtherActor :type Actor%20Object%20Reference) (OtherComp :type Primitive%20Component%20Object%20Reference) (OtherBodyIndex :type Integer) (bFromSweep :type Boolean) (SweepResult :type Hit%20Result%20Structure%20%28by%20ref%29))
  (Utilities|Casting|CastToBP_PlayableCharacter OtherActor)
  (Components|DestroyComponent (Variables|Default|GetStaticMesh))
  (Components|Activation|Activate (Variables|Default|GetNiagara) false))

(event OnComponentBeginOverlap(StaticMesh1)
  (params (OverlappedComponent :type Primitive%20Component%20Object%20Reference) (OtherActor :type Actor%20Object%20Reference) (OtherComp :type Primitive%20Component%20Object%20Reference) (OtherBodyIndex :type Integer) (bFromSweep :type Boolean) (SweepResult :type Hit%20Result%20Structure%20%28by%20ref%29))
  (Utilities|Casting|CastToBP_PlayableCharacter OtherActor)
  (Components|DestroyComponent (Variables|Default|GetStaticMesh1))
  (Components|Activation|Activate (Variables|Default|GetNiagara2) false))

(event OnComponentBeginOverlap(StaticMesh2)
  (params (OverlappedComponent :type Primitive%20Component%20Object%20Reference) (OtherActor :type Actor%20Object%20Reference) (OtherComp :type Primitive%20Component%20Object%20Reference) (OtherBodyIndex :type Integer) (bFromSweep :type Boolean) (SweepResult :type Hit%20Result%20Structure%20%28by%20ref%29))
  (Utilities|Casting|CastToBP_PlayableCharacter OtherActor)
  (Components|DestroyComponent (Variables|Default|GetStaticMesh2))
  (Components|Activation|Activate (Variables|Default|GetNiagara1) false))

(event EventBeginPlay)

(event Collision|EventActorBeginOverlap
  (params (OtherActor :type Actor%20Object%20Reference)))

(event EventTick
  (params (DeltaSeconds :type Float%20%28single-precision%29)))

(fn ConstructionScript)