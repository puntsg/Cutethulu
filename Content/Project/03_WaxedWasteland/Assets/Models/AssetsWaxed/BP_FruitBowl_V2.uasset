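; BP_FruitBowl_V2 is a fruit bowl prop made of a plate and several low-poly orange meshes that reskins itself between horror and cute versions of the world.
; The OnHorrorLoaded and OnCuteLoaded events set the first material slot on the plate and every orange to the matching horror or cute material instance.
; The construction script is empty, so all switching happens through these two events.
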(event EventOnHorrorLoaded
  (Rendering|Material|SetMaterial 0 0 "/Game/Project/03_WaxedWasteland/Assets/Models/AssetsWaxed/MI_AssetsWAWE_h.MI_AssetsWAWE_h"))

(event EventOnCuteLoaded
  (Rendering|Material|SetMaterial 0 0 "/Game/Project/03_WaxedWasteland/Assets/Models/AssetsWaxed/MI_AssetsWAWE_c.MI_AssetsWAWE_c"))

(fn ConstructionScript)