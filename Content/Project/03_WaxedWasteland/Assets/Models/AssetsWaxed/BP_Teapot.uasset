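; BP_Teapot is a teapot set piece with bridge pillar and stone meshes that switches between horror and cute visual themes.
; OnHorrorLoaded and OnCuteLoaded events swap slot 0 materials on the teapot, three pillars and three stones to the matching horror or cute variants.
; The construction script is empty, and nothing in this Blueprint triggers the theme events itself.
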(event EventOnHorrorLoaded
  (Rendering|Material|SetMaterial (Variables|Default|GetTeapot_low) 0 "/Game/Project/03_WaxedWasteland/Assets/Models/AssetsWaxed/MI_AssetsWAWE_h.MI_AssetsWAWE_h")
  (Rendering|Material|SetMaterial (Variables|Default|GetSM_bridge_pilar1) 0 "/Game/Project/02_WinterWonderland/Assets/Models/Bridge/MI_Bridge_h.MI_Bridge_h")
  (Rendering|Material|SetMaterial (Variables|Default|GetSM_Stone_11) 0 "/Game/Project/00_Generic/Assets/Models/Stones/MI_Rocks_h.MI_Rocks_h"))

(event EventOnCuteLoaded
  (Rendering|Material|SetMaterial (Variables|Default|GetTeapot_low) 0 "/Game/Project/03_WaxedWasteland/Assets/Models/AssetsWaxed/MI_AssetsWAWE_c.MI_AssetsWAWE_c")
  (Rendering|Material|SetMaterial (Variables|Default|GetSM_bridge_pilar1) 0 "/Game/Project/02_WinterWonderland/Assets/Models/Bridge/MI_Bridge_c.MI_Bridge_c")
  (Rendering|Material|SetMaterial (Variables|Default|GetSM_Stone_10) 0 "/Game/Project/00_Generic/Assets/Models/Stones/MI_Rocks_c.MI_Rocks_c"))

(fn ConstructionScript)