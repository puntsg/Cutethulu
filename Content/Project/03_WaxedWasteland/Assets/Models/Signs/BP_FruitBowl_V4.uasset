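; BP_FruitBowl_V4 is a fruit bowl prop in the Waxed Wasteland level that changes its look between cute and horror variants.
; The OnHorrorLoaded and OnCuteLoaded events swap the first material slot on the plate mesh and five orange meshes.
; The plate uses the shared WAWE asset materials, while the oranges use the Signs materials, each in a horror or cute version.
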(event EventOnHorrorLoaded
  (Rendering|Material|SetMaterial (Variables|Default|GetPlate_low) 0 "/Game/Project/03_WaxedWasteland/Assets/Models/AssetsWaxed/MI_AssetsWAWE_h.MI_AssetsWAWE_h")
  (Rendering|Material|SetMaterial (Variables|Default|GetSM_Orange3) 0 "/Game/Project/03_WaxedWasteland/Assets/Models/Signs/MI_Signs_h.MI_Signs_h"))

(event EventOnCuteLoaded
  (Rendering|Material|SetMaterial (Variables|Default|GetPlate_low) 0 "/Game/Project/03_WaxedWasteland/Assets/Models/AssetsWaxed/MI_AssetsWAWE_c.MI_AssetsWAWE_c")
  (Rendering|Material|SetMaterial (Variables|Default|GetSM_Orange3) 0 "/Game/Project/03_WaxedWasteland/Assets/Models/Signs/MI_Signs_c.MI_Signs_c"))

(fn ConstructionScript)