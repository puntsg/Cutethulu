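; BP_Sign5 is a sign prop that changes its look between cute and horror versions of the world.
; The OnCuteLoaded and OnHorrorLoaded events swap the first material slot on the sign, post, two rope bell meshes and rubble to the matching variant.
; The rubble uses dither materials in both versions, and the construction script is empty.
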(event EventOnCuteLoaded
  (Rendering|Material|SetMaterial (Variables|Default|GetSign) 0 "/Game/Project/03_WaxedWasteland/Assets/Models/Signs/MI_Signs_c.MI_Signs_c")
  (Rendering|Material|SetMaterial (Variables|Default|GetPost) 0 "/Game/Project/02_WinterWonderland/Assets/Models/Bridge/MI_Bridge_c.MI_Bridge_c")
  (Rendering|Material|SetMaterial (Variables|Default|GetSM_Ropebell) 0 "/Game/Project/02_WinterWonderland/Assets/Models/Bell/MI_bell_c.MI_bell_c")
  (Rendering|Material|SetMaterial (Variables|Default|GetSM_Rubble) 0 "/Game/Project/03_WaxedWasteland/Assets/Models/Signs/M_Signs_c_dither.M_Signs_c_dither"))

(event EventOnHorrorLoaded
  (Rendering|Material|SetMaterial (Variables|Default|GetSign) 0 "/Game/Project/03_WaxedWasteland/Assets/Models/Signs/MI_Signs_h.MI_Signs_h")
  (Rendering|Material|SetMaterial (Variables|Default|GetPost) 0 "/Game/Project/02_WinterWonderland/Assets/Models/Bridge/MI_Bridge_h.MI_Bridge_h")
  (Rendering|Material|SetMaterial (Variables|Default|GetSM_Ropebell1) 0 "/Game/Project/02_WinterWonderland/Assets/Models/Bell/MI_bell_h.MI_bell_h")
  (Rendering|Material|SetMaterial (Variables|Default|GetSM_Rubble) 0 "/Game/Project/03_WaxedWasteland/Assets/Models/Signs/M_Signs_h_dither.M_Signs_h_dither"))

(fn ConstructionScript)