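; Player controller for the Cutethulu character that owns the level UI widget and tracks the count of collected pieces.
; ShowLevelUI creates the given widget class and adds it to the viewport, but only removes the current widget if one already exists.
; HideLevelUI removes and clears that widget.
; AddPiece increments the count and, when a widget is valid, passes it to WBP_LevelUI_Base and prints it.
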(event EventBeginPlay)

(event EventTick
  (params (DeltaSeconds :type Float%20%28single-precision%29)))

(fn ConstructionScript)

(fn ShowLevelUI
  (params (WidgetClass :type User%20Widget%20Class%20Reference))
  (if (!= WidgetClass 0)
    (if (!= (Variables|Default|GetLevelUI_Widget) 0)
      (Widget|RemovefromParent (Variables|Default|GetLevelUI_Widget))
      (Variables|Default|SetLevelUI_Widget 0)
      (else
        (bind _returnvalue (UserInterface|CreateWidget WidgetClass))
        (bind _output_get (Variables|Default|SetLevelUI_Widget _returnvalue))
        (UserInterface|Viewport|AddtoViewport _output_get 0)))))

(fn HideLevelUI
  (if (!= (Variables|Default|GetLevelUI_Widget) 0)
    (Widget|RemovefromParent (Variables|Default|GetLevelUI_Widget))
    (Variables|Default|SetLevelUI_Widget 0)))

(fn AddPiece
  (bind _currentpieces (Variables|Default|GetcurrentPieces))
  (Math|Integer|IncrementInt (Variables|Default|GetcurrentPieces)
    (:%20%20
      (bind _levelui_widget (Variables|Default|GetLevelUI_Widget)
        (:then
          (bind _aswbp_level_ui_base (Utilities|Casting|CastToWBP_LevelUI_Base _levelui_widget))
          (Default|UpdatePiecesUI _aswbp_level_ui_base _currentpieces)
          (Development|PrintString (Utilities|String|ToString(Integer) _currentpieces)))
        (:else)))))