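; Dasher is a character with a forward dash ability that can push objects, plus a jump input that calls ExecuteJump.
; The ability input launches it along its facing, overriding velocity, then halts movement after a short delay.
; Tick restores the dash through a cooldown Delay triggered once the character is not falling.
; While the dash is unavailable, including cooldown, PushCollider overlaps send the forward vector to IPusheable actors via RecibirEmpuje.
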(event OnComponentBeginOverlap(PushCollider)
  (params (OverlappedComponent :type Primitive%20Component%20Object%20Reference) (OtherActor :type Actor%20Object%20Reference) (OtherComp :type Primitive%20Component%20Object%20Reference) (OtherBodyIndex :type Integer) (bFromSweep :type Boolean) (SweepResult :type Hit%20Result%20Structure%20%28by%20ref%29))
  (if (not (Variables|Default|GetCanDash))
    (bind _asipusheable (Utilities|Casting|CastToIPusheable OtherActor))
    (Default|RecibirEmpuje _asipusheable (Transformation|GetActorForwardVector))))

(event Input|EnhancedActionEvents|EnhancedInputActionIA_Ability
  (params (ActionValue :type Boolean) (ElapsedSeconds :type Float%20%28double-precision%29) (TriggeredSeconds :type Float%20%28double-precision%29) (InputAction :type Input%20Action%20Object%20Reference :default "/Game/ThirdPerson/Input/Actions/IA_Ability.IA_Ability"))
  (:Started
    (if (Variables|Default|GetCanDash)
      (Variables|Default|SetCanDash false)
      (Character|LaunchCharacter (* (Transformation|GetActorForwardVector) (Variables|Default|GetDashSpeed)) true true)
      (Utilities|FlowControl|Delay 0.2)
      (Components|Movement|StopMovementImmediately (Variables|Character|GetCharacterMovement)))))

(event Input|EnhancedActionEvents|EnhancedInputActionIA_Jump
  (params (ActionValue :type Boolean) (ElapsedSeconds :type Float%20%28double-precision%29) (TriggeredSeconds :type Float%20%28double-precision%29) (InputAction :type Input%20Action%20Object%20Reference :default "/Game/ThirdPerson/Input/Actions/IA_Jump.IA_Jump"))
  (:Started
    (CallFunction|ExecuteJump)))

(event EventBeginPlay
  (|CallParentFunction) ; This node is disabled and will not be called.\nDrag off pins to build functionality.
)

(event Collision|EventActorBeginOverlap
  (params (OtherActor :type Actor%20Object%20Reference)))

(event EventTick
  (params (DeltaSeconds :type Float%20%28single-precision%29))
  (|CallParentFunction DeltaSeconds)
  (if (not (Variables|Default|GetCanDash))
    (if (not (AI|Components|NavMovement|IsFalling (Variables|Character|GetCharacterMovement)))
      (Utilities|FlowControl|Delay (Variables|Default|GetCooldown))
      (Variables|Default|SetCanDash true))))

(fn ConstructionScript
  (|CallParentFunction))