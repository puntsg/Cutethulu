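; Spatter character Blueprint that adds a mid-air cloud platform to jumping.
; Once jumps are used up while falling, condition macros gate an optional slowdown, then a short delay before spawning a SpatterPlatform and spending a charge.
; A Timeline drives gravity scale during jumps.
; Landing triggers squash and stretch; landing off a platform also refills charges and resets gravity.
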(event Custom|RefillPlatforms
  ;[0.15 0.15 0.15 0.5] Refill Platforms
  (Variables|Default|SetPlatforms 1)
  (Variables|Default|SetJumpMaxCount 2)
  (Variables|Default|SetJumpCount 1)
  (Development|PrintString "RefillingClouds"))

(event Input|EnhancedActionEvents|EnhancedInputActionIA_Jump
  (params (ActionValue :type Boolean) (ElapsedSeconds :type Float%20%28double-precision%29) (TriggeredSeconds :type Float%20%28double-precision%29) (InputAction :type Input%20Action%20Object%20Reference :default "/Game/ThirdPerson/Input/Actions/IA_Jump.IA_Jump"))
  (bind _charactermovement (Variables|Character|GetCharacterMovement))
  ;[0.15 0.15 0.15 0.5] DoubleJump + Create Platform
  (:Started
    ;;[0.15 0.15 0.15 0.5] hasta que no este el ABP_Spatter
    (CallFunction|ExecuteJump)
    (Utilities|Jump/PlatformCondition
      (:Exit
        (Utilities|AirControlCondition
          (:Fail
            (if (Variables|Default|GetStop%20on%20create%20cloud)
              (Variables|/Script/Engine.MovementComponent|SetVelocity _charactermovement (Math|Vector|MakeVector (* (.x (Variables|/Script/Engine.MovementComponent|GetVelocity _charactermovement)) 0.5) (* (.y (Variables|/Script/Engine.MovementComponent|GetVelocity _charactermovement)) 0.5) (.z (Variables|/Script/Engine.MovementComponent|GetVelocity _charactermovement))))
              (Variables|Default|SetCanMove false))
            (Utilities|FlowControl|Delay 0.2)
            (Game|SpawnActorfromClass "/Game/Project/Blueprints/Others/SpatterPlatform.SpatterPlatform_C" (Math|Transform|MakeTransform (Transformation|GetWorldLocation (Variables|Default|GetPlatformPosition)) "0, 0, 0" "1.000000,1.000000,1.000000") "Undefined" "MultiplyWithRoot" 0 0)
            (Variables|Default|SetPlatforms (- (Variables|Default|GetPlatforms) 1))
            (Variables|Default|SetJumpCount 0)
            (Variables|Default|SetCanMove true)
            (Variables|Default|SetJumpMaxCount 1)))))))

(event EventOnJumped
  (bind _jump (Timeline|Timeline_1 PlayFromStart)
    (:Update
      (Variables|/Script/Engine.CharacterMovementComponent|SetGravityScale (Variables|Character|GetCharacterMovement) _jump))))

(event EventTick
  (params (DeltaSeconds :type Float%20%28single-precision%29))
  (|CallParentFunction DeltaSeconds)
  (Development|PrintString (Utilities|String|ToString(Float) (Variables|/Script/Engine.CharacterMovementComponent|GetAirControl (Variables|Character|GetCharacterMovement)))))

(event EventOnLanded
  (params (Hit :type Hit%20Result%20Structure%20%28by%20ref%29))
  (CallFunction|SquashStretchLand)
  (if (not (.bSuccess (Utilities|Casting|CastToSpatterPlatform (.hitactor Hit))))
    (CallFunction|RefillPlatforms)
    (Variables|/Script/Engine.CharacterMovementComponent|SetGravityScale (Variables|Character|GetCharacterMovement) 1.0)
    (bind _jump (Timeline|Timeline_1 Stop)
      (:Update
        (Variables|/Script/Engine.CharacterMovementComponent|SetGravityScale (Variables|Character|GetCharacterMovement) _jump)))))

(fn ConstructionScript
  (|CallParentFunction))