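; SpeedFish is a playable fish character whose ability is a swim-speed boost.
; Holding the ability input raises max swim speed and updates the ability UI state, and releasing or canceling restores both.
; Each tick, boosting with movement input plays a one-shot acceleration sound and widens the camera FOV through a timeline that reverses otherwise.
; Tick also calls the speed particle calculation.
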(event Input|EnhancedActionEvents|EnhancedInputActionIA_Ability
  (params (ActionValue :type Boolean) (ElapsedSeconds :type Float%20%28double-precision%29) (TriggeredSeconds :type Float%20%28double-precision%29) (InputAction :type Input%20Action%20Object%20Reference :default "/Game/ThirdPerson/Input/Actions/IA_Ability.IA_Ability"))
  (bind _charactermovement (Variables|Character|GetCharacterMovement))
  (:Triggered
    (Variables|/Script/Engine.CharacterMovementComponent|SetMaxSwimSpeed _charactermovement 1.9e+03 :!label _label)
    (Variables|SpeedFishVars|SetisSwimmingFast true)
    (CallFunction|SetUIAbilityState true))
  (:Started
    (goto _label))
  (:Canceled
    (Variables|/Script/Engine.CharacterMovementComponent|SetMaxSwimSpeed _charactermovement 1.3e+03 :!label _label_2)
    (Variables|SpeedFishVars|SetisSwimmingFast false)
    (CallFunction|SetUIAbilityState false))
  (:Completed
    (goto _label_2)))

(event EventBeginPlay)

(event Collision|EventActorBeginOverlap
  (params (OtherActor :type Actor%20Object%20Reference)))

(event EventTick
  (params (DeltaSeconds :type Float%20%28single-precision%29))
  (bind _output_get (Variables|SpeedFishVars|SetIsAccelerating (and (not (Class|KismetMathLibrary|IsZero2D (Input|EnhancedActionValues|GetIA_Move))) (Variables|SpeedFishVars|GetisSwimmingFast))))
  (if _output_get
    (if (Variables|SpeedFishVars|GetcanPlayAccelerateSound)
      (Utilities|IsValid (Variables|Default|GetSound)
        (:Is%20Valid
          (if (Audio|Components|Audio|IsPlaying (Variables|Default|GetSound))
            (Audio|Components|Audio|Stop (Variables|Default|GetSound))))
        (:Is%20Not%20Valid
          _))
      (bind _returnvalue (Audio|SpawnSound2D "/Game/Project/Assets/Sounds/Acceleration.Acceleration" 1.0 1.0 0.0 0))
      (Variables|Default|SetSound _returnvalue)
      (Variables|SpeedFishVars|SetcanPlayAccelerateSound false))
    (else
      (Variables|SpeedFishVars|SetcanPlayAccelerateSound true)))
  (CallFunction|CalculateSpeedParticles)
  (if (Variables|SpeedFishVars|GetIsAccelerating)
    (bind _newtrack_1 (Timeline|getaway Play)
      (:Update
        (Camera|SetFieldOfView (Variables|Default|GetFollowCamera) (Math|Float|Lerp 9e+01 1.2e+02 _newtrack_1))))
    (else
      (Timeline|getaway Reverse))))

(fn ConstructionScript
  (|CallParentFunction))