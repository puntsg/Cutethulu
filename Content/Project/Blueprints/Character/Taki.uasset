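; Taki is a playable character that takes a transformation from map creatures and changes into that form.
; The ability input plays an effect and sound on the targeted creature, stores its transform class and updates UI icons, optionally transforming immediately.
; The transform input prioritizes the current interactive, otherwise transforming into the first existing level actor of the stored class if allowed.
; UI updates cast to two different game modes, Proto3GameMode and TestGameMode.
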(event Input|EnhancedActionEvents|EnhancedInputActionIA_Transform
  (params (ActionValue :type Boolean) (ElapsedSeconds :type Float%20%28double-precision%29) (TriggeredSeconds :type Float%20%28double-precision%29) (InputAction :type Input%20Action%20Object%20Reference :default "/Game/ThirdPerson/Input/Actions/IA_Transform.IA_Transform"))
  (bind _currentinteractive (Variables|Default|GetCurrentInteractive))
  (bind _creaturetoswap (Variables|TakiVars|GetCreatureToSwap))
  (:Started
    (Utilities|IsValid _currentinteractive
      (:Is%20Valid
        (Class|IInteractebol|OnInteract(Message) _currentinteractive))
      (:Is%20Not%20Valid
        (Development|PrintString "Executing taki transform")
        (if (Utilities|IsValidClass _creaturetoswap)
          (bind _outactors (Actor|GetAllActorsOfClass _creaturetoswap))
          (Utilities|IsValid (Utilities|Array|Get(acopy) _outactors)
            (:Is%20Valid
              (bind _asplayable_character (Utilities|Casting|CastToPlayableCharacter (Utilities|Array|Get(acopy) _outactors)))
              (bind _astest_game_mode (Utilities|Casting|CastToTestGameMode (Game|GetGameMode)))
              (bind _cantransform (CallFunction|CanTransform))
              (if _cantransform
                (Variables|Default|SetisTransforming true)
                (CallFunction|Transform _asplayable_character)
                (Default|SetTransformationUI (Variables|/Game/Project/Blueprints/Character/TestGameMode.TestGameMode_C|GetPlayerUI _astest_game_mode)))))
          (else
            (Development|PrintString "There's no assigned class")))))))

(event Input|EnhancedActionEvents|EnhancedInputActionIA_Ability
  (params (ActionValue :type Boolean) (ElapsedSeconds :type Float%20%28double-precision%29) (TriggeredSeconds :type Float%20%28double-precision%29) (InputAction :type Input%20Action%20Object%20Reference :default "/Game/ThirdPerson/Input/Actions/IA_Ability.IA_Ability"))
  (bind _currentpoiningmapcreature (Variables|TakiVars|GetCurrentPoiningMapCreature))
  (:Started
    (Utilities|IsValid _currentpoiningmapcreature
      (:Is%20Valid
        (Niagara|SpawnSystematLocation "/Game/Knife_light/VFX/NE_attack01.NE_attack01" (Transformation|GetWorldLocation (Variables|/Game/Project/Blueprints/Scenario/SeaMapCreature.SeaMapCreature_C|GetSkeletalMesh _currentpoiningmapcreature)))
        (Variables|TakiVars|SetCreatureToSwap (Variables|/Game/Project/Blueprints/Scenario/SeaMapCreature.SeaMapCreature_C|GetTransformClass _currentpoiningmapcreature))
        (bind _asproto_3game_mode (Utilities|Casting|CastToProto3GameMode (Game|GetGameMode)))
        (Default|AssignTransformationIcons (Variables|/Game/Project/Blueprints/Character/Proto3GameMode.Proto3GameMode_C|GetPlayerUI _asproto_3game_mode) (Variables|/Game/Project/Blueprints/Scenario/SeaMapCreature.SeaMapCreature_C|GetTransformationIcon _currentpoiningmapcreature) (Variables|/Game/Project/Blueprints/Scenario/SeaMapCreature.SeaMapCreature_C|GetAbilityIcon _currentpoiningmapcreature))
        (Default|PlaySound _currentpoiningmapcreature)
        (if (Variables|Default|GetTransformAfterInteract)
          (Development|PrintString "Executing taki transform")
          (if (Utilities|IsValidClass (Variables|TakiVars|GetCreatureToSwap))
            (bind _outactors (Actor|GetAllActorsOfClass (Variables|TakiVars|GetCreatureToSwap)))
            (Utilities|IsValid (Utilities|Array|Get(acopy) _outactors)
              (:Is%20Valid
                (bind _asplayable_character (Utilities|Casting|CastToPlayableCharacter (Utilities|Array|Get(acopy) _outactors)))
                (bind _astest_game_mode (Utilities|Casting|CastToTestGameMode (Game|GetGameMode)))
                (bind _cantransform (CallFunction|CanTransform))
                (if _cantransform
                  (Variables|Default|SetisTransforming true)
                  (CallFunction|Transform _asplayable_character)
                  (Default|SetTransformationUI (Variables|/Game/Project/Blueprints/Character/TestGameMode.TestGameMode_C|GetPlayerUI _astest_game_mode)))))
            (else
              (Development|PrintString "There's no assigned class"))))))))

(event EventBeginPlay)

(event Collision|EventActorBeginOverlap
  (params (OtherActor :type Actor%20Object%20Reference)))

(fn ConstructionScript
  (|CallParentFunction))