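; Game mode for the Taki character game that sets up player UI and handles the transition from main menu camera to gameplay.
; BeginPlay applies debug display options, creates the collapsed player HUD and collectables widget, and adds the game instance's fade widget.
; PlayerTransition uses a timeline to lerp the menu camera onto Taki's follow camera while switching music, then enables input, blends view and starts the tutorial.
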(event Custom|PlayerTransition
  (bind _returnvalue (Game|GetPlayerController 0))
  (bind _returnvalue_2 (Game|Player|GetPlayerPawn 0))
  (bind _currentsoundplayer (Variables|Default|GetCurrentSoundPlayer))
  (bind _cameramainmenu (Variables|Default|GetcameraMainMenu))
  (bind _newtrack_0 (Timeline|Timeline Play)
    (:Update
      (bind _astaki (Utilities|Casting|CastToTaki (Game|Player|GetPlayerPawn 0)))
      (Transformation|SetWorldTransform _cameramainmenu (Math|Transform|Lerp(Transform) (Transformation|GetWorldTransform _cameramainmenu) (Transformation|GetWorldTransform (Variables|/Game/Project/Blueprints/Character/PlayableCharacter.PlayableCharacter_C|GetFollowCamera _astaki)) _newtrack_0) true false)
      ;[0.15 0.15 0.15 0.5] Trying to do Fade Out
      (Class|CameraComponent|SetPostProcessBlendWeight (Variables|Default|GetcameraMainMenu) _newtrack_0)
      (Audio|Components|Audio|FadeOut _currentsoundplayer 0.2 0.0 "Linear" :!class /Script/Engine.AudioComponent)
      (Utilities|FlowControl|Delay 0.2)
      (Audio|Components|Audio|SetSound _currentsoundplayer "/Game/Project/Assets/Sounds/Deep_Sea___Cinematic_Underwater_Music___Royalty_Free.Deep_Sea___Cinematic_Underwater_Music___Royalty_Free"))
    (:Finished
      (Input|EnableInput _returnvalue _returnvalue)
      (Transformation|ResetRelativeTransform (Variables|/Game/Project/Blueprints/Character/PlayableCharacter.PlayableCharacter_C|GetFollowCamera _astaki))
      (Components|Activation|SetActive (Variables|Default|GetcameraMainMenu) false false)
      (bind _astaki_2 (Utilities|Casting|CastToTaki _returnvalue_2))
      (Game|Player|SetViewTargetwithBlend (Game|GetPlayerController 0) _returnvalue_2 0.0 "VTBlend_Linear" 0.0 false)
      (Default|BasicTutorial (Variables|Default|GetPlayerUI)))))

(event EventBeginPlay
  (if (Variables|Default|GetShowFPS)
    (Development|ExecuteConsoleCommand "stat fps" 0))
  (CallFunction|Show/HidePrintString)
  (Utilities|IsValid (Variables|Default|GetPlayerUI)
    (:Is%20Valid
      _)
    (:Is%20Not%20Valid
      (bind _returnvalue (UserInterface|CreateWidget "/Game/Project/Blueprints/UI/PlayerUI.PlayerUI_C"))
      (bind _output_get (Variables|Default|SetPlayerUI _returnvalue))))
  (UserInterface|Viewport|AddtoViewport _output_get 0)
  (bind _outactors (Actor|GetAllActorsOfClass "/Game/Project/Blueprints/Character/Taki.Taki_C"))
  (Variables|Default|SetOriginalCharacter (Utilities|Array|Get(acopy) _outactors))
  (CallFunction|ShowPlayerUI false)
  (bind _asbp_cutethulu_instance (Utilities|Casting|CastToBP_CutethuluInstance (Game|GetGameInstance)))
  (UserInterface|Viewport|AddtoViewport (Variables|/Game/Project/Blueprints/Others/BP_CutethuluInstance.BP_CutethuluInstance_C|GetFadeWRef _asbp_cutethulu_instance) 0))

(fn ConstructionScript)

(fn Show/HidePrintString
  (if (Variables|Default|GetShowStrings)
    (Development|ExecuteConsoleCommand "Enableallscreenmessages" 0)
    (else
      (Development|ExecuteConsoleCommand "Disableallscreenmessages" 0)))
  (bind _returnvalue (UserInterface|CreateWidget "/Game/Project/Blueprints/UI/UI_LevelCollectables.UI_LevelCollectables_C"))
  (UserInterface|Viewport|AddtoViewport _returnvalue 0))

(fn ShowPlayerUI
  (params (IsVisible%28PlayerUI%29 :type Boolean))
  (bind _playerui (Variables|Default|GetPlayerUI))
  (if IsVisible%28PlayerUI%29
    (Widget|SetVisibility _playerui "Visible")
    (else
      (Widget|SetVisibility _playerui "Collapsed"))))

(fn Fadein
  (bind _fadewref (Variables|Default|GetFadeWRef))
  (Widget|SetVisibility _fadewref "Visible")
  (UserInterface|Animation|PlayAnimation _fadewref (Variables|/Game/Project/Blueprints/UI/WBP_Fade.WBP_Fade_C|GetFadeIn _fadewref) 0.0 1 "Forward" 1.0 false))

(fn FadeOut
  (bind _fadewref (Variables|Default|GetFadeWRef))
  (Widget|SetVisibility _fadewref "Hidden")
  (UserInterface|Animation|PlayAnimation _fadewref (Variables|/Game/Project/Blueprints/UI/WBP_Fade.WBP_Fade_C|GetFadeOut _fadewref) 0.0 1 "Forward" 1.0 false))