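; Scene component that shows floating text messages attached to its owning actor.
; Each Speak call adds a new screen-space WidgetComponent to the owner, attaches it to this component and fills it with a widget created from WidgetClass for player 0.
; The message is written to the widget's FinalText only if it casts to WBP_FloatingText.
; The component itself does not track or remove the spawned widgets.
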(event EventBeginPlay)

(event EventTick
  (params (DeltaSeconds :type Float%20%28single-precision%29)))

(fn Speak
  (params (Message :type Text))
  (bind _returnvalue (Game|AddComponentbyClass (Components|GetOwner) "/Script/UMG.WidgetComponent" false))
  (Transformation|AttachComponentToComponent _returnvalue self "None" "KeepRelative" "KeepRelative" "KeepRelative" true)
  (Class|WidgetComponent|SetWidgetSpace _returnvalue "Screen")
  (bind _returnvalue_2 (UserInterface|CreateWidget (Variables|Default|GetWidgetClass) (Game|GetPlayerController 0)))
  (UserInterface|SetWidget _returnvalue _returnvalue_2)
  (bind _aswbp_floating_text (Utilities|Casting|CastToWBP_FloatingText _returnvalue_2))
  (Variables|/Game/Project/Blueprints/UI/WBP_FloatingText.WBP_FloatingText_C|SetFinalText _aswbp_floating_text Message))