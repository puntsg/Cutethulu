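; Scene component that shows timed dialogue messages in a screen-space widget attached to its owner.
; On BeginPlay it creates the widget component and hidden widget; NewDialogue replaces the message list.
; Speak reveals and animates the widget, then NextText recursively steps through messages with length-scaled delays, though a single message shows CurrentMessage without assigning it.
; StopSpeak triggers the other animation state, but the HideOnFinish auto-call is unconnected.
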(event Custom|NextText
  (if (and (< (Variables|Default|GetDialogueIndex) (Utilities|Array|Length (Variables|Default|GetMessages))) (Variables|Default|GetIsSpeaking))
    (bind _output_get (Variables|Default|SetCurrentMessage (Utilities|Array|Get(acopy) (Variables|Default|GetMessages) (Variables|Default|GetDialogueIndex))))
    (Class|ISpeakable|Talk(Message) (Variables|Default|GetWidgetReference) _output_get)
    (Math|Integer|IncrementInt (Variables|Default|GetDialogueIndex)
      (:%20%20
        (Utilities|FlowControl|Delay (* (Utilities|String|Len (Utilities|String|ToString(Text) (Variables|Default|GetCurrentMessage))) 0.25))
        (CallFunction|NextText)))
    (else
      (Variables|Default|SetIsSpeaking false))))

(event Custom|NewDialogue
  (params (NewDialogue :type Array%20of%20Texts))
  (Utilities|Array|Clear (Variables|Default|GetMessages))
  (Variables|Default|SetMessages NewDialogue))

(event EventBeginPlay
  (bind _returnvalue (Game|AddComponentbyClass (Components|GetOwner) "/Script/UMG.WidgetComponent" false))
  (bind _output_get (Variables|Default|SetWidgetComponentReference _returnvalue))
  (Transformation|AttachComponentToComponent _output_get self "None" "KeepRelative" "KeepRelative" "KeepRelative" true)
  (Class|WidgetComponent|SetWidgetSpace (Variables|Default|GetWidgetComponentReference) "Screen")
  (bind _returnvalue_2 (UserInterface|CreateWidget (Variables|Default|GetWidgetClass) (Game|GetPlayerController 0)))
  (bind _output_get_2 (Variables|Default|SetWidgetReference _returnvalue_2))
  (UserInterface|SetWidget (Variables|Default|GetWidgetComponentReference) _output_get_2)
  (Widget|SetVisibility (Variables|Default|GetWidgetReference) "Hidden"))

(fn Speak
  (bind _widgetreference (Variables|Default|GetWidgetReference))
  (bind _widgetreference_2 (Variables|Default|GetWidgetReference))
  (if (== (Utilities|Array|Length (Variables|Default|GetMessages)) 1)
    (Class|ISpeakable|Talk(Message) _widgetreference (Variables|Default|GetCurrentMessage))
    (Widget|SetVisibility _widgetreference "SelfHitTestInvisible")
    (Class|ISpeakable|DialogueAnimation(Message) _widgetreference "NewEnumerator1")
    (else
      (Variables|Default|SetDialogueIndex 0)
      (Variables|Default|SetIsSpeaking true)
      (Widget|SetVisibility _widgetreference_2 "SelfHitTestInvisible")
      (Class|ISpeakable|DialogueAnimation(Message) _widgetreference_2 "NewEnumerator1")
      (CallFunction|NextText))))

(fn StopSpeak
  (Class|ISpeakable|DialogueAnimation(Message) (Variables|Default|GetWidgetReference) "NewEnumerator0"))