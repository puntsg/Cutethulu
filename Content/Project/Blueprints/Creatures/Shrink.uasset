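; Creature Blueprint whose ability input toggles the actor between normal and shrunken size.
; A Shrinked flag picks whether ShrinkTimeline plays forward or in reverse, driving uniform actor scale through its SizeMultiplier track.
; Input is ignored while transforming or while the timeline runs.
; When the timeline finishes, CanExecuteTransform is set to allow transforming only when not shrunk.
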(event Input|EnhancedActionEvents|EnhancedInputActionIA_Ability
  (params (ActionValue :type Boolean) (ElapsedSeconds :type Float%20%28double-precision%29) (TriggeredSeconds :type Float%20%28double-precision%29) (InputAction :type Input%20Action%20Object%20Reference :default "/Game/ThirdPerson/Input/Actions/IA_Ability.IA_Ability"))
  (:Triggered
    (if (and (not (Variables|Default|GetisTransforming)) (not (Audio|Components|Audio|IsPlaying (Variables|Default|GetShrinkTimeline))))
      (if (not (Variables|Default|GetShrinked))
        (Variables|Default|SetShrinked true)
        (bind _sizemultiplier (Timeline|ShrinkTimeline PlayFromStart)
          (:Update
            (Transformation|SetActorScale3D (Math|Vector|MakeVector _sizemultiplier _sizemultiplier _sizemultiplier)))
          (:Finished
            (Variables|Default|SetCanExecuteTransform (not (Variables|Default|GetShrinked)))))
        (else
          (Variables|Default|SetShrinked false)
          (Timeline|ShrinkTimeline ReverseFromEnd))))))

(event EventBeginPlay
  (|CallParentFunction) ; This node is disabled and will not be called.\nDrag off pins to build functionality.
)

(fn ConstructionScript
  (|CallParentFunction))