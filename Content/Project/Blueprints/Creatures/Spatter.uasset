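; Spatter is a playable creature whose ability spawns a limited supply of platforms in mid-air or underfoot.
; IA_Ability checks the remaining charges, waits briefly, then spawns a Platform just below the actor's origin and decrements the count.
; Landing on anything other than a Platform refills the charges to three, so chained platforms cannot replenish themselves.
; BeginPlay and the ability also print debug strings.
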(event Input|EnhancedActionEvents|EnhancedInputActionIA_Ability
  (params (ActionValue :type Boolean) (ElapsedSeconds :type Float%20%28double-precision%29) (TriggeredSeconds :type Float%20%28double-precision%29) (InputAction :type Input%20Action%20Object%20Reference :default "/Game/ThirdPerson/Input/Actions/IA_Ability.IA_Ability"))
  (:Started
    (if (> (Variables|Default|GetPlatforms) 0)
      (Utilities|FlowControl|Delay 0.2)
      (Game|SpawnActorfromClass "/Game/Project/Blueprints/Others/Platform.Platform_C" (Math|Transform|MakeTransform (- (Transformation|GetActorLocation) "0.000000,0.000000,3.000000") "0, 0, 0" "1.000000,1.000000,1.000000") "Undefined" "MultiplyWithRoot" 0 0)
      (bind _output_get (Variables|Default|SetPlatforms (- (Variables|Default|GetPlatforms) 1)))
      (Development|PrintString (Utilities|String|ToString(Integer) _output_get)))))

(event EventBeginPlay
  (|CallParentFunction)
  (Development|PrintString "Hello"))

(event Collision|EventActorBeginOverlap
  (params (OtherActor :type Actor%20Object%20Reference)))

(event EventTick
  (params (DeltaSeconds :type Float%20%28single-precision%29))
  (|CallParentFunction DeltaSeconds) ; This node is disabled and will not be called.\nDrag off pins to build functionality.
)

(event EventOnLanded
  (params (Hit :type Hit%20Result%20Structure%20%28by%20ref%29))
  (if (not (.bSuccess (Utilities|Casting|CastToPlatform (.hitactor Hit))))
    (Variables|Default|SetPlatforms 3)))

(fn ConstructionScript
  (|CallParentFunction))