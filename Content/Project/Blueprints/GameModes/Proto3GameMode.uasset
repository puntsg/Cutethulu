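; Game mode for a prototype that handles the main-menu-to-gameplay transition, coin count and startup setup.
; BeginPlay applies debug display toggles, starts menu music and adds the level collectables widget.
; The transition locks input, swaps widgets for PlayerUI, and uses a timeline to lerp the menu camera to Taki's follow camera while switching music, then restores control and starts the tutorial.
; UpdateCoin increments the count and broadcasts it to actors.
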(event Custom|UpdateCoin
  (bind _result (Math|Integer|IncrementInt (Variables|Default|Getcoins))
    (:%20%20
      (Variables|Default|Setcoins _result)
      (bind _outactors (Actor|GetAllActorsOfClass 0))
      (for _array_element _outactors
        (CallFunction|AddCoin _array_element (Variables|Default|Getcoins))))))

(event Custom|DeleteMenu&PlayerTransition
  (bind _returnvalue (Game|Player|GetPlayerPawn 0))
  (bind _returnvalue_2 (Game|GetPlayerController 0))
  (bind _currentsoundplayer (Variables|Default|GetCurrentSoundPlayer))
  (bind _camera (Variables|Default|Getcamera))
  (Input|DisableInput _returnvalue_2 _returnvalue_2)
  (Viewport|RemoveAllWidgets)
  (bind _returnvalue_3 (UserInterface|CreateWidget "/Game/Project/Blueprints/UI/PlayerUI.PlayerUI_C"))
  (UserInterface|Viewport|AddtoViewport _returnvalue_3 0)
  (Variables|Default|SetPlayerUI _returnvalue_3)
  (Class|GameplayStatics|SetViewportMouseCaptureMode "NoCapture")
  (Variables|Default|SetOriginalCharacter (Game|Player|GetPlayerPawn 0))
  (bind _newtrack_0 (Timeline|Timeline Play)
    (:Update
      (bind _astaki (Utilities|Casting|CastToTaki (Game|Player|GetPlayerPawn 0)))
      (Transformation|SetWorldTransform (Variables|/Script/Engine.Actor|GetRootComponent _camera) (Math|Transform|Lerp(Transform) (Transformation|GetActorTransform _camera) (Transformation|GetWorldTransform (Variables|/Game/Project/00_Generic/Bluprints/PlayableCharacters/PlayableCharacter.PlayableCharacter_C|GetFollowCamera _astaki)) _newtrack_0) true false)
      (Audio|Components|Audio|FadeOut _currentsoundplayer 0.2 0.0 "Linear" :!class /Script/Engine.AudioComponent)
      (Utilities|FlowControl|Delay 0.2)
      (Audio|Components|Audio|SetSound _currentsoundplayer "/Game/Project/00_Generic/Assets/Sounds/SoundWaves_Cues/SW_CuteMusic.SW_CuteMusic"))
    (:Finished
      (Input|EnableInput _returnvalue_2 _returnvalue_2)
      (Transformation|ResetRelativeTransform (Variables|/Game/Project/00_Generic/Bluprints/PlayableCharacters/PlayableCharacter.PlayableCharacter_C|GetFollowCamera _astaki))
      (bind _ascamera_actor (Utilities|Casting|CastToCameraActor (Variables|Default|Getcamera)))
      (Components|Activation|SetActive (Variables|/Script/Engine.CameraActor|GetCameraComponent _ascamera_actor) false false)
      (bind _astaki_2 (Utilities|Casting|CastToTaki _returnvalue))
      (Game|Player|SetViewTargetwithBlend (Game|GetPlayerController 0) _returnvalue 0.0 "VTBlend_Linear" 0.0 false)
      (Default|BasicTutorial (Variables|Default|GetPlayerUI)))))

(event EventBeginPlay
  (if (Variables|Default|GetShowFPS)
    (Development|ExecuteConsoleCommand "stat fps" 0))
  (CallFunction|Show/HidePrintString)
  (bind _returnvalue (Audio|SpawnSound2D "/Game/Project/00_Generic/Assets/Sounds/SoundWaves_Cues/SW_MainMenu.SW_MainMenu" 1.0 1.0 0.0 0 false false))
  (Variables|Default|SetCurrentSoundPlayer _returnvalue)
  (bind _returnvalue_2 (UserInterface|CreateWidget "/Game/Project/Blueprints/UI/UI_LevelCollectables.UI_LevelCollectables_C"))
  (UserInterface|Viewport|AddtoViewport _returnvalue_2 0))

(fn ConstructionScript)

(fn Show/HidePrintString
  (if (Variables|Default|GetShowStrings)
    (Development|ExecuteConsoleCommand "Enableallscreenmessages" 0)
    (else
      (Development|ExecuteConsoleCommand "Disableallscreenmessages" 0))))