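; Game mode for the Cutethulu game that sets up the HUD and tracks the player's primary and secondary creature transformations.
; Transform events and assignment functions reorder both slots, spawning missing characters and refreshing HUD icons.
; Dual-level load events manage the loading screen, while HealWorld runs a reversible darkness timeline on a material parameter collection, locking player abilities and swapping levels between fades.
; PlayerTransition blends the menu camera into Taki's follow camera, changing music.
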(event Custom|OnPlayerTransform_Event
  (params (CurrentPlayableCharacter :type Playable%20Character%20Object%20Reference) (CharacterToTransform :type Playable%20Character%20Object%20Reference))
  (if (== (Variables|Gameplay|GetSecondaryTransformation) (Variables|Gameplay|GetPrimaryTransformation))
    (bind _output_get (Variables|Gameplay|SetPrimaryTransformation CurrentPlayableCharacter))
    (Variables|Gameplay|SetSecondaryTransformation _output_get)
    (elif (== CharacterToTransform (Variables|Gameplay|GetPrimaryTransformation))
      (Variables|Gameplay|SetPrimaryTransformation (Variables|Gameplay|GetSecondaryTransformation))
      (Variables|Gameplay|SetSecondaryTransformation CurrentPlayableCharacter)
      (else
        (Variables|Gameplay|SetSecondaryTransformation (Variables|Gameplay|GetPrimaryTransformation))
        (Variables|Gameplay|SetPrimaryTransformation CurrentPlayableCharacter))))
  ;[0.15 0.15 0.15 0.5] Assign icons to hud
  (Default|AssignCurrentCreatureIcon (Variables|UI|GetPlayerUI) (.transformationicon (Variables|/Game/Project/Blueprints/Character/PlayableCharacter.PlayableCharacter_C|GetCharacterData CharacterToTransform)))
  (Default|AssignPrimaryTransformationCreatureIcon (Variables|UI|GetPlayerUI) (.transformationicon (Variables|/Game/Project/Blueprints/Character/PlayableCharacter.PlayableCharacter_C|GetCharacterData (Variables|Gameplay|GetPrimaryTransformation))))
  (Default|AssignSecondaryTransformationCreatureIcon (Variables|UI|GetPlayerUI) (.transformationicon (Variables|/Game/Project/Blueprints/Character/PlayableCharacter.PlayableCharacter_C|GetCharacterData (Variables|Gameplay|GetSecondaryTransformation)))))

(event Custom|ResetTransformations
  (bind _output_get (Variables|Gameplay|SetPrimaryTransformation (Variables|Gameplay|GetOriginalCharacter)))
  (Variables|Gameplay|SetSecondaryTransformation _output_get)
  (Default|ResetTransformationIcons (Variables|UI|GetPlayerUI)))

(event Custom|PlayerTransition
  (bind _returnvalue (Game|GetPlayerController 0))
  (bind _returnvalue_2 (Game|Player|GetPlayerPawn 0))
  (bind _currentsoundplayer (Variables|Default|GetCurrentSoundPlayer))
  (bind _cameramainmenu (Variables|Default|GetcameraMainMenu))
  (bind _newtrack_0 (Timeline|Timeline Play)
    (:Update
      (bind _astaki (Utilities|Casting|CastToTaki (Game|Player|GetPlayerPawn 0)))
      (Transformation|SetWorldTransform _cameramainmenu (Math|Transform|Lerp(Transform) (Transformation|GetWorldTransform _cameramainmenu) (Transformation|GetWorldTransform (Variables|/Game/Project/Blueprints/Character/PlayableCharacter.PlayableCharacter_C|GetFollowCamera _astaki)) _newtrack_0) true false)
      ;[0.15 0.15 0.15 0.5] Trying to do Fade Out
      (Class|CameraComponent|SetPostProcessBlendWeight (Variables|Default|GetcameraMainMenu) _newtrack_0)
      (Audio|Components|Audio|FadeOut _currentsoundplayer 0.2 0.0 "Linear" :!class /Script/Engine.AudioComponent)
      (Utilities|FlowControl|Delay 0.2)
      (Audio|Components|Audio|SetSound _currentsoundplayer "/Game/Project/00_Generic/Sounds/SoundWaves_Cues/SW_CuteMusic.SW_CuteMusic"))
    (:Finished
      (Input|EnableInput _returnvalue _returnvalue)
      (Transformation|ResetRelativeTransform (Variables|/Game/Project/Blueprints/Character/PlayableCharacter.PlayableCharacter_C|GetFollowCamera _astaki))
      (Components|Activation|SetActive (Variables|Default|GetcameraMainMenu) false false)
      (bind _astaki_2 (Utilities|Casting|CastToTaki _returnvalue_2))
      (Game|Player|SetViewTargetwithBlend (Game|GetPlayerController 0) _returnvalue_2 0.0 "VTBlend_Linear" 0.0 false)
      (Default|BasicTutorial (Variables|UI|GetPlayerUI)))))

(event EventBeginPlay
  (CallFunction|SetLoadingScreen)
  (Rendering|Material|SetScalarParameterValue "/Game/Project/Materials/MaterialParameterValues/MPC_LoadingEffect.MPC_LoadingEffect" "DarknessAmount" 0.0 :!class /Script/Engine.KismetMaterialLibrary)
  (if (Variables|Debug|GetShowFPS)
    (Development|ExecuteConsoleCommand "stat fps" 0))
  (DebugFunctions|Show/HidePrintString)
  (bind _returnvalue (UserInterface|CreateWidget "/Game/Project/Blueprints/UI/PlayerUI.PlayerUI_C"))
  (bind _output_get (Variables|UI|SetPlayerUI _returnvalue))
  (UserInterface|Viewport|AddtoViewport _output_get 0)
  (Variables|Gameplay|SetOriginalCharacter (.AsTaki (Utilities|Casting|CastToTaki (Game|Player|GetPlayerPawn 0))))
  (CallFunction|ResetTransformations)
  (UIFunctions|ShowPlayerUI true)
  (bind _asbp_cutethulu_instance (Utilities|Casting|CastToBP_CutethuluInstance (Game|GetGameInstance)))
  (UserInterface|Viewport|AddtoViewport (Variables|/Game/Project/Blueprints/Others/BP_CutethuluInstance.BP_CutethuluInstance_C|GetFadeWRef _asbp_cutethulu_instance) 0)
  (EventDispatchers|AssignOnPlayerTransform (delegate Custom|OnPlayerTransform_Event)))

(event Custom|HealWorld
  (bind _returnvalue (Class|DualLevelFunctionLibrary|GetDualLevel))
  (EventDispatchers|UnbindEventfromOnCuteLoaded _returnvalue (delegate Custom|FadeoutWorld))
  (EventDispatchers|BindEventtoOnCuteLoaded _returnvalue (delegate Custom|FadeoutWorld))
  (CallFunction|FadeinWorld))

(event Custom|SetLoadingScreen
  (bind _returnvalue (Class|DualLevelFunctionLibrary|GetDualLevel))
  (EventDispatchers|AssignOnAnyLoad _returnvalue (delegate Custom|OnAnyLoad_Event))
  (EventDispatchers|AssignOnAnyLoaded _returnvalue (delegate Custom|OnAnyLoaded_Event)))

(event Custom|FadeoutWorld
  (bind _returnvalue (Game|Player|GetPlayerPawn 0))
  (bind _asplayable_character (Utilities|Casting|CastToPlayableCharacter _returnvalue))
  (bind (_direction _darkness) (Timeline|LevelFadingTimeline Reverse)
    (:Update
      (Rendering|Material|SetScalarParameterValue "/Game/Project/Materials/MaterialParameterValues/MPC_LoadingEffect.MPC_LoadingEffect" "DarknessAmount" _darkness :!class /Script/Engine.KismetMaterialLibrary)
      (Rendering|Material|SetVectorParameterValue "/Game/Project/Materials/MaterialParameterValues/MPC_LoadingEffect.MPC_LoadingEffect" "PlayerWorldPos" (Math|Conversions|ToLinearColor(Vector) (+ (Transformation|GetActorLocation (Game|Player|GetPlayerPawn 0)) "100.000000,-88.000000,88.000000")) :!class /Script/Engine.KismetMaterialLibrary))
    (:Finished
      (if (Utilities|Enum|Equal(Enum) _direction "Backward")
        (Default|SetCanMoveandJump _asplayable_character (Utilities|Enum|Equal(Enum) _direction "Backward"))
        (Variables|/Game/Project/Blueprints/Character/PlayableCharacter.PlayableCharacter_C|SetCanExecuteTransform _asplayable_character true)
        (Variables|/Game/Project/Blueprints/Character/PlayableCharacter.PlayableCharacter_C|SetCanRotateCamera _asplayable_character true)
        (bind _ascutethulu_player_controller (Utilities|Casting|CastToCutethuluPlayerController (Game|GetPlayerController 0)))
        (Default|ShowLevelUI _ascutethulu_player_controller)
        (else
          (Class|DualLevel|SwapLevel (Class|DualLevelFunctionLibrary|GetDualLevel)))))))

(event Custom|OnAnyLoad_Event
  (Utilities|IsValid (Variables|UI|GetLoading%20Screen)
    (:Is%20Not%20Valid
      (bind _returnvalue (UserInterface|CreateWidget "/Game/Project/Blueprints/UI/LoadingScreen.LoadingScreen_C"))
      (bind _output_get (Variables|UI|SetLoading%20Screen _returnvalue))
      (UserInterface|Viewport|AddtoViewport _output_get 0))))

(event Custom|OnAnyLoaded_Event
  (Widget|RemovefromParent (Variables|UI|GetLoading%20Screen))
  (EventDispatchers|UnbindEventfromOnAnyLoad (Class|DualLevelFunctionLibrary|GetDualLevel) (delegate Custom|OnAnyLoad_Event)))

(event Custom|FadeInWorld
  (bind _returnvalue (Game|Player|GetPlayerPawn 0))
  (bind _returnvalue_2 (Game|Player|GetPlayerPawn 0))
  (bind _asplayable_character (Utilities|Casting|CastToPlayableCharacter _returnvalue))
  (bind _asplayable_character_2 (Utilities|Casting|CastToPlayableCharacter _returnvalue_2))
  (Default|SetCanMoveandJump _asplayable_character false)
  (Variables|/Game/Project/Blueprints/Character/PlayableCharacter.PlayableCharacter_C|SetCanRotateCamera _asplayable_character false)
  (Variables|/Game/Project/Blueprints/Character/PlayableCharacter.PlayableCharacter_C|SetCanExecuteTransform _asplayable_character false)
  (bind (_direction _darkness) (Timeline|LevelFadingTimeline Play)
    (:Update
      (Rendering|Material|SetScalarParameterValue "/Game/Project/Materials/MaterialParameterValues/MPC_LoadingEffect.MPC_LoadingEffect" "DarknessAmount" _darkness :!class /Script/Engine.KismetMaterialLibrary)
      (Rendering|Material|SetVectorParameterValue "/Game/Project/Materials/MaterialParameterValues/MPC_LoadingEffect.MPC_LoadingEffect" "PlayerWorldPos" (Math|Conversions|ToLinearColor(Vector) (+ (Transformation|GetActorLocation (Game|Player|GetPlayerPawn 0)) "100.000000,-88.000000,88.000000")) :!class /Script/Engine.KismetMaterialLibrary))
    (:Finished
      (if (Utilities|Enum|Equal(Enum) _direction "Backward")
        (Default|SetCanMoveandJump _asplayable_character_2 (Utilities|Enum|Equal(Enum) _direction "Backward"))
        (Variables|/Game/Project/Blueprints/Character/PlayableCharacter.PlayableCharacter_C|SetCanExecuteTransform _asplayable_character_2 true)
        (Variables|/Game/Project/Blueprints/Character/PlayableCharacter.PlayableCharacter_C|SetCanRotateCamera _asplayable_character_2 true)
        (bind _ascutethulu_player_controller (Utilities|Casting|CastToCutethuluPlayerController (Game|GetPlayerController 0)))
        (Default|ShowLevelUI _ascutethulu_player_controller)
        (else
          (Class|DualLevel|SwapLevel (Class|DualLevelFunctionLibrary|GetDualLevel)))))))

(fn ConstructionScript)

(fn Show/HidePrintString
  (if (Variables|Debug|GetShowStrings)
    (Development|ExecuteConsoleCommand "Enableallscreenmessages" 0)
    (else
      (Development|ExecuteConsoleCommand "Disableallscreenmessages" 0)))
  (bind _returnvalue (UserInterface|CreateWidget "/Game/Project/Blueprints/UI/UI_LevelCollectables.UI_LevelCollectables_C"))
  (UserInterface|Viewport|AddtoViewport _returnvalue 0))

(fn ShowPlayerUI
  (params (IsVisible%28PlayerUI%29 :type Boolean))
  (bind _playerui (Variables|UI|GetPlayerUI))
  (if IsVisible%28PlayerUI%29
    (Widget|SetVisibility _playerui "Visible")
    (else
      (Widget|SetVisibility _playerui "Collapsed"))))

(fn Fadein
  (bind _fadewref (Variables|UI|GetFadeWRef))
  (Widget|SetVisibility _fadewref "Visible")
  (UserInterface|Animation|PlayAnimation _fadewref (Variables|/Game/Project/Blueprints/UI/WBP_Fade.WBP_Fade_C|GetFadeIn _fadewref) 0.0 1 "Forward" 1.0 false))

(fn FadeOut
  (bind _fadewref (Variables|UI|GetFadeWRef))
  (Widget|SetVisibility _fadewref "Hidden")
  (UserInterface|Animation|PlayAnimation _fadewref (Variables|/Game/Project/Blueprints/UI/WBP_Fade.WBP_Fade_C|GetFadeOut _fadewref) 0.0 1 "Forward" 1.0 false))

(fn GetCharacterfromClass
  (params (Character%20class :type Playable%20Character%20Class%20Reference) (Spawn%20new%20if%20not%20found :type Boolean))
  (bind _outactors (Actor|GetAllActorsOfClass Character%20class))
  (if (Utilities|Array|IsEmpty _outactors)
    (if Spawn%20new%20if%20not%20found
      (bind _returnvalue (Game|SpawnActorfromClass Character%20class (Transformation|GetActorTransform (Game|Player|GetPlayerPawn 0)) "Undefined" "MultiplyWithRoot" 0 0))
      (return _returnvalue true)
      (else
        (return 0 false)))
    (else
      (return (Utilities|Array|Get(acopy) _outactors) true))))

(fn AssignTransform
  (params (CharacterClass :type Playable%20Character%20Class%20Reference))
  (bind _returnedcharacter (GameFunctions|GetCharacterfromClass CharacterClass true))
  (if (.bSuccess (Utilities|Casting|CastToTaki (Variables|Gameplay|GetPrimaryTransformation)))
    ;[0.15 0.15 0.15 0.5] primary equals taki
    (if (.bSuccess (Utilities|Casting|CastToTaki (Variables|Gameplay|GetSecondaryTransformation)))
      (bind _output_get (Variables|Gameplay|SetPrimaryTransformation _returnedcharacter :!label _label))
      (Default|AssignPrimaryTransformationCreatureIcon (Variables|UI|GetPlayerUI) (.transformationicon (Variables|/Game/Project/Blueprints/Character/PlayableCharacter.PlayableCharacter_C|GetCharacterData _output_get)))
      (Utilities|Casting|CastToTaki (Variables|Gameplay|GetSecondaryTransformation))
      (bind _output_get_2 (Variables|Gameplay|SetSecondaryTransformation _returnedcharacter :!label _label_2))
      (Default|AssignSecondaryTransformationCreatureIcon (Variables|UI|GetPlayerUI) (.transformationicon (Variables|/Game/Project/Blueprints/Character/PlayableCharacter.PlayableCharacter_C|GetCharacterData _output_get_2)))
      (elif (== (Utilities|GetClass (Variables|Gameplay|GetSecondaryTransformation)) CharacterClass)
        (GameFunctions|SwapCreaturetoTransform :!label _label_3)
        (else
          (goto _label))))
    (elif (not (== (Utilities|GetClass (Variables|Gameplay|GetSecondaryTransformation)) CharacterClass))
      ;[0.15 0.15 0.15 0.5] primary equals other
      (if (.bSuccess (Utilities|Casting|CastToTaki (Variables|Gameplay|GetSecondaryTransformation)))
        (goto _label_2)
        (elif (== (Utilities|GetClass (Variables|Gameplay|GetSecondaryTransformation)) CharacterClass)
          (goto _label_3)
          (else
            (goto _label)))))))

(fn SwapCreaturetoTransform
  (bind _playerui (Variables|UI|GetPlayerUI))
  (bind _output_get (LocalVariables|SetTemp (Variables|Gameplay|GetSecondaryTransformation)))
  (bind _output_get_2 (Variables|Gameplay|SetSecondaryTransformation (Variables|Gameplay|GetPrimaryTransformation)))
  (bind _output_get_3 (Variables|Gameplay|SetPrimaryTransformation _output_get))
  (Default|AssignSecondaryTransformationCreatureIcon _playerui (.transformationicon (Variables|/Game/Project/Blueprints/Character/PlayableCharacter.PlayableCharacter_C|GetCharacterData _output_get_2)))
  (Default|AssignPrimaryTransformationCreatureIcon _playerui (.transformationicon (Variables|/Game/Project/Blueprints/Character/PlayableCharacter.PlayableCharacter_C|GetCharacterData _output_get_3))))