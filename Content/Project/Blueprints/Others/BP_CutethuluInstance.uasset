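; BP_CutethuluInstance is the Game Instance for Cutethulu, providing screen fades and a debug message toggle.
; On Init it sets the main menu widget class and creates a hidden WBP_Fade widget, keeping a reference to it.
; FadeIn and FadeOut play that widget's animations, with FadeIn making it visible first.
; ShowHidePrintString enables or disables on-screen messages through console commands based on ShowStrings.
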(event EventInit
  (Variables|Default|SetMainMenuWidgetClass "/Game/Project/Blueprints/UI/MainMenu.MainMenu_C")
  (Variables|Default|GetFadeWRef
    (:then)
    (:else
      (bind _returnvalue (UserInterface|CreateWidget "/Game/Project/Blueprints/UI/WBP_Fade.WBP_Fade_C"))
      (Variables|Default|SetFadeWRef _returnvalue)
      (Widget|SetVisibility _returnvalue "Hidden"))))

(fn Show/HidePrintString
  (if (Variables|Default|GetShowStrings)
    (Development|ExecuteConsoleCommand "Enableallscreenmessages" 0)
    (else
      (Development|ExecuteConsoleCommand "Disableallscreenmessages" 0))))

(fn Fadein
  (bind _fadewref (Variables|Default|GetFadeWRef))
  (Widget|SetVisibility _fadewref "Visible")
  (UserInterface|Animation|PlayAnimation _fadewref (Variables|/Game/Project/Blueprints/UI/WBP_Fade.WBP_Fade_C|GetFadeIn _fadewref) 0.0 1 "Forward" 1.0 false))

(fn FadeOut
  (bind _fadewref (Variables|Default|GetFadeWRef))
  (UserInterface|Animation|PlayAnimation _fadewref (Variables|/Game/Project/Blueprints/UI/WBP_Fade.WBP_Fade_C|GetFadeOut _fadewref) 0.0 1 "Forward" 1.0 false))