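; BP_MainMenuCamera is the actor that opens the main menu and provides its camera view.
; On BeginPlay it snaps its camera component to the actor's transform, then runs MainMenu.
; That function creates the menu widget from the class stored in BP_CutethuluInstance, sets itself as the player's view target and shows the widget.
; It also starts underwater intro music, registering both the camera and the sound with TestGameMode.
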(event EventBeginPlay
  (Transformation|SetWorldTransform (Variables|Default|GetMainMenuCamera) (Transformation|GetActorTransform) false false)
  (Variables|Default|SetNew%20View%20Target%20MainMenu self)
  (CallFunction|MainMenu))

(event Collision|EventActorBeginOverlap
  (params (OtherActor :type Actor%20Object%20Reference)))

(event EventTick
  (params (DeltaSeconds :type Float%20%28single-precision%29)))

(fn ConstructionScript)

(fn MainMenu
  (bind _asbp_cutethulu_instance (Utilities|Casting|CastToBP_CutethuluInstance (Game|GetGameInstance)))
  (bind _returnvalue (UserInterface|CreateWidget (Variables|/Game/Project/Blueprints/Others/BP_CutethuluInstance.BP_CutethuluInstance_C|GetMainMenuWidgetClass _asbp_cutethulu_instance)))
  (bind _asmain_menu (Utilities|Casting|CastToMainMenu _returnvalue))
  (Variables|/Game/Project/Blueprints/Character/TestGameMode.TestGameMode_C|SetcameraMainMenu (.AsTest%20Game%20Mode (Utilities|Casting|CastToTestGameMode (Game|GetGameMode))) (Variables|Default|GetMainMenuCamera))
  (Game|Player|SetViewTargetwithBlend (Game|GetPlayerController 0) (Variables|Default|GetNew%20View%20Target%20MainMenu) 0.0 "VTBlend_Linear" 0.0 false)
  (UserInterface|Viewport|AddtoViewport _asmain_menu 0)
  (bind _returnvalue_2 (Audio|SpawnSound2D "/Game/Project/Assets/Sounds/Royalty_free_music_Underwater_Music_Podcast_Music_Intro_Music.Royalty_free_music_Underwater_Music_Podcast_Music_Intro_Music" 1.0 1.0 0.0 0 false false))
  (Variables|/Game/Project/Blueprints/Character/TestGameMode.TestGameMode_C|SetCurrentSoundPlayer (.AsTest%20Game%20Mode (Utilities|Casting|CastToTestGameMode (Game|GetGameMode))) _returnvalue_2))