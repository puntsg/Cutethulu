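; BP_Pusheable is an actor that can be pushed along a given direction.
; Its RecibirEmpuje (receive push) event offsets the current location by the direction times PushForce to get a target.
; A timeline then lerps the actor to that target with a swept SetActorLocation.
; When the Cube component ends an overlap, it turns on physics simulation for that cube.
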(event OnComponentEndOverlap(Cube)
  (params (OverlappedComponent :type Primitive%20Component%20Object%20Reference) (OtherActor :type Actor%20Object%20Reference) (OtherComp :type Primitive%20Component%20Object%20Reference) (OtherBodyIndex :type Integer))
  (Physics|SetSimulatePhysics (Variables|Default|GetCube) true))

(event EventBeginPlay)

(event Collision|EventActorBeginOverlap
  (params (OtherActor :type Actor%20Object%20Reference)))

(event EventTick
  (params (DeltaSeconds :type Float%20%28single-precision%29)))

(event EventRecibirEmpuje
  (params (Direccion :type Vector :default "0, 0, 0"))
  (bind _output_get (Variables|Default|SetInitialPos (Transformation|GetActorLocation)))
  (Variables|Default|SetFinalPos (+ _output_get (* Direccion (Variables|Default|GetPushForce))))
  (bind _alpha (Timeline|PushTimeLine PlayFromStart)
    (:Update
      (bind _returnvalue (Math|Vector|Lerp(Vector) (Variables|Default|GetInitialPos) (Variables|Default|GetFinalPos) _alpha))
      (Transformation|SetActorLocation _returnvalue true false))))

(fn ConstructionScript)