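; BP_Fragment is a collectable piece that the player picks up to feed a portal.
; It stays hidden until OnCuteLoaded plays a seed-to-destination level sequence, then shows an effect, starts a waiting sound and becomes collectable.
; A player overlap adds a piece to the Cutethulu player controller, swaps the sound and plays a to-portal sequence.
; When that sequence finishes, it notifies the first BP_Portal that the fragment arrived.
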(event OnComponentBeginOverlap(Sphere)
  (params (OverlappedComponent :type Primitive%20Component%20Object%20Reference) (OtherActor :type Actor%20Object%20Reference) (OtherComp :type Primitive%20Component%20Object%20Reference) (OtherBodyIndex :type Integer) (bFromSweep :type Boolean) (SweepResult :type Hit%20Result%20Structure%20%28by%20ref%29))
  (bind _audioplayer (Variables|Default|GetAudioPlayer))
  (Utilities|Casting|CastToPlayableCharacter OtherActor)
  (if (and (not (Variables|State|GetCollected)) (Variables|State|GetCanBeCollected))
    (Variables|State|SetCanBeCollected false)
    (Variables|State|SetCollected true)
    (bind _ascutethulu_player_controller (Utilities|Casting|CastToCutethuluPlayerController (Game|GetPlayerController 0)))
    (Default|AddPiece _ascutethulu_player_controller)
    (bind _returnvalue (Sequencer|Player|CreateLevelSequencePlayer (Variables|Sequences|GetToPortalSequence) (Utilities|Struct|MakeMovieSceneSequencePlaybackSettings false (Utilities|Struct|MakeMovieSceneSequenceLoopCount 0) (Utilities|Struct|MakeMovieSceneSequenceTickInterval 0.0 0.0 false false) 1.0 0.0 false false false false false false "None" true)))
    (bind _output_get (Variables|Sequences|SetLevelSequencePlayer _returnvalue))
    (Sequencer|Player|Play _output_get :!class /Script/MovieScene.MovieSceneSequencePlayer)
    (EventDispatchers|BindEventtoOnFinished _output_get (delegate Custom|CustomEvent))
    (Rendering|SetVisibility (Variables|Default|GetEffect) false false)
    (Audio|Components|Audio|Stop _audioplayer)
    (Audio|Components|Audio|SetSound _audioplayer "/Game/Project/00_Generic/Sounds/SoundWaves_Cues/SW_collectable.SW_collectable")
    (Audio|Components|Audio|Play _audioplayer 0.0)))

(event Custom|CustomEvent
  (Development|PrintString "InPortal")
  (bind _outactors (Actor|GetAllActorsOfClass "/Game/Project/Blueprints/Scenario/BP_Portal.BP_Portal_C"))
  (Default|OnFragmentRecievedEvent (Utilities|Array|Get(acopy) _outactors)))

(event Custom|OnFinished_Event
  (Development|PrintString "ReadyToCollect")
  (Variables|State|SetCanBeCollected true)
  (bind _returnvalue (Audio|SpawnSoundatLocation "/Game/Project/00_Generic/Sounds/SoundWaves_Cues/SW_WaitingCollectable.SW_WaitingCollectable" (Transformation|GetActorLocation) "0, 0, 0" 1.0 1.0 0.0 "/USDCore/USDDefaultAttenuation.USDDefaultAttenuation" 0))
  (Variables|Default|SetAudioPlayer _returnvalue)
  (Rendering|SetVisibility (Variables|Default|GetEffect) true false))

(event EventOnCuteLoaded
  (Development|SetHiddeninGame (Variables|Default|GetStaticMesh) false true)
  (bind _returnvalue (Sequencer|Player|CreateLevelSequencePlayer (Variables|Sequences|GetFromSeedToDestinationSequence) (Utilities|Struct|MakeMovieSceneSequencePlaybackSettings false (Utilities|Struct|MakeMovieSceneSequenceLoopCount 0) (Utilities|Struct|MakeMovieSceneSequenceTickInterval 0.0 0.0 false false) 1.0 0.0 false false false false false false "None" true)))
  (bind _output_get (Variables|Sequences|SetLevelSequencePlayer _returnvalue))
  (Sequencer|Player|Play _output_get :!class /Script/MovieScene.MovieSceneSequencePlayer)
  (EventDispatchers|AssignOnFinished _output_get (delegate Custom|OnFinished_Event)))

(event EventBeginPlay
  (Development|SetHiddeninGame (Variables|Default|GetStaticMesh) true true))

(fn ConstructionScript)