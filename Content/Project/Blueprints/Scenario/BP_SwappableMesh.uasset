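; BP_SwappableMesh is a scenario prop that switches its look between a cute and a horror variant.
; OnCuteLoaded and OnHorrorLoaded each set the static mesh to that variant's mesh, then apply its material array slot by slot by index.
; Both events only react to being triggered; the Blueprint has no switching logic of its own and an empty construction script.
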(event EventOnCuteLoaded
  (bind _staticmesh (Variables|Default|GetStaticMesh))
  (Components|StaticMesh|SetStaticMesh _staticmesh (Variables|Default|GetCuteMesh))
  (for (_array_element _array_index) (Variables|Default|GetCuteMaterials)
    (Rendering|Material|SetMaterial _staticmesh _array_index _array_element)))

(event EventOnHorrorLoaded
  (bind _staticmesh (Variables|Default|GetStaticMesh))
  (Components|StaticMesh|SetStaticMesh _staticmesh (Variables|Default|GetHorror%20Mesh))
  (for (_array_element _array_index) (Variables|Default|GetHorror%20Materials)
    (Rendering|Material|SetMaterial _staticmesh _array_index _array_element)))

(fn ConstructionScript)