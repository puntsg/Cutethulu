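; Coin pickup actor with a Ball component that moves back and forth along a looping ping-pong Timeline.
; When a Character overlaps it, it spawns a Niagara effect and a 2D sound, then hides and disables collision.
; The actor destroys itself once the sound finishes; no score or count is recorded here.
; Local rotation nodes driven by RotationSpeed are present but disconnected, so they never run.
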(event Custom|OnAudioFinished_Event
  (Actor|DestroyActor))

(event EventBeginPlay
  (bind (_direction _newtrack_1) (Timeline|Timeline PlayFromStart)
    (:Update
      (Transformation|SetRelativeLocation (Variables|Default|GetBall) _newtrack_1 false false))
    (:Finished
      (if (Utilities|Enum|Equal(Enum) _direction "Backward")
        (Timeline|Timeline Play)
        (else
          (Timeline|Timeline Reverse))))))

(event Collision|EventActorBeginOverlap
  (params (OtherActor :type Actor%20Object%20Reference))
  (Utilities|Casting|CastToCharacter OtherActor)
  (Niagara|SpawnSystematLocation "/Game/Knife_light/VFX/NE_attack01.NE_attack01" (Transformation|GetActorLocation))
  (bind _returnvalue (Audio|SpawnSound2D "/Game/Project/Assets/Sounds/274175-Ancient-Game-Magic-Airy-Breath-Cast-Spell.274175-Ancient-Game-Magic-Airy-Breath-Cast-Spell" 1.0 1.0 0.0 0))
  (Rendering|SetVisibility (Variables|Default|GetDefaultSceneRoot) false true)
  (Collision|SetActorEnableCollision false)
  (EventDispatchers|BindEventtoOnAudioFinished _returnvalue (delegate Custom|OnAudioFinished_Event)))

(event EventTick
  (params (DeltaSeconds :type Float%20%28single-precision%29)))

(fn ConstructionScript)