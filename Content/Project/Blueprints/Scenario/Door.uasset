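; Level-exit double door that opens once enough coins are collected and restarts the level when the player enters it.
; AddCoin compares the collected count to a minimum and calls OpenDoor once, which plays a sound and swings both door pivots via a timeline.
; When the playable character overlaps the box, a second timeline darkens the screen through the game mode's player UI, then runs the Restartlevel console command.
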(event OnComponentBeginOverlap(Box)
  (params (OverlappedComponent :type Primitive%20Component%20Object%20Reference) (OtherActor :type Actor%20Object%20Reference) (OtherComp :type Primitive%20Component%20Object%20Reference) (OtherBodyIndex :type Integer) (bFromSweep :type Boolean) (SweepResult :type Hit%20Result%20Structure%20%28by%20ref%29))
  (Utilities|Casting|CastToPlayableCharacter OtherActor)
  (bind _newtrack_0 (Timeline|Timeline_0 PlayFromStart)
    (:Update
      (bind _asproto_3game_mode (Utilities|Casting|CastToProto3GameMode (Game|GetGameMode)))
      (Default|DarkenScreen (Variables|/Game/Project/Blueprints/GameModes/Proto3GameMode.Proto3GameMode_C|GetPlayerUI _asproto_3game_mode) _newtrack_0))
    (:Finished
      (Development|ExecuteConsoleCommand "Restartlevel" 0))))

(event Custom|OpenDoor
  (Variables|Default|SetHasBeenOpened true)
  (Development|PrintString "OpeningDoor")
  (Audio|SpawnSoundatLocation "/Game/Project/Assets/Sounds/DoorSound.DoorSound" (Transformation|GetActorLocation) "0, 0, 0" 1.0 1.0 0.0 0 0)
  (bind (_direction _door1rotation _door2rotation) (Timeline|Timeline Play)
    (:Update
      (Transformation|SetRelativeRotation (Variables|Default|GetDoor1Pivot) (Math|Rotator|MakeRotator 0.0 0.0 _door1rotation) false false)
      (Transformation|SetRelativeRotation (Variables|Default|GetDoor2Pivot) (Math|Rotator|MakeRotator 0.0 0.0 _door2rotation) false false))))

(event Custom|AddCoin
  (params (Collected :type Integer))
  (Development|PrintString (Utilities|String|Append "Door has coins:" (Utilities|String|ToString(Integer) Collected)))
  (if (>= Collected (Variables|Default|Getminimum))
    (Development|PrintString "Ready toopen")
    (if (not (Variables|Default|GetHasBeenOpened))
      (CallFunction|OpenDoor))))

(event Collision|EventActorBeginOverlap
  (params (OtherActor :type Actor%20Object%20Reference)))

(fn ConstructionScript)