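; Level-exit portal that unlocks once enough fragments are collected and opens its target level when the player interacts.
; Bound dispatchers drive the logic: fragment events raise the count and broadcast the unlock, while interaction checks the unlocked flag.
; The collision volume registers the portal as Taki's current interactive and gates interaction.
; Overlap also fades the Interactive prompt widget through separate in and out timelines.
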(event OnComponentEndOverlap(InteractCollision)
  (params (OverlappedComponent :type Primitive%20Component%20Object%20Reference) (OtherActor :type Actor%20Object%20Reference) (OtherComp :type Primitive%20Component%20Object%20Reference) (OtherBodyIndex :type Integer))
  (bind _astaki (Utilities|Casting|CastToTaki OtherActor))
  (Variables|Default|SetIsCollision false)
  (Variables|/Game/Project/Blueprints/Character/Taki.Taki_C|SetCurrentInteractive _astaki 0)
  (bind _asinteractive (Utilities|Casting|CastToInteractive (UserInterface|GetWidget (Variables|Default|GetWidget))))
  (bind _alfa (Timeline|Timeline_0 Reverse)
    (:Update
      (Default|Alfa _asinteractive _alfa))
    (:Finished
      (Development|SetHiddeninGame (Variables|Default|GetWidget) true false))))

(event OnComponentBeginOverlap(InteractCollision)
  (params (OverlappedComponent :type Primitive%20Component%20Object%20Reference) (OtherActor :type Actor%20Object%20Reference) (OtherComp :type Primitive%20Component%20Object%20Reference) (OtherBodyIndex :type Integer) (bFromSweep :type Boolean) (SweepResult :type Hit%20Result%20Structure%20%28by%20ref%29))
  (bind _astaki (Utilities|Casting|CastToTaki OtherActor))
  (Variables|Default|SetIsCollision true)
  (Variables|/Game/Project/Blueprints/Character/Taki.Taki_C|SetCurrentInteractive _astaki self)
  (Development|SetHiddeninGame (Variables|Default|GetWidget) false false)
  (bind _asinteractive (Utilities|Casting|CastToInteractive (UserInterface|GetWidget (Variables|Default|GetWidget))))
  (bind _alfa (Timeline|Timeline PlayFromStart)
    (:Update
      (Default|Alfa _asinteractive _alfa))))

(event Custom|OnPlayerInteracted_Event
  (Development|PrintString "WalaWalaDubDub")
  (if (Variables|Default|GetPortalUnlocked)
    (Development|PrintString "Can pass")
    (Game|OpenLevel(byObjectReference) (Variables|Default|GetTargetLevel))
    (else
      (Development|PrintString "Quieto parao'"))))

(event Custom|onFragmentRecieved_Event
  (bind _result (Math|Integer|IncrementInt (Variables|Default|GetCollectedFragments))
    (:%20%20
      (if (>= _result (Variables|Default|GetFragmentsToPass))
        (Development|PrintString "portal unlocked")
        (Variables|Default|SetPortalUnlocked true)
        (Default|CallOnPortalUnlocked)))))

(event EventBeginPlay
  (EventDispatchers|BindEventtoOnPlayerInteracted (delegate Custom|OnPlayerInteracted_Event))
  (EventDispatchers|BindEventtoOnFragmentRecieved (delegate Custom|onFragmentRecieved_Event)))

(event EventOnInteract
  (if (Variables|Default|GetIsCollision)
    (Default|CallOnPlayerInteracted)))

(fn ConstructionScript)